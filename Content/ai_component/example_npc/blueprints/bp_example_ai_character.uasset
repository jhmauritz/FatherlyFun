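; Example AI unit character that travels via an AI pathfinder component, with axis inputs for manual movement.
; Tick turns pathfinder travel status into movement input and smoothed yaw rotation.
; Perception forwards sight to a behavior tree service and briefly diverts travel toward noises.
; Component events drive faction colors, selection, hover and highlight visuals, while time changes simulate battle by relocating, damaging or destroying the unit.
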(event `self.ReceiveBeginPlay`
  (bind _enemy_point (`self.enemy_point`))
  ;[1 1 1] Example simple ai pawn,
  ; Beginplay is here.
  (`|ExecutionSequence`
    (:`then_0`
      (`/Game/ai_component/example_data/resource_system/bp_workspace_component.init_work` (`self.bp_workspace_component`) 2))
    (:`then_1`
      (`/Game/ai_component/example_data/resource_system/bp_workspace_component.set_work_point` (`self.bp_workspace_component`) (`|MakeArray` _enemy_point _enemy_point)))))

(event `InputAxis|move_x` :consume false :overrideparent false
  (params (AxisValue :type "Float (single-precision)"))
  ;[1 1 1] Player movement logic.
  (bind (_stick_value _stick_direction) (`self.get_control_direction` AxisValue (stale `InputAxis|move_y` AxisValue) :!label _label)) ; get true axis direction by func.
  (`self.AddMovementInput` (`KismetMathLibrary.Conv_RotatorToVector` _stick_direction) _stick_value) ; add movement input of 360 direction.
)

(event `InputAxis|move_y` :consume false :overrideparent false
  (params (AxisValue :type "Float (single-precision)"))
  ;[1 1 1] Player movement logic.
  (goto _label))

(event `self.ReceiveTick`
  (params (DeltaSeconds :type "Float (single-precision)"))
  (bind _bp_ai_pathfinder_component (`self.bp_ai_pathfinder_component`))
  ;[1 1 1] Tick AI movement.
  (bind (_movement_status _is_movement _is_destination _agent_speed _agent_dir _agent_loc _target_loc _target_rot) (`/Game/ai_component/base_system/blueprints/bp_easy_ai_pathfinder_component.ai_travel_status` _bp_ai_pathfinder_component))
  (if _is_movement
    (`self.AddMovementInput` _agent_dir) ; add movement input by AI wanted\ndirection.
    (else
      (switch `EPathFollowingStatus` _movement_status ; check if not moving but waiting or idling,\nso ai can keep rotating by its wanted rotation,\nwaiting mode engages while AI is finishing destination\nbut wants to rotate to match destination rotation before going to idle, \nso rotation should be active at that period.
        (:`Idle`
          (`/Engine/EditorBlueprintResources/StandardMacros.IsValid` (`/Game/ai_component/base_system/blueprints/bp_easy_ai_pathfinder_component.target_focus` _bp_ai_pathfinder_component) ; if idle, check if AI does have target focus,\nto rotate towards it while in idle, otherwise do nothing.
            (:`Is Valid`
              _)))
        (:`Waiting`
          _))))
  (`self.rotate_character` (`KismetMathLibrary.MakeRotator` 0.0 0.0 (.yaw _target_rot)) true) ; rotate AI by its wanted rotation.
)

(event `self.bp_faction_link.ed_faction`
  (bind (_faction_data _faction_index) (`/Game/ai_component/example_data/group_system/bp_unit_component.get_faction_info` (`self.bp_unit_component`)))
  (bind ((`faction_color_2_838976A344D7000A471BF195FB0A0FDD` _faction_color)) (break `/Game/ai_component/example_data/faction_system/s_faction_data` _faction_data))
  ;[1 1 1] Unit dispatch settings,
  ; faction changes and color selection.
  (bind _asbp_simple_flag (cast `/Game/ai_component/example_npc/blueprints/bp_simple_flag` (`ChildActorComponent.ChildActor` (`self.bp_flag`))))
  (`/Game/ai_component/example_npc/blueprints/bp_simple_flag.set_flag_color` _asbp_simple_flag _faction_color)
  (`/Game/ai_component/example_data/group_system/bp_health_component.set_widget` (`self.bp_health_component`) (`WidgetComponent.GetUserWidgetObject` (`self.hp_widget`)) _faction_color _faction_index))

(event `self.bp_unit_component.ed_selection`
  (params (selection_removed :type Boolean) (faction_id :type Name))
  ;[1 1 1] Unit dispatch settings,
  ; faction changes and color selection.
  (if selection_removed
    (`SceneComponent.SetVisibility` (`self.selection_sphere`) false false)
    (else
      (`SceneComponent.SetVisibility` (`self.selection_sphere`) true false)
      (`MeshComponent.SetVectorParameterValueOnMaterials` (`self.selection_sphere`) "diffuse_color" (0.0 1.0 0.0)))))

(event `self.ReceiveHit`
  (params (MyComp :type "PrimitiveComponent Object Reference") (Other :type "Actor Object Reference") (OtherComp :type "PrimitiveComponent Object Reference") (bSelfMoved :type Boolean) (HitLocation :type "Vector Structure") (HitNormal :type "Vector Structure") (NormalImpulse :type "Vector Structure") (Hit :type "HitResult Structure (by ref)"))
  ;[1 1 1] Optional Event, on Hit, make AI units push each other.
  (bind _return_node (`/Game/ai_component/base_system/blueprints/bp_easy_ai_library.easy_ai_get_component` Other))
  (if _return_node
    (`self.K2_AddActorWorldOffset` (* (* HitNormal 8.0) (`KismetMathLibrary.RandomFloatInRange` 0.0 1.0))) ; push other actor a bit,\nby worlf offset.
  ))

(event `self.bp_unit_component.ed_hover`
  (params (hover_removed :type Boolean))
  ;[1 1 1] Unit dispatch settings,
  ; faction changes and color selection.
  (if (not (`self.is_highlight`))
    (if hover_removed
      (`MeshComponent.SetVectorParameterValueOnMaterials` (`self.Mesh`) "diffuse_color" (1.0 1.0 1.0))
      (else
        (`MeshComponent.SetVectorParameterValueOnMaterials` (`self.Mesh`) "diffuse_color" (0.21 0.28 1.0))))))

(event `self.bp_easy_ai_time_link.ed_time_changed`
  (params (current_time :type "DateTime Structure"))
  ;[1 1 1] Optional Event, on Hit, make AI units push each other.
  (bind _output_get (set `self.latest_time_location` (`NavigationSystemV1.K2_GetRandomLocationInNavigableRadius` (`KismetMathLibrary.MakeVector` 0.0) 1024.0 null null)))
  (`/Game/ai_component/base_system/blueprints/bp_easy_ai_pathfinder_component.ai_pause` (`self.bp_ai_pathfinder_component`) true)
  (`self.K2_SetActorLocation` (+ _output_get (`KismetMathLibrary.MakeVector` 0.0 0.0 (`.OutHalfHeight` (`CapsuleComponent.GetScaledCapsuleSize` (`self.CapsuleComponent`)))))) ; set them to random location in\nrange of 1024.
  (`self.K2_SetActorRotation` (`KismetMathLibrary.MakeRotator` 0.0 0.0 (`KismetMathLibrary.RandomFloatInRange` 0.0 360.0)))
  (bind _current_health (`/Game/ai_component/example_data/group_system/bp_health_component.update_hp` (`self.bp_health_component`) (`KismetMathLibrary.RandomFloatInRange` 5.0 10.0) true))
  (if (<= _current_health 0.0)
    (`self.K2_DestroyActor`)
    (else
      (`KismetSystemLibrary.RetriggerableDelay` (`KismetMathLibrary.RandomFloatInRange` 1.0 2.0))
      (`/Game/ai_component/base_system/blueprints/bp_easy_ai_pathfinder_component.ai_pause` (`self.bp_ai_pathfinder_component`) false))))

(event `self.bp_unit_component.ed_highlight`
  (params (highlight_removed :type Boolean))
  ;[1 1 1] Unit dispatch settings,
  ; faction changes and color selection.
  (if highlight_removed
    (set `self.is_highlight` false)
    (`MeshComponent.SetVectorParameterValueOnMaterials` (`self.Mesh`) "diffuse_color" (1.0 1.0 1.0))
    (else
      (set `self.is_highlight` true)
      (`MeshComponent.SetVectorParameterValueOnMaterials` (`self.Mesh`) "diffuse_color" (1.0 0.0 0.0)))))

(event `self.AIPerception.OnTargetPerceptionUpdated`
  (params (Actor :type "Actor Object Reference") (Stimulus :type "AIStimulus Structure"))
  (bind _bp_ai_pathfinder_component (`self.bp_ai_pathfinder_component`))
  ;[1 1 1] AI Perception reactions,
  ; so when hearing or seeing some target,
  ; we can send events from here to make AI react.
  (bind _returnvalue (`AIPerceptionSystem.GetSenseClassForStimulus` Stimulus))
  (if (== _returnvalue "/Script/AIModule.AISense_Sight")
    (bind (_is_valid _found_index _service_reference) (`/Game/ai_component/base_system/blueprints/bp_easy_ai_pathfinder_component.get_service` (`self.bp_ai_pathfinder_component`) "t1" false))
    (if _is_valid
      (bind _asservice_stimuli (cast `/Game/ai_component/example_npc/tree_data/service_stimuli` _service_reference))
      (`/Game/ai_component/example_npc/tree_data/service_stimuli.event_stimuli` _asservice_stimuli Actor Stimulus) ; send the stimuli data\nto AI tree service.
    )
    (elif (== _returnvalue "/Script/AIModule.AISense_Hearing")
      (`/Game/ai_component/base_system/blueprints/bp_easy_ai_pathfinder_component.ai_set_travel` _bp_ai_pathfinder_component (make `/Game/ai_component/base_system/structs/01_base/s_ai_05_travel` null (`.StimulusLocation` (break `AIStimulus` Stimulus)) (0.0 0.0 0.0) (struct) 0.0 0.0 0.0 true false false false "hearnoise"))
      (`/Game/ai_component/base_system/blueprints/bp_easy_ai_pathfinder_component.ai_pause` _bp_ai_pathfinder_component true) ; simply pauses the AI brain, stops the ticking the brain component,\nso AI does not update its tree, but keeps its latest activity in mind, if it gets unpaused again.
      (`KismetSystemLibrary.RetriggerableDelay` 1.0)
      (`/Game/ai_component/base_system/blueprints/bp_easy_ai_pathfinder_component.ai_clear_path` _bp_ai_pathfinder_component "NewEnumerator2") ; clear the path to noise
      (`/Game/ai_component/base_system/blueprints/bp_easy_ai_pathfinder_component.ai_pause` _bp_ai_pathfinder_component false) ; continue tree activity again,\npause gets automatically turned off when\nAI sets different data by func, or gets global AI clear/init func called.
    )))

(fn `get_control_direction`
  (params (axis_x :type "Float (double-precision)") (axis_y :type "Float (double-precision)"))
  (returns (stick_value :type "Float (double-precision)") (stick_direction :type "Rotator Structure"))
  ;[1 1 1] find true movement rotation
  (return (`KismetMathLibrary.FMax` (`KismetMathLibrary.Abs` axis_x) (`KismetMathLibrary.Abs` axis_y)) (`KismetMathLibrary.MakeRotator` 0.0 0.0 (.yaw (`KismetMathLibrary.NormalizedDeltaRotator` (`self.GetControlRotation`) (* (`KismetMathLibrary.MakeRotator` 0.0 0.0 (`KismetMathLibrary.DegAtan2` axis_x axis_y)) -1))))))

(fn `rotate_character`
  (params (target_rotation :type "Rotator Structure") (is_moving :type Boolean))
  ;[1 1 1] Rotate character when moving and replicate current rotation by event.
  (if is_moving
    (`self.K2_SetActorRotation` (`KismetMathLibrary.RInterpTo` (`self.K2_GetActorRotation`) target_rotation (`GameplayStatics.GetWorldDeltaSeconds`) 10.0)) ; set local rotation by target rotation.
  ))

(fn `UserConstructionScript`)