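; Minebot example NPC: a simple non-pawn actor bot with AI pathfinding, faction colors, and selection, hover and highlight feedback.
; Tick follows the pathfinder component's travel status, moving by swept SetActorLocation with interpolated yaw instead of a movement component.
; Overlapping another AI actor repositions the bot horizontally away from it after a short delay.
; Unit component events drive selection visuals, while faction updates recolor the flag and mesh and set up the health widget.
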(event `self.ReceiveBeginPlay`
  ;[1 1 1] Simple custom bot,(non pawn actor)
  ; Beginplay is here.
  (`SceneComponent.SetVisibility` (`self.selection_sphere`) false false)
  (`/Game/ai_component/example_data/resource_system/bp_workspace_component.init_work` (`self.bp_workspace_component`) 15))

(event `self.ReceiveTick`
  (params (DeltaSeconds :type "Float (single-precision)"))
  ;[1 1 1] Ticking logic for smooth movement.
  (bind (_movement_status _is_movement _is_destination _agent_speed _agent_dir _agent_loc _target_loc _target_rot) (`/Game/ai_component/base_system/blueprints/bp_easy_ai_pathfinder_component.ai_travel_status` (`self.bp_easy_ai_pathfinder_component`)))
  (if _is_movement
    (`self.K2_SetActorLocation` (+ (`self.K2_GetActorLocation`) (* _agent_dir (* (`self.speed`) (`GameplayStatics.GetWorldDeltaSeconds`)))) true) ; movement by sweep,\nbecause we don't use any of movement components here,\nonly AI logic.
    (`self.K2_SetActorRotation` (`KismetMathLibrary.RInterpTo` (`self.K2_GetActorRotation`) (`KismetMathLibrary.MakeRotator` 0.0 0.0 (.yaw _target_rot)) (`GameplayStatics.GetWorldDeltaSeconds`) 3.0)) ; rotation with interp.
  ))

(event `self.ReceiveActorBeginOverlap`
  (params (OtherActor :type "Actor Object Reference"))
  (bind _returnvalue (`self.K2_GetActorLocation` OtherActor))
  ;[1 1 1] Overlap push movement logic.
  (bind _return_node (`/Game/ai_component/base_system/blueprints/bp_easy_ai_library.easy_ai_get_component` OtherActor))
  (if _return_node
    (`KismetSystemLibrary.Delay` 0.02)
    (`/Engine/EditorBlueprintResources/StandardMacros.IsValid` OtherActor
      (:`Is Valid`
        (`self.K2_SetActorLocation` (+ _returnvalue (* (`KismetMathLibrary.MakeVector` (.x (`KismetMathLibrary.GetDirectionUnitVector` _returnvalue (`self.K2_GetActorLocation`))) (.y (`KismetMathLibrary.GetDirectionUnitVector` _returnvalue (`self.K2_GetActorLocation`)))) 100.0)))))))

(event `self.bp_unit_component.ed_selection`
  (params (selection_removed :type Boolean) (faction_id :type Name))
  ;[1 1 1] Selection and hover logic.
  (if selection_removed
    (`SceneComponent.SetVisibility` (`self.selection_sphere`) false false)
    (else
      (`SceneComponent.SetVisibility` (`self.mesh_cube`) true false)
      (`SceneComponent.SetVisibility` (`self.selection_sphere`) true false)
      (`MeshComponent.SetVectorParameterValueOnMaterials` (`self.selection_sphere`) "diffuse_color" (`KismetMathLibrary.Conv_LinearColorToVector` (`KismetMathLibrary.MakeColor` 0.0 1.0))))))

(event `self.bp_unit_component.ed_hover`
  (params (hover_removed :type Boolean))
  ;[1 1 1] Selection and hover logic.
  (if hover_removed
    (`MeshComponent.SetVectorParameterValueOnMaterials` (`self.mesh_cube`) "diffuse_color" (1.0 1.0 1.0))
    (else
      (`MeshComponent.SetVectorParameterValueOnMaterials` (`self.mesh_cube`) "diffuse_color" (0.25 0.7 0.7)))))

(event `self.bp_faction_link.ed_faction`
  (bind (_faction_data _faction_index) (`/Game/ai_component/example_data/group_system/bp_unit_component.get_faction_info` (`self.bp_unit_component`)))
  (bind _faction_color (break `/Game/ai_component/example_data/faction_system/s_faction_data` (`/Game/ai_component/example_data/group_system/bp_unit_component.get_faction_info` (`self.bp_unit_component`))))
  ;[1 1 1] Faction update, set colors.
  (bind _asbp_simple_flag (cast `/Game/ai_component/example_npc/blueprints/bp_simple_flag` (`ChildActorComponent.ChildActor` (`self.bp_flag`))))
  (`/Game/ai_component/example_npc/blueprints/bp_simple_flag.set_flag_color` _asbp_simple_flag _faction_color)
  (`MeshComponent.SetVectorParameterValueOnMaterials` (`self.mesh_cube`) "diffuse_color" (`KismetMathLibrary.Conv_LinearColorToVector` _faction_color))
  (`/Game/ai_component/example_data/group_system/bp_health_component.set_widget` (`self.bp_health_component`) (`WidgetComponent.GetUserWidgetObject` (`self.hp_widget`)) (`.faction_color_2_838976A344D7000A471BF195FB0A0FDD` (break `/Game/ai_component/example_data/faction_system/s_faction_data` _faction_data)) _faction_index))

(event `self.bp_unit_component.ed_highlight`
  (params (highlight_removed :type Boolean))
  ;[1 1 1] Selection and hover logic.
  (if highlight_removed
    (`MeshComponent.SetVectorParameterValueOnMaterials` (`self.highlight_cube`) "diffuse_color" (1.0 1.0 1.0))
    (`SceneComponent.SetVisibility` (`self.highlight_cube`) false false)
    (else
      (`MeshComponent.SetVectorParameterValueOnMaterials` (`self.highlight_cube`) "diffuse_color" (0.0 0.0 0.0))
      (`SceneComponent.SetVisibility` (`self.highlight_cube`) true false))))

(fn `UserConstructionScript`)