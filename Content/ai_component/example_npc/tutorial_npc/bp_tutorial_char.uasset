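; Example tutorial AI character that shows how to drive a simple pawn with the Easy AI components.
; Each tick it reads the pathfinder's travel status, adding movement input along the agent direction when moving and smoothly turning toward the target rotation.
; Perception stimuli are forwarded to the tutorial service fetched from the pathfinder.
; Time-link changes print the hour and relocate the character to a random navigable point.
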(event `self.ReceiveBeginPlay`
  ;[1 1 1] Example simple ai pawn,
  ; Beginplay is here.
)

(event `self.ReceiveTick`
  (params (DeltaSeconds :type "Float (single-precision)"))
  ;[1 1 1] Example simple ai pawn,
  ; Beginplay is here.
  (bind (_movement_status _is_movement _is_destination _agent_speed _agent_dir _agent_loc _target_loc _target_rot) (`/Game/ai_component/base_system/blueprints/bp_easy_ai_pathfinder_component.ai_travel_status` (`self.bp_easy_ai_pathfinder_component`)))
  (switch `EPathFollowingStatus` _movement_status
    (:`Waiting`
      _)
    (:`Moving`
      (`self.AddMovementInput` _agent_dir)))
  (`self.K2_SetActorRotation` (`KismetMathLibrary.RInterpTo` (`self.K2_GetActorRotation`) _target_rot (`GameplayStatics.GetWorldDeltaSeconds`) 7.0)))

(event `self.bp_easy_ai_pathfinder_component.ed_path_updated`
  (params (path_event :type "/Game/ai_component/base_system/enums/enum_path_update Enum" :default "NewEnumerator0") (path_cleared :type Boolean) (ai_path :type "/Game/ai_component/base_system/structs/01_base/s_ai_02_nav Structure"))
  ;[1 1 1] Example simple ai pawn,
  ; Beginplay is here.
)

(event `self.AIPerception.OnTargetPerceptionUpdated`
  (params (Actor :type "Actor Object Reference") (Stimulus :type "AIStimulus Structure"))
  ;[1 1 1] Example simple ai pawn,
  ; Beginplay is here.
  (bind _returnvalue (`AIPerceptionSystem.GetSenseClassForStimulus` Stimulus))
  (bind (_is_valid _found_index _service_reference) (`/Game/ai_component/base_system/blueprints/bp_easy_ai_pathfinder_component.get_service` (`self.bp_easy_ai_pathfinder_component`) "base_service" false))
  (bind _asservice_tutorial (cast `/Game/ai_component/example_npc/tutorial_npc/service_tutorial` _service_reference))
  (`/Game/ai_component/example_npc/tutorial_npc/service_tutorial.ai_stimuli` _asservice_tutorial Actor Stimulus _returnvalue))

(event `self.bp_easy_ai_time_link.ed_time_changed`
  (params (current_time :type "DateTime Structure"))
  ;[1 1 1] Example simple ai pawn,
  ; Beginplay is here.
  (`KismetSystemLibrary.PrintString` (`KismetStringLibrary.Conv_IntToString` (`.Hour` (`KismetMathLibrary.BreakDateTime` current_time)))) ; the part of logic from tutorial video,\nwait simulation notify example.
  (`self.K2_SetActorLocation` (`NavigationSystemV1.K2_GetRandomLocationInNavigableRadius` (`KismetMathLibrary.MakeVector` 0.0) 2048.0 null null)))

(fn `UserConstructionScript`)