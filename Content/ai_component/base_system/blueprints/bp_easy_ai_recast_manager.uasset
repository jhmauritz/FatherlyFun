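; AI recast manager that tags RecastNavMesh actors so pathfinding checks can later tell them apart by actor type.
; AssignRecastTags loops over every navmesh, takes the display name after the hyphen, lowercases it, drops a three-character prefix and adds the result as a unique tag.
; It then sets IsLoaded; BeginPlay and the construction script are empty, so the function is not called within this Blueprint.
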(event `self.ReceiveBeginPlay`
  ;[1 1 1] AI recast manager,
  ; beginplay is here.
)

(fn `assign_recast_tags`
  (locals (local_recast :type "RecastNavMesh Object Reference"))
  ;[1 1 1] Assign tags to recast actors,
  ; for pathfinding checks by actor types later.
  (bind _outactors (`GameplayStatics.GetAllActorsOfClass` "/Script/NavigationSystem.RecastNavMesh"))
  (for _array_element _outactors
    (set `local.local_recast` _array_element)
    (`KismetArrayLibrary.Array_AddUnique` (`Actor.Tags` (`local.local_recast`)) (`KismetStringLibrary.Conv_StringToName` (`KismetStringLibrary.RightChop` (`KismetStringLibrary.ToLower` (`.RightS` (`KismetStringLibrary.Split` (`KismetSystemLibrary.GetDisplayName` (`local.local_recast`)) "-"))) 3))))
  (set `self.is_loaded` true))

(fn `UserConstructionScript`)