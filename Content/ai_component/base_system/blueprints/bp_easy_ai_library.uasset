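; Blueprint function library of static lookup helpers for the Easy AI system.
; Getters find an actor's AI pathfinder (directly or via a link component), workspace, unit, faction link and owning faction, or cast it to a group manager, returning success flags.
; AI and faction lookups fall back to the world context actor.
; Other helpers find the time manager, check the recast manager's loaded flag, and randomize timer intervals to ease performance load.
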(fn `easy_ai_game_loaded`
  (returns (is_loaded :type Boolean))
  ;[1 1 1] Get if game mode is loaded, and all necessary actors are spawned.
  (bind _outactors (`GameplayStatics.GetAllActorsOfClass` null "/Game/ai_component/base_system/blueprints/bp_easy_ai_recast_manager.bp_easy_ai_recast_manager_C"))
  (if (`KismetArrayLibrary.Array_IsValidIndex` _outactors)
    (return (`/Game/ai_component/base_system/blueprints/bp_easy_ai_recast_manager.is_loaded` (`|GetArrayItem` _outactors)))
    (else
      (return false))))

(fn `easy_ai_get_component`
  (params (ai_actor :type "Actor Object Reference"))
  (returns (return_node :type Boolean) (ai_component :type "/Game/ai_component/base_system/blueprints/bp_easy_ai_pathfinder_component Object Reference"))
  (locals (local_actor :type "Actor Object Reference") (local_path :type "/Game/ai_component/base_system/blueprints/bp_easy_ai_pathfinder_component Object Reference") (local_link :type "/Game/ai_component/base_system/blueprints/bp_easy_ai_link Object Reference"))
  ;[1 1 1] Library func to get every actor's ai controller.
  (set `local.local_actor` ai_actor)
  (`/Engine/EditorBlueprintResources/StandardMacros.IsValid` (`local.local_actor`)
    (:`Is Valid`
      _)
    (:`Is Not Valid`
      (bind _asactor (cast `Actor` (`local.__WorldContext`))
        (:`then`
          (set `local.local_actor` _asactor))
        (:`CastFailed`
          (return false null)))))
  (set `local.local_path` (`Actor.GetComponentByClass` (`local.local_actor`) "/Game/ai_component/base_system/blueprints/bp_easy_ai_pathfinder_component.bp_easy_ai_pathfinder_component_C"))
  (`/Engine/EditorBlueprintResources/StandardMacros.IsValid` (`local.local_path`)
    (:`Is Valid`
      (return true (`local.local_path`)))
    (:`Is Not Valid`
      (set `local.local_link` (`Actor.GetComponentByClass` (`local.local_actor`) "/Game/ai_component/base_system/blueprints/bp_easy_ai_link.bp_easy_ai_link_C"))
      (`/Engine/EditorBlueprintResources/StandardMacros.IsValid` (`local.local_link`)
        (:`Is Valid`
          (`/Engine/EditorBlueprintResources/StandardMacros.IsValid` (`/Game/ai_component/base_system/blueprints/bp_easy_ai_link.bp_ai_component` (`local.local_link`))
            (:`Is Valid`
              (return true (`/Game/ai_component/base_system/blueprints/bp_easy_ai_link.bp_ai_component` (`local.local_link`))))
            (:`Is Not Valid`
              _)))
        (:`Is Not Valid`
          _))
      (return false null))))

(fn `easy_ai_get_controller`
  (params (ai_actor :type "Actor Object Reference"))
  (returns (return_node :type Boolean) (ai_component :type "/Game/ai_component/base_system/blueprints/bp_easy_ai_pathfinder_component Object Reference") (ai_controller :type "AIController Object Reference") (ai_pawn :type "Actor Object Reference"))
  ;[1 1 1] Library func to get every actor or pawn's ai controller.
  (bind (_return_node _ai_component) (`self.easy_ai_get_component` ai_actor (`local.__WorldContext`)))
  (return _return_node _ai_component (`/Game/ai_component/base_system/blueprints/bp_easy_ai_pathfinder_component.current_controller` _ai_component) (`/Game/ai_component/base_system/blueprints/bp_easy_ai_pathfinder_component.controlled_object` _ai_component)))

(fn `easy_ai_get_faction_link`
  (params (target_actor :type "Actor Object Reference"))
  (returns (return_node :type Boolean) (faction_link :type "/Game/ai_component/example_data/faction_system/bp_faction_link Object Reference"))
  (locals (local_actor :type "Actor Object Reference") (local_faction :type "/Game/ai_component/example_data/faction_system/bp_faction_link Object Reference"))
  ;[1 1 1] Get specified actor's faction link.
  (set `local.local_actor` target_actor)
  (`/Engine/EditorBlueprintResources/StandardMacros.IsValid` (`local.local_actor`)
    (:`Is Valid`
      (set `local.local_faction` (`Actor.GetComponentByClass` (`local.local_actor`) "/Game/ai_component/example_data/faction_system/bp_faction_link.bp_faction_link_C"))
      (`/Engine/EditorBlueprintResources/StandardMacros.IsValid` (`local.local_faction`)
        (:`Is Valid`
          (return true (`local.local_faction`)))
        (:`Is Not Valid`
          _)))
    (:`Is Not Valid`
      _))
  (return false null))

(fn `easy_ai_get_faction_manager`
  (params (target_actor :type "Actor Object Reference"))
  (returns (return_node :type Boolean) (faction_reference :type "/Game/ai_component/example_data/faction_system/bp_faction_manager Object Reference"))
  (locals (local_actor :type "Actor Object Reference"))
  ;[1 1 1] Get specified actor's faction actor.
  (set `local.local_actor` target_actor)
  (`/Engine/EditorBlueprintResources/StandardMacros.IsValid` (`local.local_actor`)
    (:`Is Valid`
      _)
    (:`Is Not Valid`
      (bind _asactor (cast `Actor` (`local.__WorldContext`))
        (:`then`
          (set `local.local_actor` _asactor))
        (:`CastFailed`
          (return false null)))))
  (bind (_return_node _faction_link) (`self.easy_ai_get_faction_link` (`local.local_actor`)))
  (if _return_node
    (bind (_return_node_2 _faction_reference) (`/Game/ai_component/example_data/faction_system/bp_faction_link.get_owner_faction` _faction_link))
    (return _return_node_2 _faction_reference)
    (else
      (return false null))))

(fn `easy_ai_get_group`
  (params (target_actor :type "Actor Object Reference"))
  (returns (return_node :type Boolean) (group_manager :type "/Game/ai_component/example_data/group_system/bp_group_manager Object Reference"))
  (locals (local_actor :type "Actor Object Reference"))
  ;[1 1 1] Get specified actor's group link.
  (set `local.local_actor` target_actor)
  (`/Engine/EditorBlueprintResources/StandardMacros.IsValid` (`local.local_actor`)
    (:`Is Valid`
      (bind _asbp_group_manager (cast `/Game/ai_component/example_data/group_system/bp_group_manager` (`local.local_actor`))
        (:`then`
          (return true _asbp_group_manager))
        (:`CastFailed`
          _)))
    (:`Is Not Valid`
      _))
  (return false null))

(fn `easy_ai_get_time_manager`
  (returns (return_node :type Boolean) (time_manager :type "/Game/ai_component/day_system/blueprints/bp_easy_ai_time_manager Object Reference"))
  (locals (local_actor :type "Actor Object Reference"))
  ;[1 1 1] Get time manager logic.
  (bind _outactors (`GameplayStatics.GetAllActorsOfClass` null "/Game/ai_component/day_system/blueprints/bp_easy_ai_time_manager.bp_easy_ai_time_manager_C"))
  (if (`KismetArrayLibrary.Array_IsValidIndex` _outactors)
    (return true (`|GetArrayItem` _outactors))
    (else
      (return false null))))

(fn `easy_ai_get_unit`
  (params (target_actor :type "Actor Object Reference"))
  (returns (return_node :type Boolean) (unit_reference :type "/Game/ai_component/example_data/group_system/bp_unit_component Object Reference"))
  (locals (local_actor :type "Actor Object Reference") (local_unit :type "/Game/ai_component/example_data/group_system/bp_unit_component Object Reference"))
  ;[1 1 1] Get specified actor's unit component.
  (set `local.local_actor` target_actor)
  (`/Engine/EditorBlueprintResources/StandardMacros.IsValid` (`local.local_actor`)
    (:`Is Valid`
      (set `local.local_unit` (`Actor.GetComponentByClass` (`local.local_actor`) "/Game/ai_component/example_data/group_system/bp_unit_component.bp_unit_component_C"))
      (`/Engine/EditorBlueprintResources/StandardMacros.IsValid` (`local.local_unit`)
        (:`Is Valid`
          (return true (`local.local_unit`)))
        (:`Is Not Valid`
          _)))
    (:`Is Not Valid`
      _))
  (return false null))

(fn `easy_ai_get_workspace`
  (params (target_actor :type "Actor Object Reference"))
  (returns (return_node :type Boolean) (workspace_reference :type "/Game/ai_component/example_data/resource_system/bp_workspace_component Object Reference"))
  (locals (local_actor :type "Actor Object Reference") (local_workspace :type "/Game/ai_component/example_data/resource_system/bp_workspace_component Object Reference"))
  ;[1 1 1] Get specified actor's workspace component.
  (set `local.local_actor` target_actor)
  (`/Engine/EditorBlueprintResources/StandardMacros.IsValid` (`local.local_actor`)
    (:`Is Valid`
      (set `local.local_workspace` (`Actor.GetComponentByClass` (`local.local_actor`) "/Game/ai_component/example_data/resource_system/bp_workspace_component.bp_workspace_component_C"))
      (`/Engine/EditorBlueprintResources/StandardMacros.IsValid` (`local.local_workspace`)
        (:`Is Valid`
          (return true (`local.local_workspace`)))
        (:`Is Not Valid`
          _)))
    (:`Is Not Valid`
      _))
  (return false null))

(fn `easy_ai_timer_randomizer`
  (params (base_value :type "Float (double-precision)") (random_value :type "Float (double-precision)"))
  (returns (ReturnValue :type "Float (double-precision)"))
  ;[1 1 1] Easy AI return base value + random, like in AI service nodes, to make timers with random values,
  ; to keep performance higher.
  (return (`KismetMathLibrary.FClamp` (+ base_value (`KismetMathLibrary.RandomFloatInRange` (* random_value -1.0) random_value)) 0.016667 1000.0)))