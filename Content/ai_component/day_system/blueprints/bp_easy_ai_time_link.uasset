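; Actor component that links its owner to the Easy AI day system time manager and relays time changes.
; On BeginPlay it caches the time manager and adds the easyai_time_link tag to the owner.
; Its time_changed event reads the manager's current date-time through GetCurrentTime and broadcasts it through the TimeChanged dispatcher.
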(event `self.ReceiveBeginPlay`
  ;[1 1 1] Time manager link component, to notify when waiting time updates.
  (bind (_return_node _time_manager) (`/Game/ai_component/base_system/blueprints/bp_easy_ai_library.easy_ai_get_time_manager`))
  (set `self.time_manager` _time_manager)
  (`KismetArrayLibrary.Array_AddUnique` (`Actor.Tags` (`self.GetOwner`)) "easyai_time_link"))

(event `time_changed`
  ;[1 1 1] Time manager link component, to notify when waiting time updates.
  (bind _current_date_time (`self.get_current_time`))
  (`self.ed_time_changed` _current_date_time))

(fn `get_current_time`
  (returns (current_date_time :type "DateTime Structure"))
  ;[1 1 1] Get current date in quick way.
  (return (`/Game/ai_component/day_system/blueprints/bp_easy_ai_time_manager.current_date_time` (`self.time_manager`))))