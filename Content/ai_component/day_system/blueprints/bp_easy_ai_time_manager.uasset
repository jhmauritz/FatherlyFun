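; Easy AI time manager that runs the in-game date and clock from a configurable start time and speed, shown in an on-screen widget.
; Tick advances the clock while unpaused.
; Waiting pauses the game and skips one hour per delayed loop pass until the requested hours run out.
; Each skipped hour notifies tagged actors' time-link components in ascending priority order, then calls a time-changed dispatcher.
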(event `self.ReceiveBeginPlay`
  ;[1 1 1] Time manager logic,
  ; beginplay logic is here.
  (`|ExecutionSequence`
    (:`then_0`
      (`self.set_starting_time`))
    (:`then_1`
      (`self.add_time_widget`))))

(event `self.ReceiveTick`
  (params (DeltaSeconds :type "Float (single-precision)"))
  ;[1 1 1] Time manager logic,
  ; beginplay logic is here.
  (`|ExecutionSequence`
    (:`then_0`
      (if (not (`GameplayStatics.IsGamePaused`))
        (`self.tick_timespan_ms`)))
    (:`then_1`
      (`self.update_widget`))))

(event `start_wait`
  (params (hours_to_wait :type Integer))
  ;[1 1 1] Waiting logic is here.
  (set `self.hours_to_wait` hours_to_wait)
  (set `self.is_waiting` true)
  (`GameplayStatics.SetGamePaused` true)
  (`self.wait_loop`))

(event `wait_loop`
  ;[1 1 1] Waiting logic is here.
  (`KismetSystemLibrary.RetriggerableDelay` (`self.wait_delay`))
  (if (> (`self.hours_to_wait`) 0)
    (`self.wait_update`)
    (else
      (`self.stop_wait`))))

(event `stop_wait`
  ;[1 1 1] Waiting logic is here.
  (if (`self.is_waiting`)
    (set `self.is_waiting` false)
    (set `self.hours_to_wait` 0)
    (`GameplayStatics.SetGamePaused` false)))

(fn `add_time_widget`
  ;[1 1 1] Add and assign current time widget.
  (`/Engine/EditorBlueprintResources/StandardMacros.IsValid` (`self.w_time_reference`)
    (:`Is Not Valid`
      (bind _returnvalue (`|CreateWidget` "/Game/ai_component/day_system/blueprints/w_time_manager.w_time_manager_C"))
      (set `self.w_time_reference` _returnvalue)
      (`UserWidget.AddToViewport` (`self.w_time_reference`) 0))))

(fn `convert_digit_string`
  (params (input_int :type Integer) (use_single_digit :type Boolean))
  (returns (ReturnValue :type String))
  (bind _returnvalue (`KismetStringLibrary.Conv_IntToString` input_int))
  ;[1 1 1] Convert digit to string,
  ; by using zero value if needed.
  (return (`KismetMathLibrary.SelectString` _returnvalue (`KismetMathLibrary.SelectString` (`KismetStringLibrary.Concat_StrStr` "0" _returnvalue) _returnvalue (< (`KismetStringLibrary.Len` _returnvalue) 2)) use_single_digit)))

(fn `get_current_date_time`
  (returns (Hour :type Integer) (Minute :type Integer) (Second :type Integer) (Day :type Integer) (Month :type Integer) (Year :type Integer))
  (bind (_year _month _day _hour _minute _second) (`KismetMathLibrary.BreakDateTime` (`self.current_date_time`)))
  ;[1 1 1] Return current time.
  (return _hour _minute _second _day _month _year))

(fn `get_string_date_time`
  (returns (hour :type String) (minute :type String) (second :type String) (day :type String) (month :type String) (year :type String))
  (bind (_hour _minute _second _day _month _year) (`self.get_current_date_time`))
  ;[1 1 1] Get string time.
  (return (`self.convert_digit_string` _hour) (`self.convert_digit_string` _minute) (`self.convert_digit_string` _second) (`self.convert_digit_string` _day) (`self.convert_digit_string` _month) (`self.convert_digit_string` _year)))

(fn `prioritize_time`
  (locals (local_actors :type "Array of Actor Object Reference") (local_priority :type "Array of Integer"))
  (bind _indexofminvalue (`KismetMathLibrary.MinOfIntArray` (`local.local_priority`)))
  (bind _returnvalue (`self.GetComponentByClass` (`|GetArrayItem` (`local.local_actors`) _indexofminvalue) "/Game/ai_component/day_system/blueprints/bp_easy_ai_time_link.bp_easy_ai_time_link_C"))
  ;[1 1 1] Prioritized send time.
  (bind _outactors (`GameplayStatics.GetAllActorsWithTag` "easyai_time_link"))
  (bind (_arrayindex _arrayelement) (`/Engine/EditorBlueprintResources/StandardMacros.ReverseForEachLoop` _outactors)
    (:`LoopBody`
      (bind _returnvalue_2 (`self.GetComponentByClass` _arrayelement "/Game/ai_component/day_system/blueprints/bp_easy_ai_time_link.bp_easy_ai_time_link_C"))
      (`/Engine/EditorBlueprintResources/StandardMacros.IsValid` _returnvalue_2
        (:`Is Valid`
          (if (`/Game/ai_component/day_system/blueprints/bp_easy_ai_time_link.notify_time` _returnvalue_2)
            (`KismetArrayLibrary.Array_Add` (`local.local_actors`) _arrayelement)
            (`KismetArrayLibrary.Array_Add` (`local.local_priority`) (`/Game/ai_component/day_system/blueprints/bp_easy_ai_time_link.notify_priority` _returnvalue_2))))))
    (:`Completed`
      (if (>= _indexofminvalue 0) :!label _label
        (`/Engine/EditorBlueprintResources/StandardMacros.IsValid` _returnvalue
          (:`Is Valid`
            (`/Game/ai_component/day_system/blueprints/bp_easy_ai_time_link.time_changed` _returnvalue)
            (`KismetArrayLibrary.Array_Remove` (`local.local_actors`) _indexofminvalue)
            (`KismetArrayLibrary.Array_Remove` (`local.local_priority`) _indexofminvalue)
            (goto _label)))))))

(fn `set_starting_time`
  (bind (_year _month _day _hour _minute _second _millisecond) (break `/Game/ai_component/day_system/structs/s_day_struct` (`self.starting_time`)))
  ;[1 1 1] Set world starting time as current on beginplay,
  ; should be skipped when game is loaded and etc.
  (set `self.current_date_time` (`KismetMathLibrary.MakeDateTime` _year _month _day _hour _minute _second _millisecond)))

(fn `tick_timespan_hr`
  (params (Hours :type "Float (double-precision)"))
  ;[1 1 1] Tick update timespan by hours.
  (set `self.current_date_time` (+ (`self.current_date_time`) (`KismetMathLibrary.FromHours` Hours))))

(fn `tick_timespan_ms`
  ;[1 1 1] Tick and add time to current one.
  (set `self.current_date_time` (+ (`self.current_date_time`) (`KismetMathLibrary.FromMilliseconds` (* (`GameplayStatics.GetWorldDeltaSeconds`) (* (`self.time_speed`) 1000.0))))))

(fn `update_widget`
  (bind (_hour _minute _second _day _month _year) (`self.get_string_date_time`))
  ;[1 1 1] Update widget's time text,
  ; each tick.
  (`/Engine/EditorBlueprintResources/StandardMacros.IsValid` (`self.w_time_reference`)
    (:`Is Valid`
      (`TextBlock.SetText` (`/Game/ai_component/day_system/blueprints/w_time_manager.time_text` (`self.w_time_reference`)) (`KismetTextLibrary.Conv_StringToText` (`KismetStringLibrary.Concat_StrStr` _hour ":" _minute ":" _second " \n" _day "/" _month "/" _year))))))

(fn `UserConstructionScript`)

(fn `wait_update`
  ;[1 1 1] Waiting update by delay loop, will skip 1 hour and update loop,
  ; also call notify event to update any actors that are needed.
  (if (`self.is_waiting`)
    (`|ExecutionSequence`
      (:`then_0`
        (if (> (`self.hours_to_wait`) 0)
          (`/Engine/EditorBlueprintResources/StandardMacros.DecrementInt` (`self.hours_to_wait`)
            (:`  `
              (`self.tick_timespan_hr` 1.0)
              (`self.prioritize_time`)
              (`self.ed_time_changed`)))))
      (:`then_1`
        (`self.wait_loop`)))))