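; Resource actor for an AI worker example, holding a depletable resource count shown on a 3D widget refreshed every tick.
; A workspace component manages four worker slots at arrow-defined work points.
; On request it adds a box collider at a worker's point for the navmesh, and destroys it when that worker is removed.
; RemoveResources clamps withdrawals to the remaining stock and returns the amount taken.
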(event `self.ReceiveBeginPlay`
  ;[1 1 1] Resource actor,
  ; Beginplay is here.
  (`/Game/ai_component/example_data/resource_system/bp_workspace_component.init_work` (`self.bp_workspace_component`) 4)
  (`/Game/ai_component/example_data/resource_system/bp_workspace_component.set_work_point` (`self.bp_workspace_component`) (`|MakeArray` (`self.Arrow`) (`self.Arrow1`) (`self.Arrow2`) (`self.Arrow3`) :!type "SceneComponent Object Reference")))

(event `self.ReceiveTick`
  (params (DeltaSeconds :type "Float (single-precision)"))
  ;[1 1 1] Resource actor,
  ; Beginplay is here.
  (bind _asw_resource_value (cast `/Game/ai_component/example_data/resource_system/w_resource_value` (`WidgetComponent.GetUserWidgetObject` (`self.widget_count`))))
  (`TextBlock.SetText` (`/Game/ai_component/example_data/resource_system/w_resource_value.text_value` _asw_resource_value) (`KismetTextLibrary.Conv_IntToText` (`self.resources_count`) false false)))

(event `set_work_collision`
  (params (worker_actor :type "Actor Object Reference"))
  ;[1 1 1] Resource actor,
  ; Beginplay is here.
  (bind (_is_valid _found_index _work_point _nav_collider) (`/Game/ai_component/example_data/resource_system/bp_workspace_component.get_worker` (`self.bp_workspace_component`) worker_actor))
  (if _is_valid
    (`/Engine/EditorBlueprintResources/StandardMacros.IsValid` _nav_collider ; check if there are no nav collider exist.
      (:`Is Not Valid`
        (bind _returnvalue (`AddComponent|NODE_AddBoxComponent-3` :`RelativeTransform` (`KismetMathLibrary.MakeTransform` (.location (`SceneComponent.GetRelativeTransform` _work_point)) (.rotation (`SceneComponent.GetRelativeTransform` _work_point))))) ; set box collider for navmesh.
        (`/Game/ai_component/example_data/resource_system/bp_workspace_component.set_collider` (`self.bp_workspace_component`) _found_index _returnvalue)))))

(event `self.bp_workspace_component.ed_worker_removed`
  (params (slot_index :type Integer) (worker_actor :type "Actor Object Reference") (work_point :type "SceneComponent Object Reference") (nav_collider :type "BoxComponent Object Reference"))
  ;[1 1 1] Resource actor,
  ; Beginplay is here.
  (`/Engine/EditorBlueprintResources/StandardMacros.IsValid` nav_collider
    (:`Is Valid`
      (`ActorComponent.K2_DestroyComponent` nav_collider) ; colliders will be auto removed by index of worker\nwhen the worker is removed.
    )))

(event `self.bp_workspace_component.ed_worker_added`
  (params (slot_index :type Integer) (worker_actor :type "Actor Object Reference") (working_point :type "SceneComponent Object Reference"))
  ;[1 1 1] Resource actor,
  ; Beginplay is here.
)

(fn `remove_resources`
  (params (remove_count :type Integer))
  (returns (is_exist :type Boolean) (removed_value :type Integer))
  (locals (local_value :type Integer :default 0))
  ;[1 1 1] Remove resources count.
  (set `local.local_value` remove_count)
  (set `local.local_value` (`KismetMathLibrary.Clamp` (`local.local_value`) 0 (`self.resources_count`)))
  (set `self.resources_count` (- (`self.resources_count`) (`local.local_value`)))
  (return (> (`local.local_value`) 0) (`local.local_value`)))

(fn `UserConstructionScript`)