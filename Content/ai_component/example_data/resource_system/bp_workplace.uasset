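; Workplace actor Blueprint in an AI resource-system example that sets itself up as a place of work on BeginPlay.
; It initializes its workspace component, then writes its work name and ID into a w_resource_value widget shown through a widget component.
; If that widget cast succeeds, it also adds the work ID to its actor tags.
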(event `self.ReceiveBeginPlay`
  ;[1 1 1] Simple workplace logic,
  ; Beginplay is here.
  (`/Game/ai_component/example_data/resource_system/bp_workspace_component.init_work` (`self.bp_workspace_component`) 1)
  (bind _asw_resource_value (cast `/Game/ai_component/example_data/resource_system/w_resource_value` (`WidgetComponent.GetUserWidgetObject` (`self.widget_text`))))
  (`TextBlock.SetText` (`/Game/ai_component/example_data/resource_system/w_resource_value.text_value` _asw_resource_value) (`|FormatText` "Name: {NameInfo} \nID: {IDINFO}" (`self.work_name`) (`KismetTextLibrary.Conv_NameToText` (`self.work_id`))))
  (`KismetArrayLibrary.Array_AddUnique` (`self.Tags`) (`self.work_id`)))

(fn `UserConstructionScript`)