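; Workspace component for AI workers and resource actors, managing which workers occupy which work slots.
; SetWorker fills or frees slots with work points and nav colliders, updating each worker's LatestWork back-reference, which EndPlay uses to release its slot.
; Search functions rank targets by distance, free slots and occupancy-based weighting.
; Pick functions approve a workspace only when the requesting worker is also that workspace's closest idle candidate.
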(event `self.ReceiveBeginPlay`
  ;[1 1 1] Workspace finder component,
  ; beginplay is here.
)

(event `self.ReceiveTick`
  (params (DeltaSeconds :type "Float (single-precision)"))
  ;[1 1 1] Workspace finder component,
  ; beginplay is here.
  (bind (_arrayindex _arrayelement) (`/Engine/EditorBlueprintResources/StandardMacros.ReverseForEachLoop` (`self.worker_actors`))
    (:`LoopBody`
      (`/Engine/EditorBlueprintResources/StandardMacros.IsValid` _arrayelement
        (:`Is Not Valid`
          (`self.set_worker` null _arrayindex false false true) ; clearing unexisting workers from data,\nif found out that they are not valid.
        )))))

(event `self.ReceiveEndPlay`
  (params (EndPlayReason :type "EEndPlayReason Enum" :default "Destroyed"))
  (bind _latest_work (`self.latest_work`))
  ;[1 1 1] Workspace finder component,
  ; beginplay is here.
  (`/Engine/EditorBlueprintResources/StandardMacros.IsValid` _latest_work
    (:`Is Valid`
      (bind (_return_node _workspace_reference) (`/Game/ai_component/base_system/blueprints/bp_easy_ai_library.easy_ai_get_workspace` _latest_work))
      (if _return_node
        (`self.set_worker` _workspace_reference (`self.GetOwner`) 0 false false true)))))

(fn `check_free_slot`
  (returns (ReturnValue :type Boolean) (found_index :type Integer) (workers_length :type Integer))
  (locals (local_empty :type "Actor Object Reference"))
  (bind _returnvalue (`KismetArrayLibrary.Array_Find` (`self.worker_actors`) (`local.local_empty`)))
  ;[1 1 1] Check for free place on workers.
  (return (>= _returnvalue 0) _returnvalue (`self.workers_length`)))

(fn `find_closest_array`
  (params (main_actors :type "Array of Actor Object Reference") (work_actors :type "Array of Actor Object Reference") (max_priority_workers :type Integer) (max_valid_workers :type Integer))
  (returns (is_valid :type Boolean) (closest_unit :type "Actor Object Reference") (closest_enemy :type "Actor Object Reference") (MinValue :type "Float (double-precision)"))
  (locals (local_resouce_actors :type "Array of Actor Object Reference") (local_main_actors :type "Array of Actor Object Reference") (local_distance :type "Array of Float (double-precision)") (local_closest_resource :type "Array of Actor Object Reference") (local_index :type Integer :default 0) (local_unit :type "Actor Object Reference") (local_priority :type Integer) (local_invalid :type Integer))
  (bind (_indexofminvalue _minvalue) (`KismetMathLibrary.MinOfFloatArray` (`local.local_distance`)))
  ;[1 1 1] Find closest array to other array of actors,
  ; so basically this shows which actor from first array is closest to actor from other array,
  ; outputs both actors that are closest to each other.
  (set `local.local_main_actors` main_actors)
  (set `local.local_resouce_actors` work_actors)
  (set `local.local_priority` max_priority_workers)
  (set `local.local_invalid` max_valid_workers)
  (if (`KismetArrayLibrary.Array_IsValidIndex` (`local.local_resouce_actors`))
    (for (_array_element _array_index) (`local.local_main_actors`)
      (set `local.local_unit` _array_element)
      (set `local.local_index` _array_index)
      (bind (_is_valid _closest_enemy _minvalue_2) (`self.find_closest_target` (`local.local_unit`) (`local.local_resouce_actors`) (`local.local_priority`) (`local.local_invalid`)))
      (`KismetArrayLibrary.Array_Set` (`local.local_closest_resource`) (`local.local_index`) _closest_enemy true)
      (`KismetArrayLibrary.Array_Set` (`local.local_distance`) (`local.local_index`) _minvalue_2 true))
    (if (>= _indexofminvalue 0)
      (return (< _minvalue (`self.max_length`)) (`|GetArrayItem` (`local.local_main_actors`) _indexofminvalue) (`|GetArrayItem` (`local.local_closest_resource`) _indexofminvalue) _minvalue)
      (else
        (return false null null (`self.max_length`))))
    (else
      (return false null null (`self.max_length`)))))

(fn `find_closest_base`
  (params (main_actor :type "Actor Object Reference") (work_actors :type "Array of Actor Object Reference"))
  (returns (is_valid :type Boolean) (closest_found :type "Actor Object Reference") (MinValue :type "Float (double-precision)"))
  (locals (local_resouce_actors :type "Array of Actor Object Reference") (local_main_actor :type "Actor Object Reference") (local_resource :type "Actor Object Reference") (local_distance_array :type "Array of Float (double-precision)") (local_distance_value :type "Float (double-precision)" :default 0.0))
  (bind (_indexofminvalue _minvalue) (`KismetMathLibrary.MinOfFloatArray` (`local.local_distance_array`)))
  ;[1 1 1] Find closest actor from array to main actor.
  (set `local.local_main_actor` main_actor)
  (set `local.local_resouce_actors` work_actors)
  (for _array_element (`local.local_resouce_actors`)
    (set `local.local_resource` _array_element)
    (set `local.local_distance_value` (`Actor.GetDistanceTo` (`local.local_resource`) (`local.local_main_actor`)))
    (bind (_return_node _workspace_reference) (`/Game/ai_component/base_system/blueprints/bp_easy_ai_library.easy_ai_get_workspace` (`local.local_resource`)))
    (if _return_node
      (bind _returnvalue (`self.check_free_slot` _workspace_reference))
      (if (and _returnvalue (`/Game/ai_component/example_data/resource_system/bp_workspace_component.can_work` _workspace_reference))
        (`KismetArrayLibrary.Array_Add` (`local.local_distance_array`) (`local.local_distance_value`))
        (else
          (`KismetArrayLibrary.Array_Add` (`local.local_distance_array`) (`self.max_length`) :!label _label)))
      (else
        (goto _label))))
  (if (>= _indexofminvalue 0)
    (return (< _minvalue (`self.max_length`)) (`|GetArrayItem` (`local.local_resouce_actors`) _indexofminvalue) _minvalue)
    (else
      (return false null (`self.max_length`)))))

(fn `find_closest_scalar`
  (params (main_actor :type "Actor Object Reference") (work_actors :type "Array of Actor Object Reference") (priority_length :type "Array of Integer") (priority_scale :type "Array of Float (double-precision)"))
  (returns (is_valid :type Boolean) (closest_found :type "Actor Object Reference") (MinValue :type "Float (double-precision)"))
  (locals (local_resouce_actors :type "Array of Actor Object Reference") (local_main_actor :type "Actor Object Reference") (local_resource :type "Actor Object Reference") (local_distance_array :type "Array of Float (double-precision)") (local_priority :type "Array of Integer") (local_distance_value :type "Float (double-precision)" :default 0.0) (local_scale :type "Array of Float (double-precision)") (local_found :type Integer))
  (bind _local_found (`local.local_found`))
  (bind _local_scale (`local.local_scale`))
  (bind (_indexofminvalue _minvalue) (`KismetMathLibrary.MinOfFloatArray` (`local.local_distance_array`)))
  ;[1 1 1] Find closest actor from array to main actor.
  (set `local.local_main_actor` main_actor)
  (set `local.local_resouce_actors` work_actors)
  (set `local.local_priority` priority_length)
  (set `local.local_scale` priority_scale)
  (for _array_element (`local.local_resouce_actors`)
    (set `local.local_resource` _array_element)
    (set `local.local_distance_value` (`Actor.GetDistanceTo` (`local.local_resource`) (`local.local_main_actor`)))
    (bind (_return_node _workspace_reference) (`/Game/ai_component/base_system/blueprints/bp_easy_ai_library.easy_ai_get_workspace` (`local.local_resource`)))
    (if _return_node
      (bind (_returnvalue _found_index _workers_length) (`self.check_free_slot` _workspace_reference))
      (set `local.local_found` -1)
      (if (and _returnvalue (`/Game/ai_component/example_data/resource_system/bp_workspace_component.can_work` _workspace_reference))
        (bind (_arrayindex _arrayelement) (`/Engine/EditorBlueprintResources/StandardMacros.ReverseForEachLoop` (`local.local_priority`))
          (:`LoopBody`
            (if (>= _workers_length _arrayelement)
              (set `local.local_found` 0)))
          (:`Completed`
            (if (>= _local_found 0)
              (if (`KismetArrayLibrary.Array_IsValidIndex` _local_scale _local_found)
                (`KismetArrayLibrary.Array_Add` (`local.local_distance_array`) (* (`local.local_distance_value`) (`|GetArrayItem` _local_scale _workers_length)))
                (else
                  (`KismetArrayLibrary.Array_Add` (`local.local_distance_array`) (`self.max_length`) :!label _label))))))
        (else
          (goto _label)))
      (else
        (goto _label))))
  (if (>= _indexofminvalue 0)
    (return (< _minvalue (`self.max_length`)) (`|GetArrayItem` (`local.local_resouce_actors`) _indexofminvalue) _minvalue)
    (else
      (return false null (`self.max_length`)))))

(fn `find_closest_target`
  (params (main_actor :type "Actor Object Reference") (work_actors :type "Array of Actor Object Reference") (max_priority_workers :type Integer) (max_valid_workers :type Integer))
  (returns (is_valid :type Boolean) (closest_enemy :type "Actor Object Reference") (MinValue :type "Float (double-precision)"))
  (locals (local_resouce_actors :type "Array of Actor Object Reference") (local_main_actor :type "Actor Object Reference") (local_resource :type "Actor Object Reference") (local_distance_array :type "Array of Float (double-precision)") (local_priority :type Integer) (local_distance_value :type "Float (double-precision)" :default 0.0) (local_invalid :type Integer) (local_workers :type Integer :default 0))
  (bind (_indexofminvalue _minvalue) (`KismetMathLibrary.MinOfFloatArray` (`local.local_distance_array`)))
  ;[1 1 1] Find closest actor from array to main actor.
  (set `local.local_main_actor` main_actor)
  (set `local.local_resouce_actors` work_actors)
  (set `local.local_priority` max_priority_workers)
  (set `local.local_invalid` max_valid_workers)
  (bind (_return_node _workspace_reference) (`/Game/ai_component/base_system/blueprints/bp_easy_ai_library.easy_ai_get_workspace` (`local.local_main_actor`)))
  (if _return_node
    (bind _returnvalue (`self.get_self_working` _workspace_reference))
    (if _returnvalue
      (return false null (`self.max_length`))
      (else
        (for _array_element (`local.local_resouce_actors`)
          (set `local.local_resource` _array_element)
          (set `local.local_distance_value` (`Actor.GetDistanceTo` (`local.local_resource`) (`local.local_main_actor`)))
          (bind (_return_node_2 _workspace_reference_2) (`/Game/ai_component/base_system/blueprints/bp_easy_ai_library.easy_ai_get_workspace` (`local.local_resource`)))
          (bind (_returnvalue_2 _found_index _workers_length) (`self.check_free_slot` _workspace_reference_2))
          (set `local.local_workers` _workers_length)
          (`KismetArrayLibrary.Array_Add` (`local.local_distance_array`) (`KismetMathLibrary.SelectFloat` (`KismetMathLibrary.SelectFloat` (`local.local_distance_value`) (* (`local.local_distance_value`) 2.0) (<= (`local.local_workers`) (`local.local_priority`))) (`self.max_length`) (<= (`local.local_workers`) (`local.local_invalid`)))))
        (if (>= _indexofminvalue 0)
          (return (< _minvalue (`self.max_length`)) (`|GetArrayItem` (`local.local_resouce_actors`) _indexofminvalue) _minvalue)
          (else
            (return false null (`self.max_length`))))))))

(fn `find_closest_worker`
  (params (resource_actor :type "Actor Object Reference") (work_actors :type "Array of Actor Object Reference"))
  (returns (is_valid :type Boolean) (closest_worker :type "Actor Object Reference") (MinValue :type "Float (double-precision)"))
  (locals (local_work_actors :type "Array of Actor Object Reference") (local_resource :type "Actor Object Reference") (local_worker :type "Actor Object Reference") (local_distance_array :type "Array of Float (double-precision)") (local_distance_value :type "Float (double-precision)" :default 0.0))
  (bind _local_distance_array (`local.local_distance_array`))
  (bind (_indexofminvalue _minvalue) (`KismetMathLibrary.MinOfFloatArray` (`local.local_distance_array`)))
  ;[1 1 1] Find closest actor from array to main actor.
  (set `local.local_resource` resource_actor)
  (set `local.local_work_actors` work_actors)
  (for (_array_element _array_index) (`local.local_work_actors`)
    (set `local.local_worker` _array_element)
    (`/Engine/EditorBlueprintResources/StandardMacros.IsValid` (`local.local_worker`)
      (:`Is Valid`
        (`/Engine/EditorBlueprintResources/StandardMacros.IsValid` (`local.local_resource`)
          (:`Is Valid`
            (set `local.local_distance_value` (`Actor.GetDistanceTo` (`local.local_worker`) (`local.local_resource`)))
            (bind (_return_node _workspace_reference) (`/Game/ai_component/base_system/blueprints/bp_easy_ai_library.easy_ai_get_workspace` (`local.local_worker`)))
            (if _return_node
              (bind _returnvalue (`self.get_self_working` _workspace_reference))
              (if (and (not _returnvalue) (`/Game/ai_component/example_data/resource_system/bp_workspace_component.can_work` _workspace_reference))
                (`KismetArrayLibrary.Array_Set` _local_distance_array _array_index (`Actor.GetDistanceTo` (`local.local_worker`) (`local.local_resource`)) true)
                (else
                  (`KismetArrayLibrary.Array_Set` _local_distance_array _array_index (`self.max_length`) true :!label _label)))
              (else
                (goto _label))))))))
  (if (>= _indexofminvalue 0)
    (return (< _minvalue (`self.max_length`)) (`|GetArrayItem` (`local.local_work_actors`) _indexofminvalue) _minvalue)
    (else
      (return false null (`self.max_length`)))))

(fn `get_closest_slot`
  (params (worker_actor :type "Actor Object Reference"))
  (returns (is_valid :type Boolean) (found_index :type Integer))
  (locals (local_actor :type "Actor Object Reference") (local_distance :type "Array of Float (double-precision)") (local_max_float :type "Float (double-precision)" :default 3.8375042132696105e+18) (local_loc :type "Vector Structure" :default (0.0 0.0 0.0)))
  (bind _worker_actors (`self.worker_actors`))
  (bind (_indexofminvalue _minvalue) (`KismetMathLibrary.MinOfFloatArray` (`local.local_distance`)))
  ;[1 1 1] Find closest work point.
  (set `local.local_actor` worker_actor)
  (if (`KismetArrayLibrary.Array_IsValidIndex` (`self.work_points`))
    (for (_array_element _array_index) (`self.work_points`)
      (`/Engine/EditorBlueprintResources/StandardMacros.IsValid` _array_element
        (:`Is Valid`
          (set `local.local_loc` (`SceneComponent.K2_GetComponentLocation` _array_element)))
        (:`Is Not Valid`
          (set `local.local_loc` (`Actor.K2_GetActorLocation` (`self.GetOwner`)))))
      (if (`KismetArrayLibrary.Array_IsValidIndex` _worker_actors _array_index)
        (if (== (`|GetArrayItem` _worker_actors _array_index) null)
          (`KismetArrayLibrary.Array_Set` (`local.local_distance`) _array_index (`KismetMathLibrary.VSize` (- (`local.local_loc`) (`Actor.K2_GetActorLocation` (`local.local_actor`)))) true)
          (else
            (`KismetArrayLibrary.Array_Set` (`local.local_distance`) _array_index (`local.local_max_float`) true)))))
    (if (>= _indexofminvalue 0)
      (return (< _minvalue (`local.local_max_float`)) _indexofminvalue)
      (else
        (return false -1)))
    (else
      (return false -1))))

(fn `get_self_working`
  (returns (ReturnValue :type Boolean) (latest_work :type "Actor Object Reference"))
  ;[1 1 1] Get if self working actor is valid and return actor.
  (return (`KismetSystemLibrary.IsValid` (`self.latest_work`)) (`self.latest_work`)))

(fn `get_work_point`
  (params (worker_actor :type "Actor Object Reference"))
  (returns (is_valid :type Boolean) (work_point :type "SceneComponent Object Reference"))
  (bind _work_points (`self.work_points`))
  ;[1 1 1] Get working point ref.
  (bind (_is_valid _found_index) (`self.get_worker` worker_actor))
  (if _is_valid
    (bind _returnvalue (`KismetArrayLibrary.Array_IsValidIndex` _work_points _found_index))
    (if _returnvalue
      (bind _output (`|GetArrayItem` _work_points _found_index))
      (`/Engine/EditorBlueprintResources/StandardMacros.IsValid` _output
        (:`Is Valid`
          (return _returnvalue _output))
        (:`Is Not Valid`
          _))))
  (return false (`Actor.RootComponent` (`self.GetOwner`))))

(fn `get_worker`
  (params (worker_actor :type "Actor Object Reference"))
  (returns (is_valid :type Boolean) (found_index :type Integer) (work_point :type "SceneComponent Object Reference") (nav_collider :type "BoxComponent Object Reference"))
  (locals (local_index :type Integer))
  ;[1 1 1] Get worker reference.
  (set `local.local_index` (`KismetArrayLibrary.Array_Find` (`self.worker_actors`) worker_actor))
  (if (>= (`local.local_index`) 0)
    (return (!= (`|GetArrayItem` (`self.worker_actors`) (`local.local_index`)) null) (`local.local_index`) (`|GetArrayItem` (`self.work_points`) (`local.local_index`)) (`|GetArrayItem` (`self.nav_colliders`) (`local.local_index`)))
    (else
      (return false (`local.local_index`) null null))))

(fn `init_work`
  (params (work_size :type Integer))
  (locals (local_size :type Integer))
  ;[1 1 1] Init work by work-points.
  (set `local.local_size` work_size)
  (`KismetArrayLibrary.Array_Resize` (`self.worker_actors`) (`local.local_size`))
  (`KismetArrayLibrary.Array_Resize` (`self.work_points`) (`local.local_size`))
  (`KismetArrayLibrary.Array_Resize` (`self.nav_colliders`) (`local.local_size`)))

(fn `pick_interval_closest`
  (params (main_worker :type "Actor Object Reference") (other_workers :type "Array of Actor Object Reference") (available_resources :type "Array of Actor Object Reference") (priority_length :type "Array of Integer (by ref)") (priority_scale :type "Array of Float (double-precision) (by ref)"))
  (returns (is_valid :type Boolean) (closest_workspace :type "Actor Object Reference"))
  (locals (local_other_resources :type "Array of Actor Object Reference") (local_res :type "Actor Object Reference") (local_worker :type "Actor Object Reference") (local_other_workers :type "Array of Actor Object Reference"))
  ;[1 1 1] Pick best matching workspace.
  (set `local.local_worker` main_worker)
  (set `local.local_other_workers` other_workers)
  (set `local.local_other_resources` available_resources)
  (bind (_is_valid _closest_found) (`self.find_closest_scalar` (`local.local_worker`) (`local.local_other_resources`) priority_length priority_scale))
  (if _is_valid
    (set `local.local_res` _closest_found)
    (bind (_return_node _workspace_reference) (`/Game/ai_component/base_system/blueprints/bp_easy_ai_library.easy_ai_get_workspace` (`local.local_res`)))
    (if _return_node
      (bind (_is_valid_2 _closest_worker) (`self.find_closest_worker` _workspace_reference (`local.local_res`) (`local.local_other_workers`)))
      (return (== _closest_worker (`local.local_worker`)) (`local.local_res`))
      (else
        _)))
  (return false null))

(fn `pick_very_closest`
  (params (main_worker :type "Actor Object Reference") (other_workers :type "Array of Actor Object Reference") (available_resources :type "Array of Actor Object Reference"))
  (returns (is_valid :type Boolean) (closest_workspace :type "Actor Object Reference"))
  (locals (local_other_resources :type "Array of Actor Object Reference") (local_res :type "Actor Object Reference") (local_worker :type "Actor Object Reference") (local_other_workers :type "Array of Actor Object Reference"))
  ;[1 1 1] Pick best matching workspace.
  (set `local.local_worker` main_worker)
  (set `local.local_other_workers` other_workers)
  (set `local.local_other_resources` available_resources)
  (bind (_is_valid _closest_found) (`self.find_closest_base` (`local.local_worker`) (`local.local_other_resources`)))
  (if _is_valid
    (set `local.local_res` _closest_found)
    (bind (_return_node _workspace_reference) (`/Game/ai_component/base_system/blueprints/bp_easy_ai_library.easy_ai_get_workspace` (`local.local_res`)))
    (if _return_node
      (bind (_is_valid_2 _closest_worker) (`self.find_closest_worker` _workspace_reference (`local.local_res`) (`local.local_other_workers`)))
      (if _is_valid_2
        (return (== _closest_worker (`local.local_worker`)) (`local.local_res`))
        (else
          _))))
  (return false null))

(fn `set_collider`
  (params (slot_index :type Integer) (nav_collider :type "BoxComponent Object Reference"))
  ;[1 1 1] Set nav collider.
  (`KismetArrayLibrary.Array_Set` (`self.nav_colliders`) slot_index nav_collider))

(fn `set_self_working`
  (params (latest_work :type "Actor Object Reference"))
  (locals (local_work :type "Actor Object Reference"))
  ;[1 1 1] Set self as latest working.
  (set `local.local_work` latest_work)
  (`/Engine/EditorBlueprintResources/StandardMacros.IsValid` (`self.latest_work`)
    (:`Is Valid`
      (`|ExecutionSequence`
        (:`then_0`
          (bind (_return_node _workspace_reference) (`/Game/ai_component/base_system/blueprints/bp_easy_ai_library.easy_ai_get_workspace` (`self.latest_work`)))
          (`self.set_worker` _workspace_reference (`self.GetOwner`) 0 false false true))
        (:`then_1`
          (set `self.latest_work` (`local.local_work`) :!label _label))))
    (:`Is Not Valid`
      (goto _label))))

(fn `set_work_point`
  (params (work_points :type "Array of SceneComponent Object Reference"))
  ;[1 1 1] Set working helper points.
  (set `self.work_points` work_points))

(fn `set_worker`
  (params (worker_actor :type "Actor Object Reference") (slot_index :type Integer) (replace_existing :type Boolean) (use_closest :type Boolean) (remove_worker :type Boolean))
  (returns (is_success :type Boolean))
  (locals (local_worker :type "Actor Object Reference") (local_index :type Integer) (local_closest :type Boolean) (local_remove :type Boolean) (local_replace :type Boolean))
  (bind _output (`|GetArrayItem` (`self.worker_actors`) (`local.local_index`)))
  ;[1 1 1] Set to add new worker to specific slot index.
  (set `local.local_worker` worker_actor)
  (set `local.local_index` slot_index)
  (set `local.local_replace` replace_existing)
  (set `local.local_closest` use_closest)
  (set `local.local_remove` remove_worker)
  (bind _is_valid (`self.get_worker` (`local.local_worker`)))
  (if _is_valid
    (if (`local.local_remove`)
      (`/Engine/EditorBlueprintResources/StandardMacros.IsValid` (`local.local_worker`)
        (:`Is Valid`
          (set `local.local_index` (`KismetArrayLibrary.Array_Find` (`self.worker_actors`) (`local.local_worker`))))
        (:`Is Not Valid`
          _))
      (if (>= (`local.local_index`) 0)
        (`/Engine/EditorBlueprintResources/StandardMacros.DecrementInt` (`self.workers_length`)
          (:`  `
            (`self.ed_worker_removed` (`local.local_index`) (`|GetArrayItem` (`self.worker_actors`) (`local.local_index`)) (`|GetArrayItem` (`self.work_points`) (`local.local_index`)) (`|GetArrayItem` (`self.nav_colliders`) (`local.local_index`)))
            (`KismetArrayLibrary.Array_Set` (`self.worker_actors`) (`local.local_index`))
            (`KismetArrayLibrary.Array_Set` (`self.nav_colliders`) (`local.local_index`))
            (bind (_return_node _workspace_reference) (`/Game/ai_component/base_system/blueprints/bp_easy_ai_library.easy_ai_get_workspace` (`local.local_worker`)))
            (if _return_node
              (`self.set_self_working` _workspace_reference null))
            (return true)))
        (else
          (return false)))
      (else
        (return false)))
    (elif (not (`local.local_remove`))
      (if (`local.local_closest`)
        (`/Engine/EditorBlueprintResources/StandardMacros.IsValid` (`local.local_worker`)
          (:`Is Valid`
            (bind (_is_valid_2 _found_index) (`self.get_closest_slot` (`local.local_worker`)))
            (if _is_valid_2
              (bind _is_success (`self.set_worker` (`local.local_worker`) _found_index))
              (return _is_success)
              (else
                _)))
          (:`Is Not Valid`
            _))
        (return false)
        (else
          (`/Engine/EditorBlueprintResources/StandardMacros.IsValid` _output
            (:`Is Valid`
              (if (`local.local_replace`)
                (`self.set_worker` _output 0 false false true)
                (bind _is_success_2 (`self.set_worker` (`local.local_worker`) (`local.local_index`) false (`local.local_closest`)))
                (return _is_success_2)
                (else
                  (return false))))
            (:`Is Not Valid`
              (`KismetArrayLibrary.Array_Set` (`self.worker_actors`) (`local.local_index`) (`local.local_worker`))
              (`/Engine/EditorBlueprintResources/StandardMacros.IncrementInt` (`self.workers_length`)
                (:`  `
                  (`self.ed_worker_added` (`local.local_index`) (`local.local_worker`) (`|GetArrayItem` (`self.work_points`) (`local.local_index`)))
                  (bind (_return_node_2 _workspace_reference_2) (`/Game/ai_component/base_system/blueprints/bp_easy_ai_library.easy_ai_get_workspace` (`local.local_worker`)))
                  (if _return_node_2
                    (`self.set_self_working` _workspace_reference_2 (`self.GetOwner`)))
                  (return true)))))))
      (else
        (return false)))))

(fn `set_working_condition`
  (params (can_work :type Boolean))
  ;[1 1 1] Working condition by default.
  (set `self.can_work` can_work))