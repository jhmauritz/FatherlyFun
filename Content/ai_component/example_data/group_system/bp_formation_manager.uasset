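; Formation helper for AI squads that computes per-unit destinations and measures groups.
; SetFormationDestination lays units out in a rotated box up to eight wide, using BoxFormation's row/column offset plus a median offset to center it on the target.
; Circle and custom offset-table formations are separate functions it does not call.
; Other queries derive group median and bounds from EasyAi unit locations and agent bounds, or find the unit nearest a location in XY.
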(fn `box_formation`
  (params (squad_index :type Integer) (squad_direction :type "Rotator Structure") (box_length :type Integer) (array_length :type Integer) (x_offset :type "Float (double-precision)") (y_offset :type "Float (double-precision)"))
  (returns (ReturnValue :type "Vector Structure") (median_offset :type "Vector Structure"))
  (locals (local_index :type Integer) (local_box_length :type Integer) (local_x_offset :type "Float (double-precision)") (local_y_offset :type "Float (double-precision)") (local_array_length :type Integer) (local_direction :type "Rotator Structure"))
  ;[1 1 1] Box formation.
  (set `local.local_index` squad_index)
  (set `local.local_direction` squad_direction)
  (set `local.local_box_length` box_length)
  (set `local.local_array_length` array_length)
  (set `local.local_x_offset` x_offset)
  (set `local.local_y_offset` y_offset)
  (return (+ (* (`KismetMathLibrary.GetForwardVector` (`local.local_direction`)) (* (/ (`local.local_index`) (`local.local_box_length`)) (`local.local_x_offset`))) (* (`KismetMathLibrary.GetRightVector` (`local.local_direction`)) (* (mod (`local.local_index`) (`local.local_box_length`)) (`local.local_y_offset`)))) (+ (/ (* (* (`KismetMathLibrary.GetForwardVector` (`local.local_direction`)) (* (`local.local_x_offset`) -1.0)) (- (`KismetMathLibrary.Conv_IntToDouble` (`KismetMathLibrary.Round` (/ (`KismetMathLibrary.Conv_IntToDouble` (`local.local_array_length`)) (`KismetMathLibrary.Conv_IntToDouble` (`local.local_box_length`))))) 1.0)) 2.0) (/ (* (* (`KismetMathLibrary.GetRightVector` (`local.local_direction`)) (* (`local.local_y_offset`) -1.0)) (- (`KismetMathLibrary.Conv_IntToDouble` (`local.local_box_length`)) 1.0)) 2.0))))

(fn `circle_formation`
  (params (circle_radius :type "Float (double-precision)") (squad_index :type Integer) (squad_length :type Integer))
  (returns (ReturnValue :type "Vector Structure"))
  ;[1 1 1] Circle formation logic.
  (return (* (`KismetMathLibrary.GetForwardVector` (`KismetMathLibrary.MakeRotator` 0.0 0.0 (`KismetMathLibrary.Conv_IntToDouble` (* squad_index (/ 360 squad_length))))) circle_radius)))

(fn `custom_formation`
  (params (squad_index :type Integer) (squad_direction :type "Rotator Structure") (squad_offset :type "Float (double-precision)"))
  (returns (ReturnValue :type "Vector Structure"))
  (locals (local_offsets_y :type "Array of Vector Structure") (local_index :type Integer) (local_length :type Integer))
  (bind _local_offsets_y (`local.local_offsets_y`))
  ;[1 1 1] Custom formation.
  (return (+ (* (`KismetMathLibrary.GetRightVector` squad_direction) (.x (`|GetArrayItem` _local_offsets_y (mod squad_index (`KismetArrayLibrary.Array_Length` _local_offsets_y))))) (* (`KismetMathLibrary.GetForwardVector` squad_direction) (.y (`|GetArrayItem` _local_offsets_y (mod squad_index (`KismetArrayLibrary.Array_Length` _local_offsets_y))))))))

(fn `get_closest_unit`
  (params (location :type "Vector Structure") (units :type "Array of Actor Object Reference"))
  (returns (ReturnValue :type Boolean) (closest_unit :type "Actor Object Reference"))
  (locals (local_units :type "Array of Actor Object Reference") (local_distance :type "Array of Float (double-precision)") (local_location :type "Vector Structure"))
  (bind _indexofminvalue (`KismetMathLibrary.MinOfFloatArray` (`local.local_distance`)))
  ;[1 1 1] Get closest unit to specific location.
  (set `local.local_location` location)
  (set `local.local_units` units)
  (if (`KismetArrayLibrary.Array_IsValidIndex` (`local.local_units`))
    (for _array_element (`local.local_units`)
      (`KismetArrayLibrary.Array_Add` (`local.local_distance`) (`KismetMathLibrary.VSizeXY` (- (`Actor.K2_GetActorLocation` _array_element) (`local.local_location`)))))
    (return (>= _indexofminvalue 0) (`|GetArrayItem` (`local.local_units`) _indexofminvalue))
    (else
      (return false null))))

(fn `get_group_average`
  (params (group_location :type "Array of Vector Structure") (group_bounds :type "Array of Vector Structure"))
  (returns (median_point :type "Vector Structure") (average_bounds :type "Vector Structure"))
  (locals (local_groups_location :type "Array of Vector Structure") (local_groups_bounds :type "Array of Vector Structure") (local_average_point :type "Vector Structure") (local_bounds_x :type "Array of Float (double-precision)") (local_bounds_y :type "Array of Float (double-precision)") (local_bounds_z :type "Array of Float (double-precision)") (local_bounds :type "Array of Vector Structure") (local_average_bounds :type "Vector Structure" :default (0.0 0.0 0.0)))
  ;[1 1 1] Get group average location and bounds by vector array.
  (set `local.local_groups_location` group_location)
  (set `local.local_groups_bounds` group_bounds)
  (set `local.local_average_point` (`KismetMathLibrary.GetVectorArrayAverage` (`local.local_groups_location`)))
  (for (_array_element _array_index) (`local.local_groups_location`)
    (`KismetArrayLibrary.Array_Add` (`local.local_bounds_x`) (.x (+ (- _array_element (`local.local_average_point`)) (`|GetArrayItem` (`local.local_groups_bounds`) _array_index))))
    (`KismetArrayLibrary.Array_Add` (`local.local_bounds_y`) (.y (+ (- _array_element (`local.local_average_point`)) (`|GetArrayItem` (`local.local_groups_bounds`) _array_index))))
    (`KismetArrayLibrary.Array_Add` (`local.local_bounds_z`) (.z (+ (- _array_element (`local.local_average_point`)) (`|GetArrayItem` (`local.local_groups_bounds`) _array_index)))))
  (set `local.local_average_bounds` (`KismetMathLibrary.MakeVector` (`KismetMathLibrary.FMax` (`.MaxValue` (`KismetMathLibrary.MaxOfFloatArray` (`local.local_bounds_x`))) (`KismetMathLibrary.Abs` (`.MinValue` (`KismetMathLibrary.MinOfFloatArray` (`local.local_bounds_x`))))) (`KismetMathLibrary.FMax` (`.MaxValue` (`KismetMathLibrary.MaxOfFloatArray` (`local.local_bounds_y`))) (`KismetMathLibrary.Abs` (`.MinValue` (`KismetMathLibrary.MinOfFloatArray` (`local.local_bounds_y`))))) (`KismetMathLibrary.FMax` (`.MaxValue` (`KismetMathLibrary.MaxOfFloatArray` (`local.local_bounds_z`))) (`KismetMathLibrary.Abs` (`.MinValue` (`KismetMathLibrary.MinOfFloatArray` (`local.local_bounds_z`)))))))
  (return (`local.local_average_point`) (`local.local_average_bounds`)))

(fn `get_group_median`
  (params (group_actors :type "Array of Actor Object Reference"))
  (returns (group_median :type "Vector Structure") (group_bounds :type "Vector Structure"))
  (locals (local_units_location :type "Array of Vector Structure") (local_units_bound :type "Array of Vector Structure") (local_group_location :type "Array of Vector Structure") (local_group_bounds :type "Array of Vector Structure") (local_group_list :type "Array of Actor Object Reference") (local_bounds :type "Vector Structure" :default (0.0 0.0 0.0)))
  ;[1 1 1] Get group median point and bounds.
  (set `local.local_group_list` group_actors)
  (for _array_element (`local.local_group_list`)
    (bind (_return_node _group_manager) (`/Game/ai_component/base_system/blueprints/bp_easy_ai_library.easy_ai_get_group` _array_element))
    (bind (_arrayindex _arrayelement) (`/Engine/EditorBlueprintResources/StandardMacros.ReverseForEachLoop` (`/Game/ai_component/example_data/group_system/bp_group_manager.current_units` _group_manager))
      (:`LoopBody`
        (`/Engine/EditorBlueprintResources/StandardMacros.IsValid` _arrayelement
          (:`Is Valid`
            (`KismetArrayLibrary.Array_Add` (`local.local_units_location`) (`Actor.K2_GetActorLocation` _arrayelement))
            (bind (_return_node_2 _ai_component) (`/Game/ai_component/base_system/blueprints/bp_easy_ai_library.easy_ai_get_component` _arrayelement))
            (`KismetArrayLibrary.Array_Add` (`local.local_units_bound`) (`.agent_bounds_5_558734884CB8F58A66714F8EA2C5A7FB` (break `/Game/ai_component/base_system/structs/01_base/s_ai_08_agent_settings` (`/Game/ai_component/base_system/blueprints/bp_easy_ai_pathfinder_component.ai_agent` _ai_component)))))))))
  (for _ (`local.local_group_list`)
    (bind (_median_point _average_bounds) (`self.get_group_average` (`local.local_units_location`) (`local.local_units_bound`)))
    (`KismetArrayLibrary.Array_Add` (`local.local_group_location`) _median_point)
    (`KismetArrayLibrary.Array_Add` (`local.local_group_bounds`) _average_bounds))
  (return (`KismetMathLibrary.GetVectorArrayAverage` (`local.local_group_location`)) (`KismetMathLibrary.GetVectorArrayAverage` (`local.local_group_bounds`))))

(fn `set_formation_destination`
  (params (squad_actors :type "Array of Actor Object Reference") (target_location :type "Vector Structure") (target_rotation :type "Rotator Structure"))
  (returns (return_points :type "Array of Vector Structure"))
  (locals (local_target :type "Vector Structure") (local_units :type "Array of Actor Object Reference") (local_rotation :type "Rotator Structure") (local_index :type Integer) (local_locations :type "Array of Vector Structure") (local_offset :type "Vector Structure" :default (0.0 0.0 0.0)) (local_median :type "Vector Structure" :default (0.0 0.0 0.0)))
  (bind _returnvalue (`KismetArrayLibrary.Array_Length` (`local.local_units`)))
  ;[1 1 1] Set formation target location
  (set `local.local_units` squad_actors)
  (set `local.local_target` target_location)
  (set `local.local_rotation` target_rotation)
  (for (_ _array_index) (`local.local_units`)
    (set `local.local_index` _array_index)
    (bind (_returnvalue_2 _median_offset) (`self.box_formation` (`local.local_index`) (`local.local_rotation`) (`KismetMathLibrary.Clamp` _returnvalue 1 8) _returnvalue 180.0 180.0))
    (set `local.local_offset` _returnvalue_2)
    (set `local.local_median` _median_offset)
    (`KismetArrayLibrary.Array_Add` (`local.local_locations`) (+ (`local.local_target`) (`local.local_offset`) (`local.local_median`))))
  (return (`local.local_locations`)))