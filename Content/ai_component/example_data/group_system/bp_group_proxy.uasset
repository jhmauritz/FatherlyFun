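; Group proxy actor that moves several merged squads as one formation toward a shared travel destination.
; It spawns a point actor per unit and follows a nav path, adjusting its speed by its distance to the nearest unit.
; A randomized timer lays the points out through the formation manager, using capsule traces against static obstacles.
; Each tick prunes invalid or reassigned units; the timer destroys the proxy when no groups or units remain.
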(event `self.ReceiveBeginPlay`
  ;[1 1 1] Proxy group logic,
  ; tick group movement for all unit members,
  ; as a merged squads, formation movement,
  ; beginplay is here.
)

(event `self.ReceiveTick`
  (params (DeltaSeconds :type "Float (single-precision)"))
  ;[1 1 1] Proxy group logic,
  ; tick group movement for all unit members,
  ; as a merged squads, formation movement,
  ; beginplay is here.
  (`self.refresh_units`)
  (`self.tick_proxy`)
  (`KismetSystemLibrary.DrawDebugSphere` (`self.K2_GetActorLocation`) 100.0 1 (struct :`R` 0.331302 :`G` 1.0 :`B` 0.950214 :`A` 1.0))
  (`KismetSystemLibrary.DrawDebugPoint` (`self.travel_destination`) 10.0 (struct :`R` 0.416667 :`G` 0.5 :`B` 0.25 :`A` 1.0) 1.0))

(fn `add_actual_unit`
  (params (actual_unit :type "Actor Object Reference") (remove_unit :type Boolean))
  (locals (local_unit :type "Actor Object Reference") (local_remove :type Boolean) (local_index :type Integer))
  ;[1 1 1] Add or remove actual unit from proxy formation.
  (set `local.local_unit` actual_unit)
  (set `local.local_remove` remove_unit)
  (set `local.local_index` (`KismetArrayLibrary.Array_Find` (`self.actual_units`) (`local.local_unit`)))
  (if (>= (`local.local_index`) 0)
    (if (`local.local_remove`)
      (`KismetArrayLibrary.Array_Remove` (`self.actual_units`) (`local.local_index`)))
    (elif (not (`local.local_remove`))
      (`KismetArrayLibrary.Array_Add` (`self.actual_units`) (`local.local_unit`)))))

(fn `arrow_travel`
  (locals (local_formation :type "Array of Vector Structure"))
  (bind _arrow_units (`self.arrow_units`))
  (bind (_outradius _outhalfheight) (`CapsuleComponent.GetScaledCapsuleSize` (`self.root_capsule`)))
  ;[1 1 1] Update arrow's location.
  (bind _return_points (`/Game/ai_component/example_data/group_system/bp_formation_manager.set_formation_destination` :`self` (`self.bp_formation_manager`) :`squad_actors` (`self.arrow_units`) :`target_location` (`SceneComponent.K2_GetComponentLocation` (`self.root_capsule`))))
  (set `local.local_formation` _return_points)
  (for (_array_element _array_index) (`local.local_formation`)
    (if (`KismetArrayLibrary.Array_IsValidIndex` _arrow_units _array_index)
      (bind (_outhit _returnvalue) (`KismetSystemLibrary.CapsuleTraceSingleForObjects` (`SceneComponent.K2_GetComponentLocation` (`self.root_capsule`)) _array_element (* _outradius 2.0) (* _outhalfheight 0.8) (`|MakeArray` "ObjectTypeQuery1" :!type "EObjectTypeQuery Enum") false (`|MakeArray` self :!type "Actor Object Reference")))
      (if _returnvalue
        (bind _output (`|GetArrayItem` _arrow_units _array_index))
        (`self.K2_SetActorLocation` _output (`KismetMathLibrary.MakeVector` (.x (`.Location` (`GameplayStatics.BreakHitResult` _outhit))) (.y (`.Location` (`GameplayStatics.BreakHitResult` _outhit))) (.z _array_element)) false false)
        (else
          (`self.K2_SetActorLocation` _output _array_element false false)))))
  (bind (_returnvalue_2 _closest_unit) (`/Game/ai_component/example_data/group_system/bp_formation_manager.get_closest_unit` (`self.bp_formation_manager`) (`self.K2_GetActorLocation`) (`self.actual_units`)))
  (if _returnvalue_2
    (set `self.distance_to_actor` (`KismetMathLibrary.VSizeXY` (- (`self.K2_GetActorLocation` _closest_unit) (`self.K2_GetActorLocation`))))))

(fn `check_location`
  (params (unit_actor :type "Actor Object Reference"))
  (returns (ReturnValue :type Boolean))
  (locals (local_success :type Boolean))
  ;[1 1 1] Confirm that all units are in the place.
  (`|ExecutionSequence`
    (:`then_0`
      (bind (_is_valid _found_index _point_actor) (`self.find_actual_unit` unit_actor))
      (if _is_valid
        (bind (_return_node _ai_component) (`/Game/ai_component/base_system/blueprints/bp_easy_ai_library.easy_ai_get_component` unit_actor))
        (if _return_node
          (set `local.local_success` (== (`/Game/ai_component/base_system/blueprints/bp_easy_ai_pathfinder_component.ai_get_agent_location` _ai_component) (`NavigationSystemV1.K2_ProjectPointToNavigation` (`self.K2_GetActorLocation` _point_actor) null null (50.0 50.0 100.0)) :`ErrorTolerance` 50.0)))))
    (:`then_1`
      (return (`local.local_success`)))))

(fn `check_units_at_location`
  (returns (ReturnValue :type Boolean))
  (locals (local_fail :type Boolean))
  ;[1 1 1] Confirm that all units are in the place.
  (bind (_arrayindex _arrayelement) (`/Engine/EditorBlueprintResources/StandardMacros.ReverseForEachLoop` (`self.actual_units`))
    (:`LoopBody`
      (bind _returnvalue (`self.check_location` _arrayelement))
      (if (not _returnvalue)
        (set `local.local_fail` true)))
    (:`Completed`
      (return (not (`local.local_fail`))))))

(fn `find_actual_unit`
  (params (unit_actor :type "Actor Object Reference"))
  (returns (is_valid :type Boolean) (found_index :type Integer) (point_actor :type "/Game/ai_component/example_data/group_system/bp_group_point Object Reference"))
  (locals (local_unit :type "Actor Object Reference"))
  (bind _returnvalue (`KismetArrayLibrary.Array_Find` (`self.actual_units`) (`local.local_unit`)))
  ;[1 1 1] Find unit actor by ref.
  (set `local.local_unit` unit_actor)
  (if (>= _returnvalue 0)
    (return true _returnvalue (`|GetArrayItem` (`self.arrow_units`) _returnvalue))
    (else
      (return false 0 null))))

(fn `init_proxy`
  (params (group_list :type "Array of /Game/ai_component/example_data/group_system/bp_group_manager Object Reference") (travel_destination :type "Vector Structure"))
  (locals (local_group :type "/Game/ai_component/example_data/group_system/bp_group_manager Object Reference") (local_units :type "Array of Actor Object Reference"))
  ;[1 1 1] Init proxy and engage movement.
  (set `self.group_list` group_list)
  (set `self.travel_destination` travel_destination)
  (`|ExecutionSequence`
    (:`then_0`
      (`KismetArrayLibrary.Array_Clear` (`self.persistent_units`))
      (bind (_arrayindex _arrayelement) (`/Engine/EditorBlueprintResources/StandardMacros.ReverseForEachLoop` (`self.arrow_units`))
        (:`LoopBody`
          (`self.K2_DestroyActor` _arrayelement))
        (:`Completed`
          (`KismetArrayLibrary.Array_Clear` (`self.arrow_units`)))))
    (:`then_1`
      (for _array_element (`self.group_list`)
        (set `local.local_group` _array_element)
        (`/Game/ai_component/example_data/group_system/bp_group_manager.assign_proxy` (`local.local_group`) self)
        (set `local.local_units` (`/Game/ai_component/example_data/group_system/bp_group_manager.current_units` (`local.local_group`)))
        (`KismetArrayLibrary.Array_Append` (`self.persistent_units`) (`local.local_units`)))
      (`|ExecutionSequence`
        (:`then_0`
          (set `self.actual_units` (`self.persistent_units`))
          (for _ (`self.actual_units`)
            (bind _returnvalue (`AddComponent|NODE_AddChildActorComponent-4` :`bManualAttachment` true))
            (bind _asbp_group_point (cast `/Game/ai_component/example_data/group_system/bp_group_point` (`ChildActorComponent.ChildActor` _returnvalue)))
            (`KismetArrayLibrary.Array_Add` (`self.arrow_units`) _asbp_group_point)))
        (:`then_1`
          (set `self.proxy_traveling` true)
          (`self.set_proxy_location` false)
          (bind _nav_path (`/Game/ai_component/base_system/blueprints/bp_easy_ai_pathfinder_component.ai_set_travel` (`self.bp_easy_ai_pathfinder_component`) (make `/Game/ai_component/base_system/structs/01_base/s_ai_05_travel` null (`self.travel_destination`) (`KismetMathLibrary.MakeVector` 500.0 500.0 250.0) (struct) 0.0 0.0 0.0 false false false false "p_proxy")))
          (set `self.current_path` _nav_path)
          (`self.set_movement_timer`))))))

(fn `proxy_destroy`
  ;[1 1 1] Safe destroying proxy actor.
  (`KismetSystemLibrary.K2_ClearTimer` null "set_movement_timer")
  (`self.K2_DestroyActor`))

(fn `refresh_units`
  (bind _arrow_units (`self.arrow_units`))
  ;[1 1 1] Clean destroyed units from proxy update list.
  (bind (_arrayindex _arrayelement) (`/Engine/EditorBlueprintResources/StandardMacros.ReverseForEachLoop` (`self.actual_units`))
    (:`LoopBody`
      (`/Engine/EditorBlueprintResources/StandardMacros.IsValid` _arrayelement
        (:`Is Valid`
          (bind (_return_node _unit_reference) (`/Game/ai_component/base_system/blueprints/bp_easy_ai_library.easy_ai_get_unit` _arrayelement))
          (if _return_node
            (if (== (`/Game/ai_component/example_data/group_system/bp_group_manager.group_proxy` (`/Game/ai_component/example_data/group_system/bp_unit_component.group_manager` _unit_reference)) self)
              (if (not (`KismetArrayLibrary.Array_IsValidIndex` _arrow_units _arrayindex))
                (bind _returnvalue (`AddComponent|NODE_AddChildActorComponent-5` :`bManualAttachment` true))
                (bind _asbp_group_point (cast `/Game/ai_component/example_data/group_system/bp_group_point` (`ChildActorComponent.ChildActor` _returnvalue)))
                (`KismetArrayLibrary.Array_Set` (`self.arrow_units`) _arrayindex _asbp_group_point true))
              (else
                (`self.K2_DestroyActor` (`|GetArrayItem` _arrow_units _arrayindex) :!label _label)
                (`KismetArrayLibrary.Array_Remove` _arrow_units _arrayindex)
                (`KismetArrayLibrary.Array_Remove` (`self.actual_units`) _arrayindex)))))
        (:`Is Not Valid`
          (goto _label))))))

(fn `set_movement_timer`
  ;[1 1 1] Update proxy movement by timer.
  (if (and (`KismetArrayLibrary.Array_IsValidIndex` (`self.group_list`)) (`KismetArrayLibrary.Array_IsValidIndex` (`self.actual_units`)))
    (`self.arrow_travel`)
    (`KismetSystemLibrary.K2_SetTimer` null "set_movement_timer" (`/Game/ai_component/base_system/blueprints/bp_easy_ai_library.easy_ai_timer_randomizer` (`self.timer_movement_base`) (`self.timer_movement_random`)))
    (else
      (`self.proxy_destroy`))))

(fn `set_proxy_location`
  (params (update_direction :type Boolean))
  (locals (local_recast :type "RecastNavMesh Object Reference") (local_target_location :type "Vector Structure" :default (0.0 0.0 0.0)) (local_direction :type Boolean) (local_closest_unit :type "Vector Structure" :default (0.0 0.0 0.0)) (local_bounds :type "Vector Structure"))
  (bind _returnvalue (`KismetMathLibrary.MakeVector` 0.0 0.0 (`CapsuleComponent.GetScaledCapsuleHalfHeight` (`self.root_capsule`))))
  (bind _returnvalue_2 (+ (`local.local_target_location`) (* (`KismetMathLibrary.GetDirectionUnitVector` (`local.local_target_location`) (`self.travel_destination`)) (* (`KismetMathLibrary.FMax` (.x (`local.local_bounds`)) (.y (`local.local_bounds`))) 1.05))))
  (bind (_projectedlocation _returnvalue_3) (`NavigationSystemV1.K2_ProjectPointToNavigation` _returnvalue_2 (`local.local_recast`) null (5.0 5.0 250.0)))
  ;[1 1 1] Set to find correct proxy location.
  (set `local.local_direction` update_direction)
  (bind (_returnvalue_4 _closest_unit) (`/Game/ai_component/example_data/group_system/bp_formation_manager.get_closest_unit` (`self.bp_formation_manager`) (`self.travel_destination`) (`self.actual_units`)))
  (if _returnvalue_4
    (bind (_return_node _ai_component) (`/Game/ai_component/base_system/blueprints/bp_easy_ai_library.easy_ai_get_component` _closest_unit))
    (set `local.local_bounds` (`.agent_bounds_5_558734884CB8F58A66714F8EA2C5A7FB` (break `/Game/ai_component/base_system/structs/01_base/s_ai_08_agent_settings` (`/Game/ai_component/base_system/blueprints/bp_easy_ai_pathfinder_component.ai_agent` _ai_component))))
    (set `local.local_closest_unit` (`self.K2_GetActorLocation` _closest_unit)))
  (if (<= (`KismetMathLibrary.VSizeXY` (- (`local.local_target_location`) (`self.travel_destination`))) 100.0)
    (set `local.local_target_location` (`self.travel_destination`))
    (else
      (set `local.local_target_location` (`local.local_closest_unit`))))
  (bind _recast_data (`/Game/ai_component/base_system/blueprints/bp_easy_ai_pathfinder_component.ai_get_agent_recast` (`self.bp_easy_ai_pathfinder_component`) false "NewEnumerator0"))
  (set `local.local_recast` _recast_data)
  (if (`local.local_direction`)
    (`/Engine/EditorBlueprintResources/StandardMacros.IsValid` (`self.current_path`)
      (:`Is Valid`
        (if (`KismetArrayLibrary.Array_IsValidIndex` (`NavigationPath.PathPoints` (`self.current_path`)) 1)
          (set `local.local_target_location` (`KismetMathLibrary.VLerp` (`self.K2_GetActorLocation`) (`|GetArrayItem` (`NavigationPath.PathPoints` (`self.current_path`)) 1) 0.5))))
      (:`Is Not Valid`
        _)))
  (if _returnvalue_3
    (`self.K2_SetActorLocation` (+ _projectedlocation _returnvalue))
    (else
      (`self.K2_SetActorLocation` (+ _returnvalue_2 _returnvalue)))))

(fn `tick_proxy`
  ;[1 1 1] Tick movement for self and all units.
  (if (`self.proxy_traveling`)
    (bind (_movement_status _is_movement _is_destination _agent_speed _agent_dir _agent_loc _target_loc _target_rot _path_length _target_distance) (`/Game/ai_component/base_system/blueprints/bp_easy_ai_pathfinder_component.ai_travel_status` (`self.bp_easy_ai_pathfinder_component`)))
    (set `self.is_moving` _is_movement)
    (if (`self.is_moving`)
      (if (`KismetArrayLibrary.Array_IsValidIndex` (`self.actual_units`))
        (bind (_return_node _unit_reference) (`/Game/ai_component/base_system/blueprints/bp_easy_ai_library.easy_ai_get_unit` (`|GetArrayItem` (`self.actual_units`))))
        (if _return_node
          (`self.K2_SetActorLocation` (+ (* _agent_dir (* (`KismetMathLibrary.SelectFloat` (`KismetMathLibrary.MapRangeClamped` _target_distance 100.0 0.0 1.0) 1.0 _is_destination) (* (`self.proxy_current_speed`) (`GameplayStatics.GetWorldDeltaSeconds`)))) (`self.K2_GetActorLocation`)))
          (bind _unit_speed (`/Game/ai_component/example_data/group_system/bp_unit_component.unit_speed` _unit_reference))
          (set `self.proxy_current_speed` (`KismetMathLibrary.MapRangeClamped` (`self.distance_to_actor`) 1000.0 500.0 (* _unit_speed 0.7) (* _unit_speed 1.2))))))))

(fn `update_proxy`
  (params (travel_destination :type "Vector Structure"))
  ;[1 1 1] Send to new location the same proxy.
  (set `self.travel_destination` travel_destination)
  (`self.set_proxy_location` false)
  (bind _nav_path (`/Game/ai_component/base_system/blueprints/bp_easy_ai_pathfinder_component.ai_set_travel` (`self.bp_easy_ai_pathfinder_component`) (make `/Game/ai_component/base_system/structs/01_base/s_ai_05_travel` null (`self.travel_destination`) (`KismetMathLibrary.MakeVector` 500.0 500.0 250.0) (struct) 0.0 0.0 0.0 true false false false "p_proxy")))
  (set `self.current_path` _nav_path)
  (`self.set_proxy_location` true)
  (`self.set_movement_timer`))

(fn `UserConstructionScript`)