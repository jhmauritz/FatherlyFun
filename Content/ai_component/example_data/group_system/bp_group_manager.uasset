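; Group manager actor that holds a squad of AI units, registers them with a faction and relays selection and highlighting.
; Once the AI system loads, it sets the faction and can auto-spawn units in box formation.
; Randomized timers, which spread performance cost, send units toward their points on a shared group proxy and destroy the proxy once it stops moving.
; Tick prunes invalid units, destroys the empty group and optionally draws debug bounds.
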(event `self.ReceiveBeginPlay`
  ;[1 1 1] Unit manager's beginplay is here.
  (`/Game/ai_component/base_system/blueprints/bp_easy_ai_macro_library.easy_ai_is_loaded` ; macro to wait until AI system is loaded.
    (:`success`
      (if (not (`self.group_loaded`))
        (`self.init_group` (`self.faction_index`))))))

(event `self.ReceiveTick`
  (params (DeltaSeconds :type "Float (single-precision)"))
  ;[1 1 1] Unit manager's beginplay is here.
  (if (`self.group_loaded`)
    (`self.refresh_units`)
    (if (`self.debug_bounds`)
      (bind (_center _boxextent) (`GameplayStatics.GetActorArrayBounds` (`self.current_units`) true))
      (`KismetSystemLibrary.DrawDebugBox` _center _boxextent (struct :`R` 1.0 :`G` 1.0 :`B` 1.0 :`A` 1.0) (struct) 0.0 5.0))))

(fn `add_units`
  (params (new_units :type "Array of Actor Object Reference") (clear_existing :type Boolean))
  (locals (local_units :type "Array of Actor Object Reference") (local_clear :type Boolean))
  ;[1 1 1] Add new units to this unit stack.
  (set `local.local_units` new_units)
  (set `local.local_clear` clear_existing)
  (`/Engine/EditorBlueprintResources/StandardMacros.IsValid` (`self.faction_reference`)
    (:`Is Valid`
      (if (`local.local_clear`)
        (`self.clear_units`)
        (else
          (for _array_element (`local.local_units`)
            (`self.set_unit` _array_element))
          (for _array_element_2 (`local.local_units`)
            (bind (_return_node _unit_reference) (`/Game/ai_component/base_system/blueprints/bp_easy_ai_library.easy_ai_get_unit` _array_element_2))
            (`/Game/ai_component/example_data/group_system/bp_unit_component.ed_group_loaded` _unit_reference)))))))

(fn `assign_proxy`
  (params (new_proxy :type "/Game/ai_component/example_data/group_system/bp_group_proxy Object Reference"))
  (locals (local_proxy :type "/Game/ai_component/example_data/group_system/bp_group_proxy Object Reference"))
  ;[1 1 1] Assign group proxy movement.
  (set `local.local_proxy` new_proxy)
  (`/Engine/EditorBlueprintResources/StandardMacros.IsValid` (`self.group_proxy`)
    (:`Is Valid`
      (`self.remove_proxy`))
    (:`Is Not Valid`
      _))
  (set `self.group_proxy` (`local.local_proxy`))
  (set `self.new_proxy` true)
  (if (not (`KismetSystemLibrary.K2_IsTimerActive` null "check_movement_timer"))
    (`KismetSystemLibrary.K2_SetTimer` null "check_movement_timer" (`/Game/ai_component/base_system/blueprints/bp_easy_ai_library.easy_ai_timer_randomizer` (`self.group_timer_base`) (`self.group_timer_random`)))))

(fn `check_movement_stop`
  ;[1 1 1] Movement stop logic.
  (`KismetSystemLibrary.K2_SetTimer` null "check_movement_timer" (`/Game/ai_component/base_system/blueprints/bp_easy_ai_library.easy_ai_timer_randomizer` (`self.group_timer_base`) (`self.group_timer_random`)))
  (`/Engine/EditorBlueprintResources/StandardMacros.IsValid` (`self.group_proxy`)
    (:`Is Valid`
      (if (not (`/Game/ai_component/example_data/group_system/bp_group_proxy.is_moving` (`self.group_proxy`)))
        (`/Game/ai_component/example_data/group_system/bp_group_proxy.proxy_destroy` (`self.group_proxy`))
        (`KismetSystemLibrary.K2_ClearTimer` null "check_movement_timer")
        (`KismetSystemLibrary.K2_ClearTimer` null "check_movement_stop")))))

(fn `check_movement_timer`
  (locals (local_unit :type "Actor Object Reference") (local_ai_data :type "/Game/ai_component/base_system/blueprints/bp_easy_ai_pathfinder_component Object Reference"))
  (bind ((`current_path_2_CFBB136745EC78C10A89DF85D69DA9C7` _current_path) (`path_message_35_14BC9E984F3CC11A8F1203A51D17F0A2` _path_message)) (break `/Game/ai_component/base_system/structs/01_base/s_ai_02_nav` (`/Game/ai_component/base_system/blueprints/bp_easy_ai_pathfinder_component.ai_path` (`local.local_ai_data`))))
  ;[1 1 1] Check group movement by timer logic, always random value to prevent performance drop.
  (`/Engine/EditorBlueprintResources/StandardMacros.IsValid` (`self.group_proxy`)
    (:`Is Valid`
      (if (`KismetArrayLibrary.Array_IsValidIndex` (`self.current_units`))
        (bind (_arrayindex _arrayelement) (`/Engine/EditorBlueprintResources/StandardMacros.ReverseForEachLoop` (`self.current_units`))
          (:`LoopBody`
            (set `local.local_unit` _arrayelement)
            (bind (_return_node _ai_component) (`/Game/ai_component/base_system/blueprints/bp_easy_ai_library.easy_ai_get_component` (`local.local_unit`)))
            (if _return_node
              (set `local.local_ai_data` _ai_component)
              (bind (_is_valid _found_index _point_actor) (`/Game/ai_component/example_data/group_system/bp_group_proxy.find_actual_unit` (`self.group_proxy`) (`local.local_unit`)))
              (if _is_valid
                (if (`self.new_proxy`)
                  (bind _returnvalue (!= _current_path _point_actor))
                  (`/Game/ai_component/base_system/blueprints/bp_easy_ai_pathfinder_component.ai_set_travel` (`local.local_ai_data`) (make `/Game/ai_component/base_system/structs/01_base/s_ai_05_travel` (`Actor.RootComponent` _point_actor) (0.0 0.0 0.0) (0.0 0.0 0.0) (struct) 0.0 0.0 0.0 _returnvalue false true false "g_proxy") :!label _label)
                  (else
                    (switch `name` _path_message
                      (:`None`
                        (goto _label))
                      (:`g_proxy`
                        (if _returnvalue
                          (goto _label)))))))))
          (:`Completed`
            (`KismetSystemLibrary.K2_SetTimer` null "check_movement_stop" (`self.group_timer_stop`))
            (set `self.new_proxy` false)))
        (else
          (`KismetSystemLibrary.K2_ClearTimer` null "check_movement_timer" :!label _label_2)
          (`KismetSystemLibrary.K2_ClearTimer` null "check_movement_stop"))))
    (:`Is Not Valid`
      (goto _label_2))))

(fn `clear_units`
  ;[1 1 1] Clear all units.
  (bind (_arrayindex _arrayelement) (`/Engine/EditorBlueprintResources/StandardMacros.ReverseForEachLoop` (`self.current_units`))
    (:`LoopBody`
      (`self.set_unit` _arrayelement true))))

(fn `get_unit`
  (params (unit_actor :type "Actor Object Reference"))
  (returns (ReturnValue :type Boolean) (found_index :type Integer))
  (bind _returnvalue (`KismetArrayLibrary.Array_Find` (`self.current_units`) unit_actor))
  ;[1 1 1] Find existing unit in the stack.
  (return (>= _returnvalue 0) _returnvalue))

(fn `highlight_group`
  (params (remove :type Boolean))
  ;[1 1 1] Highlight whole group logic.
  (for _array_element (`self.current_units`)
    (bind (_return_node _unit_reference) (`/Game/ai_component/base_system/blueprints/bp_easy_ai_library.easy_ai_get_unit` _array_element))
    (if _return_node
      (`/Game/ai_component/example_data/group_system/bp_unit_component.receive_highlight` _unit_reference remove))))

(fn `init_group`
  (params (faction_index :type Integer))
  ;[1 1 1] Init group logic,
  ; set group faction, and autospawn units if enabled.
  (`|ExecutionSequence`
    (:`then_0`
      (`self.set_group_faction` faction_index)
      (`/Engine/EditorBlueprintResources/StandardMacros.IsValid` (`self.faction_reference`)
        (:`Is Valid`
          (if (`self.auto_spawn_units`)
            (`self.spawn_units` (`self.units_count`) (`self.unit_class`))))))
    (:`then_1`
      (set `self.group_loaded` true))))

(fn `refresh_units`
  ;[1 1 1] Refresh and unregister unexisting units.
  (bind (_arrayindex _arrayelement) (`/Engine/EditorBlueprintResources/StandardMacros.ReverseForEachLoop` (`self.current_units`))
    (:`LoopBody`
      (`/Engine/EditorBlueprintResources/StandardMacros.IsValid` _arrayelement ; remove destroyed units from group list.
        (:`Is Not Valid`
          (`KismetArrayLibrary.Array_Remove` (`self.current_units`) _arrayindex))))
    (:`Completed`
      (if (not (`KismetArrayLibrary.Array_IsValidIndex` (`self.current_units`)))
        (`self.K2_DestroyActor`) ; if no units in loaded group\nthen destroy group.
      ))))

(fn `remove_proxy`
  (returns (latest_proxy_location :type "Vector Structure") (return_node :type Boolean))
  (locals (local_proxy :type "Vector Structure" :default (0.0 0.0 0.0)))
  (bind _returnvalue (`KismetArrayLibrary.Array_Find` (`/Game/ai_component/example_data/group_system/bp_group_proxy.group_list` (`self.group_proxy`)) self))
  ;[1 1 1] Remove any existing proxy movement.
  (`/Engine/EditorBlueprintResources/StandardMacros.IsValid` (`self.group_proxy`)
    (:`Is Valid`
      (if (>= _returnvalue 0)
        (`KismetArrayLibrary.Array_Remove` (`/Game/ai_component/example_data/group_system/bp_group_proxy.group_list` (`self.group_proxy`)) _returnvalue)
        (set `local.local_proxy` (`self.K2_GetActorLocation` (`self.group_proxy`)))
        (set `self.group_proxy` null)
        (return (`local.local_proxy`) true)
        (else
          (return (0.0 0.0 0.0) false))))
    (:`Is Not Valid`
      (return (0.0 0.0 0.0) false))))

(fn `select_group`
  (params (selection_removed :type Boolean))
  ;[1 1 1] Group selection func.
  (for _array_element (`self.current_units`)
    (bind (_return_node _unit_reference) (`/Game/ai_component/base_system/blueprints/bp_easy_ai_library.easy_ai_get_unit` _array_element))
    (if _return_node
      (`/Game/ai_component/example_data/group_system/bp_unit_component.receive_selection` _unit_reference selection_removed))))

(fn `set_group_faction`
  (params (faction_index :type Integer))
  (locals (local_faction :type Integer))
  ;[1 1 1] Set units faction.
  (set `local.local_faction` faction_index)
  (`|ExecutionSequence`
    (:`then_0`
      (set `self.faction_index` (`local.local_faction`))
      (bind (_return_node _faction_reference) (`/Game/ai_component/example_data/faction_system/bp_faction_link.set_owner_faction` (`self.bp_faction_link`) (`local.local_faction`)))
      (if _return_node
        (set `self.faction_reference` _faction_reference)
        (`/Game/ai_component/example_data/faction_system/bp_faction_manager.register_groups` (`self.faction_reference`) false self)))
    (:`then_1`
      (for _array_element (`self.current_units`)
        (bind (_return_node_2 _faction_link) (`/Game/ai_component/base_system/blueprints/bp_easy_ai_library.easy_ai_get_faction_link` _array_element))
        (`/Game/ai_component/example_data/faction_system/bp_faction_link.set_owner_faction` _faction_link (`self.faction_index`))))))

(fn `set_unit`
  (params (unit_actor :type "Actor Object Reference") (remove_unit :type Boolean))
  (locals (local_unit :type "Actor Object Reference") (local_remove :type Boolean))
  ;[1 1 1] Set new unit to stack.
  (set `local.local_unit` unit_actor)
  (set `local.local_remove` remove_unit)
  (bind (_returnvalue _found_index) (`self.get_unit` (`local.local_unit`)))
  (if _returnvalue
    (if (`local.local_remove`)
      (`KismetArrayLibrary.Array_Remove` (`self.current_units`) _found_index)
      (bind (_return_node _unit_reference) (`/Game/ai_component/base_system/blueprints/bp_easy_ai_library.easy_ai_get_unit` (`local.local_unit`)))
      (if _return_node
        (`/Game/ai_component/example_data/group_system/bp_unit_component.init_unit` _unit_reference self (`self.faction_index`) true)
        (`/Game/ai_component/example_data/faction_system/bp_faction_manager.register_units` (`self.faction_reference`) true (`local.local_unit`))
        (`/Engine/EditorBlueprintResources/StandardMacros.IsValid` (`self.group_proxy`)
          (:`Is Valid`
            (`/Game/ai_component/example_data/group_system/bp_group_proxy.add_actual_unit` (`self.group_proxy`) (`local.local_unit`) true)))))
    (elif (not (`local.local_remove`))
      (`KismetArrayLibrary.Array_Add` (`self.current_units`) (`local.local_unit`))
      (bind (_return_node_2 _unit_reference_2) (`/Game/ai_component/base_system/blueprints/bp_easy_ai_library.easy_ai_get_unit` (`local.local_unit`)))
      (if _return_node_2
        (`/Game/ai_component/example_data/group_system/bp_unit_component.init_unit` _unit_reference_2 self (`self.faction_index`) false)
        (`/Game/ai_component/example_data/faction_system/bp_faction_manager.register_units` (`self.faction_reference`) false (`local.local_unit`))
        (`/Engine/EditorBlueprintResources/StandardMacros.IsValid` (`self.group_proxy`)
          (:`Is Valid`
            (`/Game/ai_component/example_data/group_system/bp_group_proxy.add_actual_unit` (`self.group_proxy`) (`local.local_unit`) false)))))))

(fn `spawn_units`
  (params (spawn_count :type Integer) (unit_class :type "Actor Class Reference"))
  (locals (local_units :type "Array of Actor Object Reference") (local_count :type Integer) (local_class :type "Actor Class Reference") (local_transform :type "Transform Structure"))
  (bind _unit_health (`self.unit_health`))
  (bind _rotation (.rotation (`SceneComponent.K2_GetComponentToWorld` (`self.spawn_point`))))
  ;[1 1 1] Spawn units from class.
  (set `local.local_count` spawn_count)
  (set `local.local_class` unit_class)
  (for _index (range (`local.local_count`))
    (bind (_returnvalue _median_offset) (`/Game/ai_component/example_data/group_system/bp_formation_manager.box_formation` (`self.bp_formation_manager`) _index _rotation (`KismetMathLibrary.Clamp` (`local.local_count`) 1 8) (`local.local_count`) 100.0 100.0))
    (set `local.local_transform` (`KismetMathLibrary.MakeTransform` (+ _returnvalue _median_offset (.location (`SceneComponent.K2_GetComponentToWorld` (`self.spawn_point`)))) _rotation (.scale (`SceneComponent.K2_GetComponentToWorld` (`self.spawn_point`)))))
    (bind _returnvalue_2 (`|SpawnActorFromClass` (`local.local_class`) (`local.local_transform`) "AdjustIfPossibleButAlwaysSpawn" "SelectDefaultAtRuntime" null null))
    (`self.set_unit` _returnvalue_2)
    (`KismetArrayLibrary.Array_Add` (`local.local_units`) _returnvalue_2)
    (bind _returnvalue_3 (`self.GetComponentByClass` _returnvalue_2 "/Game/ai_component/example_data/group_system/bp_health_component.bp_health_component_C"))
    (`/Engine/EditorBlueprintResources/StandardMacros.IsValid` _returnvalue_3
      (:`Is Valid`
        (set `/Game/ai_component/example_data/group_system/bp_health_component.current_health` _unit_health _returnvalue_3)
        (set `/Game/ai_component/example_data/group_system/bp_health_component.max_health` _unit_health _returnvalue_3))))
  (`self.add_units` (`local.local_units`)))

(fn `UserConstructionScript`)