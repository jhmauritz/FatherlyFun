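; Actor component that makes its owner a unit in the group system, handling group membership, faction, selection and movement.
; After a short BeginPlay delay, an ungrouped unit spawns its own group manager using its faction, since selection requires a group.
; InitUnit stores or clears the group reference and applies the faction.
; Selection, hover, highlight and init calls fire event dispatchers, while UnitMove sends travel targets to the AI component.
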(event `self.ReceiveBeginPlay`
  ;[1 1 1] Unit component,
  ; Beginplay is here.
  (`KismetSystemLibrary.Delay` 0.2) ; delay to let groups and factions to be loaded.
  (`/Engine/EditorBlueprintResources/StandardMacros.IsValid` (`self.group_manager`)
    (:`Is Not Valid`
      (bind _returnvalue (`|SpawnActorFromClass` "/Game/ai_component/example_data/group_system/bp_group_manager.bp_group_manager_C" (`Actor.GetTransform` (`self.GetOwner`)) "AlwaysSpawn" "OverrideRootScale" null null))
      (bind (_return_node _faction_link) (`/Game/ai_component/base_system/blueprints/bp_easy_ai_library.easy_ai_get_faction_link` (`self.GetOwner`)))
      (if _return_node
        (`/Game/ai_component/example_data/group_system/bp_group_manager.init_group` _returnvalue (`/Game/ai_component/example_data/faction_system/bp_faction_link.faction_index` _faction_link)) ; init the group with faction\nsame as units.
        (`/Game/ai_component/example_data/group_system/bp_group_manager.add_units` _returnvalue (`|MakeArray` (`self.GetOwner`)) false)))))

(event `self.ReceiveTick`
  (params (DeltaSeconds :type "Float (single-precision)"))
  ;[1 1 1] Unit component,
  ; Beginplay is here.
)

(fn `get_faction_info`
  (returns (faction_data :type "/Game/ai_component/example_data/faction_system/s_faction_data Structure") (faction_index :type Integer))
  ;[1 1 1] Get unit's faction info.
  (bind (_return_node _faction_reference) (`/Game/ai_component/base_system/blueprints/bp_easy_ai_library.easy_ai_get_faction_manager` (`self.GetOwner`)))
  (if _return_node
    (return (`/Game/ai_component/example_data/faction_system/bp_faction_manager.faction_data` _faction_reference) (`/Game/ai_component/example_data/faction_system/bp_faction_manager.faction_index` _faction_reference))
    (else
      (return (struct) -1))))

(fn `get_group_info`
  (returns (is_group :type Boolean) (group_actor :type "/Game/ai_component/example_data/group_system/bp_group_manager Object Reference"))
  ;[1 1 1] Get unit member actor as self,
  ; group or single if there is no group.
  (`/Engine/EditorBlueprintResources/StandardMacros.IsValid` (`self.group_manager`)
    (:`Is Valid`
      (return true (`self.group_manager`)))
    (:`Is Not Valid`
      (return false null))))

(fn `init_unit`
  (params (group_reference :type "/Game/ai_component/example_data/group_system/bp_group_manager Object Reference") (faction_index :type Integer) (is_removed :type Boolean))
  (locals (local_removed :type Boolean) (local_manager :type Boolean) (local_faction_index :type Integer))
  (bind _returnvalue (`Actor.GetComponentByClass` (`self.GetOwner`) "/Game/ai_component/example_data/faction_system/bp_faction_link.bp_faction_link_C"))
  ;[1 1 1] Init the unit link to the component.
  (set `self.group_manager` group_reference)
  (set `local.local_faction_index` faction_index)
  (set `local.local_removed` is_removed)
  (`|ExecutionSequence`
    (:`then_0`
      (if (`local.local_removed`)
        (set `self.group_manager` null)
        (else
          (`/Engine/EditorBlueprintResources/StandardMacros.IsValid` _returnvalue
            (:`Is Valid`
              (`/Game/ai_component/example_data/faction_system/bp_faction_link.set_owner_faction` _returnvalue (`local.local_faction_index`)))))))
    (:`then_1`
      (`self.ed_init`))))

(fn `receive_highlight`
  (params (selection_removed :type Boolean))
  (locals (local_removed :type Boolean))
  ;[1 1 1] Receive highlight logic.
  (set `local.local_removed` selection_removed)
  (`self.ed_highlight` (`local.local_removed`)))

(fn `receive_hover`
  (params (hover_removed :type Boolean))
  ;[1 1 1] Unit receive hover logic.
  (`self.ed_hover` hover_removed))

(fn `receive_selection`
  (params (selection_removed :type Boolean))
  (locals (local_removed :type Boolean))
  ;[1 1 1] Receive selection for unit.
  (set `local.local_removed` selection_removed)
  (`self.ed_selection` (`local.local_removed`)))

(fn `unit_move`
  (params (location :type "Vector Structure"))
  ;[1 1 1] Move this speicfic unit.
  (bind (_return_node _ai_component) (`/Game/ai_component/base_system/blueprints/bp_easy_ai_library.easy_ai_get_component` (`self.GetOwner`)))
  (`/Game/ai_component/base_system/blueprints/bp_easy_ai_pathfinder_component.ai_set_travel` _ai_component (make `/Game/ai_component/base_system/structs/01_base/s_ai_05_travel` null location (100.0 100.0 250.0))))