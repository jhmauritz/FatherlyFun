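; Health component Blueprint from the AI component group system example that tracks an actor's current health and drives its HP widget.
; UpdateHp adds or subtracts the absolute amount based on a remove flag, clamps it between zero and max health, refreshes the widget and returns the result.
; SetWidget stores an HP widget and initializes it with faction color and index.
; UpdateWidget feeds it health normalized to a 0–1 range.
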(fn `set_widget`
  (params (hp_widget :type "UserWidget Object Reference") (faction_color :type "LinearColor Structure") (faction_index :type Integer))
  ;[1 1 1] Set widget assign logic.
  (set `self.w_hp` hp_widget)
  (bind _asw_hp_value (cast `/Game/ai_component/example_data/group_system/w_hp_value` (`self.w_hp`)))
  (`/Game/ai_component/example_data/group_system/w_hp_value.init_widget` _asw_hp_value faction_color faction_index)
  (`self.update_widget`))

(fn `update_hp`
  (params (add_value :type "Float (double-precision)") (remove_health :type Boolean))
  (returns (current_health :type "Float (double-precision)"))
  (bind _returnvalue (`KismetMathLibrary.Abs` add_value))
  ;[1 1 1] Update hp value.
  (set `self.current_health` (`KismetMathLibrary.FClamp` (+ (`self.current_health`) (`KismetMathLibrary.SelectFloat` (* _returnvalue -1.0) _returnvalue remove_health)) 0.0 (`self.max_health`)))
  (`|ExecutionSequence`
    (:`then_0`
      (`self.update_widget`))
    (:`then_1`
      (return (`self.current_health`)))))

(fn `update_widget`
  ;[1 1 1] Update health widget logic.
  (bind _asw_hp_value (cast `/Game/ai_component/example_data/group_system/w_hp_value` (`self.w_hp`)))
  (`/Game/ai_component/example_data/group_system/w_hp_value.hp_value` _asw_hp_value (`KismetMathLibrary.MapRangeClamped` (`self.current_health`) 0.0 (`self.max_health`) 0.0 1.0)))