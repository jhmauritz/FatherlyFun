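; Faction link that gives an owning actor a faction index and resolves it to that faction's bp_faction_manager.
; The lookup finds actors tagged "faction_" plus the index and casts the first match, returning a success flag and the manager reference.
; Setting a new faction updates the index, runs the lookup and fires the EdFaction dispatcher, which also fires on BeginPlay.
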(event `self.ReceiveBeginPlay`
  ;[1 1 1] Faction finder
  ; for owning actors,
  ; beginplay is here.
  (`self.ed_faction`))

(fn `get_owner_faction`
  (returns (return_node :type Boolean) (faction_reference :type "/Game/ai_component/example_data/faction_system/bp_faction_manager Object Reference"))
  ;[1 1 1] Get owner faction by index.
  (bind _outactors (`GameplayStatics.GetAllActorsWithTag` (`KismetStringLibrary.Conv_StringToName` (`KismetStringLibrary.Concat_StrStr` "faction_" (`KismetStringLibrary.Conv_IntToString` (`self.faction_index`))))))
  (if (`KismetArrayLibrary.Array_IsValidIndex` _outactors)
    (bind _asbp_faction_manager (cast `/Game/ai_component/example_data/faction_system/bp_faction_manager` (`|GetArrayItem` _outactors))
      (:`then`
        (return true _asbp_faction_manager))
      (:`CastFailed`
        _)))
  (return false null))

(fn `set_owner_faction`
  (params (new_faction :type Integer))
  (returns (return_node :type Boolean) (faction_reference :type "/Game/ai_component/example_data/faction_system/bp_faction_manager Object Reference"))
  ;[1 1 1] Set new owners faction.
  (set `self.faction_index` new_faction)
  (bind (_return_node _faction_reference) (`self.get_owner_faction`))
  (`self.ed_faction`)
  (return _return_node _faction_reference))