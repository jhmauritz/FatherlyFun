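; Faction spawner Blueprint that creates faction manager actors from a data-driven faction list.
; InitFactions loops over FactionList and, for each index not yet valid in FactionsData, spawns a Bp_faction_manager, stores it there and initializes it with the entry's data and index.
; BeginPlay and the construction script are empty here, so nothing in these graphs calls InitFactions.
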(event `self.ReceiveBeginPlay`
  ;[1 1 1] Faction data spawner,
  ; beginplay is here.
  ; This does spawn all the factions from current list by data.
)

(fn `init_factions`
  (locals (local_transform :type "Transform Structure") (local_data :type "/Game/ai_component/example_data/faction_system/s_faction_data Structure") (local_index :type Integer) (local_faction :type "/Game/ai_component/example_data/faction_system/bp_faction_manager Object Reference"))
  ;[1 1 1] Spawn factions by id.
  (for (_array_element _array_index) (`self.faction_list`)
    (set `local.local_data` _array_element)
    (set `local.local_index` _array_index)
    (if (not (`KismetArrayLibrary.Array_IsValidIndex` (`self.factions_data`) (`local.local_index`)))
      (bind _returnvalue (`|SpawnActorFromClass` "/Game/ai_component/example_data/faction_system/bp_faction_manager.bp_faction_manager_C" (`local.local_transform`) "AlwaysSpawn" "OverrideRootScale" null null))
      (set `local.local_faction` _returnvalue)
      (`KismetArrayLibrary.Array_Add` (`self.factions_data`) (`local.local_faction`))
      (`/Game/ai_component/example_data/faction_system/bp_faction_manager.init_faction` (`local.local_faction`) (`local.local_data`) (`local.local_index`)))))

(fn `UserConstructionScript`)