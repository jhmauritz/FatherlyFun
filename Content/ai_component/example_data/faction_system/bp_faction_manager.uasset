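; Faction manager actor for an RTS-style game that tracks one faction's buildings, resources, gatherers, registered units and groups, and selection state.
; Tick updates group hover from the pawn under the cursor and prunes destroyed entries from the registration and selection lists.
; SendGroup merges units from selected groups of its own faction, then either spawns a group proxy for larger squads or assigns formation travel points to each unit's AI component.
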(event `self.ReceiveBeginPlay`
  ;[1 1 1] Faction actor,
  ; beginplay is here.
  ; This acts like city manager for all units.
  (`self.init_logic`) ; init basic logic.
)

(event `self.ReceiveTick`
  (params (DeltaSeconds :type "Float (single-precision)"))
  ;[1 1 1] Faction actor,
  ; beginplay is here.
  ; This acts like city manager for all units.
  (`self.check_hover` (`.HitActor` (`GameplayStatics.BreakHitResult` (`PlayerController.GetHitResultUnderCursorForObjects` (`GameplayStatics.GetPlayerController` 0) (`|MakeArray` "ObjectTypeQuery3" :!type "EObjectTypeQuery Enum") false)))) ; on tick checks hover of units under mouse.
  (`self.register_refresh`) ; refresh registered units,\nif they are destroyed.
  (`self.selection_refresh`) ; refresh selected units\nif they are destroyed.
)

(fn `add_building`
  (params (building_ref :type "/Game/ai_component/example_data/faction_system/example_bulding Object Reference") (remove :type Boolean))
  ;[1 1 1] Add or remove bulding from list.
  (bind (_is_valid _found_index _actor_reference) (`self.get_building` building_ref))
  (if _is_valid
    (if remove
      (`KismetArrayLibrary.Array_Remove` (`self.building_list`) _found_index))
    (else
      (`KismetArrayLibrary.Array_Add` (`self.building_list`) _actor_reference))))

(fn `add_gatherer`
  (params (resource_id :type Name) (gatherer_actor :type "Actor Object Reference") (remove_gather :type Boolean))
  ;[1 1 1] Add resource gatherer to list.
  (bind (_is_valid _found_index) (`self.get_gatherer` gatherer_actor))
  (if _is_valid
    (if remove_gather
      (`KismetArrayLibrary.Array_Remove` (`self.gatherer_id`) _found_index)
      (`KismetArrayLibrary.Array_Remove` (`self.resource_id`) _found_index))
    (elif (not remove_gather)
      (`KismetArrayLibrary.Array_Add` (`self.gatherer_id`) gatherer_actor)
      (`KismetArrayLibrary.Array_Add` (`self.resource_id`) resource_id))))

(fn `add_resource`
  (params (resource_type :type "/Game/ai_component/example_data/resource_system/enum_resource_type Enum" :default "NewEnumerator3") (add_count :type Integer) (set_resources :type Boolean))
  (locals (local_type :type "/Game/ai_component/example_data/resource_system/enum_resource_type Enum" :default "NewEnumerator0") (local_add :type Integer) (local_set :type Boolean))
  ;[1 1 1] Add or set resources count
  (set `local.local_type` resource_type)
  (set `local.local_add` add_count)
  (set `local.local_set` set_resources)
  (`KismetArrayLibrary.Array_Set` (`self.current_resources`) (`KismetMathLibrary.Conv_ByteToInt` (`local.local_type`)) (`KismetMathLibrary.SelectInt` (`local.local_add`) (+ (`|GetArrayItem` (`self.current_resources`) (`KismetMathLibrary.Conv_ByteToInt` (`local.local_type`))) (`local.local_add`)) (`local.local_set`))))

(fn `check_hover`
  (params (hit_actor :type "Actor Object Reference"))
  (locals (local_actor :type "Actor Object Reference") (local_unit :type "/Game/ai_component/example_data/group_system/bp_unit_component Object Reference"))
  (bind (_is_group _group_actor) (`/Game/ai_component/example_data/group_system/bp_unit_component.get_group_info` (`local.local_unit`)))
  ;[1 1 1] Units hover logic.
  (set `local.local_actor` hit_actor)
  (bind (_return_node _unit_reference) (`/Game/ai_component/base_system/blueprints/bp_easy_ai_library.easy_ai_get_unit` (`local.local_actor`)))
  (if _return_node
    (set `local.local_unit` _unit_reference)
    (if (!= (`.group_actor` (`/Game/ai_component/example_data/group_system/bp_unit_component.get_group_info` (`local.local_unit`))) (`self.latest_hovered`))
      (`|ExecutionSequence`
        (:`then_0`
          (`self.clear_hover`))
        (:`then_1`
          (set `self.latest_hovered` _group_actor)
          (set `self.hovered_groups` (`/Game/ai_component/example_data/group_system/bp_group_manager.current_units` _group_actor))
          (for _array_element (`self.hovered_groups`)
            (bind (_return_node_2 _unit_reference_2) (`/Game/ai_component/base_system/blueprints/bp_easy_ai_library.easy_ai_get_unit` _array_element))
            (`/Game/ai_component/example_data/group_system/bp_unit_component.receive_hover` _unit_reference_2 false)))))
    (else
      (`self.clear_hover`))))

(fn `clear_hover`
  ;[1 1 1] Clear units hovered logic.
  (for _array_element (`self.hovered_groups`)
    (`/Engine/EditorBlueprintResources/StandardMacros.IsValid` _array_element
      (:`Is Valid`
        (bind (_return_node _unit_reference) (`/Game/ai_component/base_system/blueprints/bp_easy_ai_library.easy_ai_get_unit` _array_element))
        (`/Game/ai_component/example_data/group_system/bp_unit_component.receive_hover` _unit_reference true))))
  (`KismetArrayLibrary.Array_Clear` (`self.hovered_groups`))
  (set `self.latest_hovered` null))

(fn `find_buildings`
  (params (FilterClass :type "/Game/ai_component/example_data/faction_system/example_bulding Class Reference"))
  (returns (is_exist :type Boolean) (building_count :type Integer) (building_list :type "Array of Actor Object Reference"))
  ;[1 1 1] find buildings by class.
  (bind _filteredarray (`KismetArrayLibrary.FilterArray` (`self.building_list`) FilterClass))
  (return (`KismetArrayLibrary.Array_IsValidIndex` _filteredarray) (`KismetArrayLibrary.Array_Length` _filteredarray) _filteredarray))

(fn `find_gatherers`
  (params (resource_id :type Name))
  (returns (is_valid :type Boolean) (array_length :type Integer) (sorted_list :type "Array of Name"))
  (locals (local_list_array :type "Array of Name") (local_id :type Name) (local_index :type Integer :default 0) (local_sorted_array :type "Array of Name") (local_gatherer_array :type "Array of Actor Object Reference") (local_sorted_gatherers :type "Array of Actor Object Reference"))
  (bind _local_index (`local.local_index`))
  ;[1 1 1] Find gatherers by type ID list.
  (set `local.local_id` resource_id)
  (set `local.local_list_array` (`self.resource_id`))
  (set `local.local_gatherer_array` (`self.gatherer_id`))
  (set `local.local_index` (`KismetArrayLibrary.Array_Find` (`local.local_list_array`) (`local.local_id`)) :!label _label)
  (if (>= (`local.local_index`) 0)
    (`KismetArrayLibrary.Array_Add` (`local.local_sorted_array`) (`|GetArrayItem` (`local.local_list_array`) _local_index))
    (`KismetArrayLibrary.Array_Add` (`local.local_sorted_gatherers`) (`|GetArrayItem` (`local.local_gatherer_array`) _local_index))
    (`KismetArrayLibrary.Array_Remove` (`local.local_gatherer_array`) (`local.local_index`))
    (`KismetArrayLibrary.Array_Remove` (`local.local_list_array`) (`local.local_index`))
    (goto _label)
    (else
      (return (`KismetArrayLibrary.Array_IsValidIndex` (`local.local_sorted_array`)) (`KismetArrayLibrary.Array_Length` (`local.local_sorted_array`)) (`local.local_sorted_array`)))))

(fn `get_building`
  (params (building_ref :type "/Game/ai_component/example_data/faction_system/example_bulding Object Reference"))
  (returns (is_valid :type Boolean) (found_index :type Integer) (actor_reference :type "/Game/ai_component/example_data/faction_system/example_bulding Object Reference"))
  (bind _building_list (`self.building_list`))
  (bind _returnvalue (`KismetArrayLibrary.Array_Find` _building_list building_ref))
  ;[1 1 1] Get how much bulding of same ID exist in the array.
  (if (>= _returnvalue 0)
    (return false _returnvalue (`|GetArrayItem` _building_list _returnvalue))))

(fn `get_gatherer`
  (params (actor_id :type "Actor Object Reference"))
  (returns (is_valid :type Boolean) (found_index :type Integer) (resource_id :type Name))
  (bind _returnvalue (`KismetArrayLibrary.Array_Find` (`self.gatherer_id`) actor_id))
  (bind _returnvalue_2 (>= _returnvalue 0))
  ;[1 1 1] Get resource gatherers.
  (if _returnvalue_2
    (return _returnvalue_2 _returnvalue (`|GetArrayItem` (`self.resource_id`) _returnvalue))
    (else
      (return false _returnvalue "None"))))

(fn `get_resource`
  (params (resource_type :type "/Game/ai_component/example_data/resource_system/enum_resource_type Enum" :default "NewEnumerator3"))
  (returns (is_exist :type Boolean) (resource_count :type Integer))
  (bind _output (`|GetArrayItem` (`self.current_resources`) (`KismetMathLibrary.Conv_ByteToInt` resource_type)))
  ;[1 1 1] Get resource count by type.
  (return (> _output 0) _output))

(fn `highlight_actor`
  (params (remove :type Boolean) (actor_reference :type "Actor Object Reference"))
  (locals (local_actor :type "Actor Object Reference") (local_index :type Integer :default 0) (local_remove :type Boolean))
  ;[1 1 1] add selected actor
  (set `local.local_remove` remove)
  (set `local.local_actor` actor_reference)
  (set `local.local_index` (`KismetArrayLibrary.Array_Find` (`self.highlight_groups`) (`local.local_actor`)))
  (if (`local.local_remove`)
    (if (>= (`local.local_index`) 0)
      (`KismetArrayLibrary.Array_Remove` (`self.highlight_groups`) (`local.local_index`))
      (bind (_return_node _group_manager) (`/Game/ai_component/base_system/blueprints/bp_easy_ai_library.easy_ai_get_group` (`local.local_actor`)))
      (if _return_node
        (`/Game/ai_component/example_data/group_system/bp_group_manager.highlight_group` _group_manager true)))
    (elif (not (>= (`local.local_index`) 0))
      (`KismetArrayLibrary.Array_Add` (`self.highlight_groups`) (`local.local_actor`))
      (bind (_return_node_2 _group_manager_2) (`/Game/ai_component/base_system/blueprints/bp_easy_ai_library.easy_ai_get_group` (`local.local_actor`)))
      (if _return_node_2
        (`/Game/ai_component/example_data/group_system/bp_group_manager.highlight_group` _group_manager_2 false)))))

(fn `init_faction`
  (params (faction_data :type "/Game/ai_component/example_data/faction_system/s_faction_data Structure") (faction_index :type Integer))
  ;[1 1 1] Init faction logic.
  (set `self.faction_data` faction_data)
  (set `self.faction_index` faction_index)
  (`KismetArrayLibrary.Array_AddUnique` (`self.Tags`) (`KismetStringLibrary.Conv_StringToName` (`KismetStringLibrary.Concat_StrStr` "faction_" (`KismetStringLibrary.Conv_IntToString` (`self.faction_index`))))))

(fn `init_logic`
  ;[1 1 1] Faction Init logic.
  (`|ExecutionSequence`
    (:`then_0`
      (`KismetArrayLibrary.Array_Resize` (`self.current_resources`) (enumcount `/Game/ai_component/example_data/resource_system/enum_resource_type`)))))

(fn `register_groups`
  (params (remove_group :type Boolean) (group_actor :type "Actor Object Reference"))
  (locals (local_remove :type Boolean) (local_actor :type "Actor Object Reference") (local_index :type Integer))
  ;[1 1 1] Assign unit groups to this faction.
  (set `local.local_remove` remove_group)
  (set `local.local_actor` group_actor)
  (set `local.local_index` (`KismetArrayLibrary.Array_Find` (`self.registered_groups`) (`local.local_actor`)))
  (if (`local.local_remove`)
    (if (>= (`local.local_index`) 0)
      (`KismetArrayLibrary.Array_Remove` (`self.registered_groups`) (`local.local_index`)))
    (elif (not (>= (`local.local_index`) 0))
      (`KismetArrayLibrary.Array_Add` (`self.registered_groups`) (`local.local_actor`)))))

(fn `register_refresh`
  (bind _registered_groups (`self.registered_groups`))
  (bind _registered_units (`self.registered_units`))
  ;[1 1 1] Refresh groups and units.
  (bind (_arrayindex _arrayelement) (`/Engine/EditorBlueprintResources/StandardMacros.ReverseForEachLoop` _registered_groups)
    (:`LoopBody`
      (`/Engine/EditorBlueprintResources/StandardMacros.IsValid` _arrayelement
        (:`Is Not Valid`
          (`KismetArrayLibrary.Array_Remove` _registered_groups _arrayindex))))
    (:`Completed`
      (bind (_arrayindex_2 _arrayelement_2) (`/Engine/EditorBlueprintResources/StandardMacros.ReverseForEachLoop` _registered_units)
        (:`LoopBody`
          (`/Engine/EditorBlueprintResources/StandardMacros.IsValid` _arrayelement_2
            (:`Is Not Valid`
              (`KismetArrayLibrary.Array_Remove` _registered_units _arrayindex_2))))))))

(fn `register_units`
  (params (remove_unit :type Boolean) (unit_actor :type "Actor Object Reference"))
  (locals (local_remove :type Boolean) (local_actor :type "Actor Object Reference") (local_index :type Integer))
  ;[1 1 1] Assign unit groups to this faction.
  (set `local.local_remove` remove_unit)
  (set `local.local_actor` unit_actor)
  (set `local.local_index` (`KismetArrayLibrary.Array_Find` (`self.registered_units`) (`local.local_actor`)))
  (if (`local.local_remove`)
    (if (>= (`local.local_index`) 0)
      (`KismetArrayLibrary.Array_Remove` (`self.registered_units`) (`local.local_index`)))
    (elif (not (>= (`local.local_index`) 0))
      (`KismetArrayLibrary.Array_Add` (`self.registered_units`) (`local.local_actor`)))))

(fn `select_actor`
  (params (remove_selection :type Boolean) (actor_reference :type "Actor Object Reference"))
  (locals (local_actor :type "Actor Object Reference") (local_index :type Integer :default 0) (local_remove :type Boolean))
  ;[1 1 1] add selected actor
  (set `local.local_remove` remove_selection)
  (set `local.local_actor` actor_reference)
  (set `local.local_index` (`KismetArrayLibrary.Array_Find` (`self.selected_groups`) (`local.local_actor`)))
  (if (`local.local_remove`)
    (if (>= (`local.local_index`) 0)
      (`KismetArrayLibrary.Array_Remove` (`self.selected_groups`) (`local.local_index`))
      (bind (_return_node _group_manager) (`/Game/ai_component/base_system/blueprints/bp_easy_ai_library.easy_ai_get_group` (`local.local_actor`)))
      (if _return_node
        (`/Game/ai_component/example_data/group_system/bp_group_manager.select_group` _group_manager true)))
    (elif (not (>= (`local.local_index`) 0))
      (`KismetArrayLibrary.Array_Add` (`self.selected_groups`) (`local.local_actor`))
      (bind (_return_node_2 _group_manager_2) (`/Game/ai_component/base_system/blueprints/bp_easy_ai_library.easy_ai_get_group` (`local.local_actor`)))
      (if _return_node_2
        (`/Game/ai_component/example_data/group_system/bp_group_manager.select_group` _group_manager_2 false)))))

(fn `selection_refresh`
  (bind _selected_groups (`self.selected_groups`))
  (bind _highlight_groups (`self.highlight_groups`))
  (bind _hovered_groups (`self.hovered_groups`))
  (bind _latest_send_groups (`self.latest_send_groups`))
  ;[1 1 1] Refresh selections.
  (bind (_arrayindex _arrayelement) (`/Engine/EditorBlueprintResources/StandardMacros.ReverseForEachLoop` _selected_groups)
    (:`LoopBody`
      (`/Engine/EditorBlueprintResources/StandardMacros.IsValid` _arrayelement
        (:`Is Not Valid`
          (`KismetArrayLibrary.Array_Remove` _selected_groups _arrayindex))))
    (:`Completed`
      (bind (_arrayindex_2 _arrayelement_2) (`/Engine/EditorBlueprintResources/StandardMacros.ReverseForEachLoop` _highlight_groups)
        (:`LoopBody`
          (`/Engine/EditorBlueprintResources/StandardMacros.IsValid` _arrayelement_2
            (:`Is Not Valid`
              (`KismetArrayLibrary.Array_Remove` _highlight_groups _arrayindex_2))))
        (:`Completed`
          (bind (_arrayindex_3 _arrayelement_3) (`/Engine/EditorBlueprintResources/StandardMacros.ReverseForEachLoop` _hovered_groups)
            (:`LoopBody`
              (`/Engine/EditorBlueprintResources/StandardMacros.IsValid` _arrayelement_3
                (:`Is Not Valid`
                  (`KismetArrayLibrary.Array_Remove` _hovered_groups _arrayindex_3))))
            (:`Completed`
              (bind (_arrayindex_4 _arrayelement_4) (`/Engine/EditorBlueprintResources/StandardMacros.ReverseForEachLoop` _latest_send_groups)
                (:`LoopBody`
                  (`/Engine/EditorBlueprintResources/StandardMacros.IsValid` _arrayelement_4
                    (:`Is Not Valid`
                      (`KismetArrayLibrary.Array_Remove` _latest_send_groups _arrayindex_4))))))))))))

(fn `send_group`
  (params (target_location :type "Vector Structure") (target_rotation :type "Rotator Structure") (use_proxy :type Boolean))
  (locals (local_target_point :type "Vector Structure") (local_proxy :type "/Game/ai_component/example_data/group_system/bp_group_proxy Object Reference") (local_selected_group :type "/Game/ai_component/example_data/group_system/bp_group_manager Object Reference") (local_owning_groups :type "Array of /Game/ai_component/example_data/group_system/bp_group_manager Object Reference") (local_merged_units :type "Array of Actor Object Reference") (local_use_proxy :type Boolean :default false) (local_transform :type "Transform Structure") (local_rotation :type "Rotator Structure"))
  ;[1 1 1] Send selected units to specific location.
  (set `local.local_target_point` target_location)
  (set `local.local_rotation` target_rotation)
  (set `local.local_use_proxy` use_proxy)
  (for _array_element (`self.selected_groups`)
    (bind (_return_node _group_manager) (`/Game/ai_component/base_system/blueprints/bp_easy_ai_library.easy_ai_get_group` _array_element))
    (set `local.local_selected_group` _group_manager)
    (if (== (`/Game/ai_component/example_data/group_system/bp_group_manager.faction_index` (`local.local_selected_group`)) (`self.faction_index`))
      (`KismetArrayLibrary.Array_Add` (`local.local_owning_groups`) (`local.local_selected_group`))
      (for _array_element_2 (`/Game/ai_component/example_data/group_system/bp_group_manager.current_units` (`local.local_selected_group`))
        (`KismetArrayLibrary.Array_Add` (`local.local_merged_units`) _array_element_2))))
  (if (`KismetArrayLibrary.Array_IsValidIndex` (`local.local_owning_groups`))
    (if (`local.local_use_proxy`)
      (if (> (`KismetArrayLibrary.Array_Length` (`local.local_merged_units`)) 5)
        (bind _returnvalue (`|SpawnActorFromClass` "/Game/ai_component/example_data/group_system/bp_group_proxy.bp_group_proxy_C" (`local.local_transform`) "AlwaysSpawn" "OverrideRootScale" null null))
        (set `local.local_proxy` _returnvalue)
        (set `self.latest_proxy` (`local.local_proxy`))
        (set `self.latest_send_groups` (`local.local_owning_groups`))
        (`/Game/ai_component/example_data/group_system/bp_group_proxy.init_proxy` (`local.local_proxy`) (`local.local_owning_groups`) (`local.local_target_point`))
        (else
          (bind _return_points (`/Game/ai_component/example_data/group_system/bp_formation_manager.set_formation_destination` (`self.bp_formation_manager`) (`local.local_merged_units`) (`local.local_target_point`) (`local.local_rotation`) :!label _label))
          (for (_array_element_3 _array_index) _return_points
            (bind (_return_node_2 _ai_component) (`/Game/ai_component/base_system/blueprints/bp_easy_ai_library.easy_ai_get_component` (`|GetArrayItem` (`local.local_merged_units`) _array_index)))
            (`/Game/ai_component/base_system/blueprints/bp_easy_ai_pathfinder_component.ai_set_travel` _ai_component (make `/Game/ai_component/base_system/structs/01_base/s_ai_05_travel` null _array_element_3 (0.0 0.0 0.0) (struct) 0.0 0.0 0.0 true false false false "g_merged")))))
      (else
        (goto _label)))))

(fn `UserConstructionScript`)