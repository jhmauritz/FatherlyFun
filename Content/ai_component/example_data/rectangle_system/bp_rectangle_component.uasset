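; Rectangle component that provides mouse drag-box selection of unit groups for an owning faction.
; It spawns a rectangle widget, tracks mouse start and end points, and starts dragging beyond a tolerance.
; While dragging, Tick syncs the faction's selected and highlighted groups with actors passed in from HUD draw.
; Shift keeps the selection, Ctrl removes boxed groups, and selection stays within one faction, with the owner's groups taking priority.
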(event `self.ReceiveBeginPlay`
  ;[1 1 1] Rectangle logic beginplay.
)

(event `hud_draw_rectangle`
  (params (rectangle_actors :type "Array of Actor Object Reference"))
  ;[1 1 1] Rectangle logic beginplay.
  (set `self.current_rectangle` rectangle_actors) ; hold rectangle actors here from hud draw.
)

(event `self.ReceiveTick`
  (params (DeltaSeconds :type "Float (single-precision)"))
  ;[1 1 1] Rectangle logic beginplay.
  (`/Engine/EditorBlueprintResources/StandardMacros.IsValid` (`self.owner_faction`)
    (:`Is Valid`
      (`self.rectangle_tick`) ; on tick check rectangle mouse logic,\nstart/end locations.
      (bind _can_drag_selection (`self.check_for_use`)) ; check if drag by mouse is enabled and we can use it now.
      (if _can_drag_selection
        (`|ExecutionSequence`
          (:`then_0`
            (`self.rectangle_clear_selection` (`self.current_rectangle`)))
          (:`then_1`
            (`self.rectangle_add_selection` (`self.current_rectangle`))))))))

(fn `check_for_use`
  (returns (can_drag_selection :type Boolean))
  ;[1 1 1] Check if enabled and can be used.
  (if (`self.is_dragging`)
    (if (`self.windowed_rectangle`)
      (return true)
      (elif (`self.mouse_on_screen`)
        (return true)
        (else
          _))))
  (return false))

(fn `init_rectangle`
  (params (owning_Faction :type "/Game/ai_component/example_data/faction_system/bp_faction_manager Object Reference"))
  ;[1 1 1] Init rectangle component and spawn widget.
  (`|ExecutionSequence`
    (:`then_0`
      (`/Engine/EditorBlueprintResources/StandardMacros.IsValid` (`self.rectangle_widget_reference`)
        (:`Is Not Valid`
          (bind _returnvalue (`|CreateWidget` "/Game/ai_component/example_data/rectangle_system/w_rectangle_layout.w_rectangle_layout_C"))
          (set `self.rectangle_widget_reference` _returnvalue)
          (`|ExecutionSequence`
            (:`then_0`
              (`/Game/ai_component/example_data/rectangle_system/w_rectangle_layout.init_rectangle` (`self.rectangle_widget_reference`) self))
            (:`then_1`
              (`UserWidget.AddToViewport` (`self.rectangle_widget_reference`) 0))))))
    (:`then_1`
      (set `self.owner_faction` owning_Faction))))

(fn `rectangle_add_selection`
  (params (rectangle_result :type "Array of Actor Object Reference"))
  (locals (local_rectangle :type "Array of Actor Object Reference") (local_found_groups :type "Array of Actor Object Reference") (local_selection :type "Actor Object Reference") (local_group_actor :type "/Game/ai_component/example_data/group_system/bp_group_manager Object Reference") (local_group_faction :type Integer))
  ;[1 1 1] Rectangle add selections to storage.
  (set `local.local_rectangle` rectangle_result)
  (if (not (`PlayerController.IsInputKeyDown` (`GameplayStatics.GetPlayerController` 0) "LeftControl"))
    (bind (_arrayindex _arrayelement) (`/Engine/EditorBlueprintResources/StandardMacros.ReverseForEachLoop` (`local.local_rectangle`))
      (:`LoopBody`
        (set `local.local_selection` _arrayelement)
        (bind (_return_node _unit_reference) (`/Game/ai_component/base_system/blueprints/bp_easy_ai_library.easy_ai_get_unit` (`local.local_selection`)))
        (if _return_node
          (bind (_is_group _group_actor) (`/Game/ai_component/example_data/group_system/bp_unit_component.get_group_info` _unit_reference))
          (if _is_group
            (set `local.local_group_actor` _group_actor)
            (if (not (`KismetArrayLibrary.Array_Contains` (`local.local_found_groups`) (`local.local_group_actor`)))
              (`KismetArrayLibrary.Array_Add` (`local.local_found_groups`) (`local.local_group_actor`))
              (set `local.local_group_faction` (`/Game/ai_component/example_data/group_system/bp_group_manager.faction_index` (`local.local_group_actor`)))
              (if (< (`self.latest_selected_faction`) 0)
                (`/Game/ai_component/example_data/faction_system/bp_faction_manager.select_actor` (`self.owner_faction`) false (`local.local_group_actor`) :!label _label)
                (set `self.latest_selected_faction` (`local.local_group_faction`))
                (`/Game/ai_component/example_data/faction_system/bp_faction_manager.highlight_actor` (`self.owner_faction`) false (`local.local_group_actor`))
                (elif (== (`self.latest_selected_faction`) (`local.local_group_faction`))
                  (goto _label)
                  (elif (== (`/Game/ai_component/example_data/faction_system/bp_faction_manager.faction_index` (`self.owner_faction`)) (`local.local_group_faction`))
                    (`|ExecutionSequence`
                      (:`then_0`
                        (`self.rectangle_clear_selection` (`|MakeArray`)))
                      (:`then_1`
                        (goto _label)))))))))))))

(fn `rectangle_clear_selection`
  (params (rectangle_result :type "Array of Actor Object Reference") (released :type Boolean))
  (locals (local_rectangle :type "Array of Actor Object Reference") (local_squad :type "Array of Actor Object Reference") (local_group_actor :type "Actor Object Reference") (local_found :type Boolean) (local_released :type Boolean))
  ;[1 1 1] Rectangle remove selection logic.
  (set `local.local_rectangle` rectangle_result)
  (set `local.local_released` released)
  (bind (_arrayindex _arrayelement) (`/Engine/EditorBlueprintResources/StandardMacros.ReverseForEachLoop` (`/Game/ai_component/example_data/faction_system/bp_faction_manager.selected_groups` (`self.owner_faction`)))
    (:`LoopBody`
      (set `local.local_group_actor` _arrayelement)
      (bind _asbp_group_manager (cast `/Game/ai_component/example_data/group_system/bp_group_manager` (`local.local_group_actor`)))
      (set `local.local_squad` (`/Game/ai_component/example_data/group_system/bp_group_manager.current_units` _asbp_group_manager))
      (set `local.local_found` false)
      (for _array_element (`local.local_rectangle`)
        (if (`KismetArrayLibrary.Array_Contains` (`local.local_squad`) _array_element)
          (set `local.local_found` true)
          (break)))
      (if (`local.local_released`)
        (`/Game/ai_component/example_data/faction_system/bp_faction_manager.highlight_actor` (`self.owner_faction`) true (`local.local_group_actor`))
        (elif (not (`PlayerController.IsInputKeyDown` (`GameplayStatics.GetPlayerController` 0) "LeftShift"))
          (if (`PlayerController.IsInputKeyDown` (`GameplayStatics.GetPlayerController` 0) "LeftControl")
            (if (`local.local_found`)
              (`/Game/ai_component/example_data/faction_system/bp_faction_manager.select_actor` (`self.owner_faction`) true (`local.local_group_actor`)))
            (elif (not (`local.local_found`))
              (`/Game/ai_component/example_data/faction_system/bp_faction_manager.select_actor` (`self.owner_faction`) true (`local.local_group_actor`))
              (`/Game/ai_component/example_data/faction_system/bp_faction_manager.highlight_actor` (`self.owner_faction`) true (`local.local_group_actor`)))))))
    (:`Completed`
      (if (not (`KismetArrayLibrary.Array_IsValidIndex` (`/Game/ai_component/example_data/faction_system/bp_faction_manager.selected_groups` (`self.owner_faction`))))
        (set `self.latest_selected_faction` -1)))))

(fn `rectangle_enabled`
  (params (is_pressed :type Boolean))
  (locals (local_pressed :type Boolean))
  ;[1 1 1] Enable Disable on click logic.
  (set `local.local_pressed` is_pressed)
  (`/Engine/EditorBlueprintResources/StandardMacros.IsValid` (`self.owner_faction`)
    (:`Is Valid`
      (`|ExecutionSequence`
        (:`then_0`
          (if (`local.local_pressed`)
            (`|ExecutionSequence`
              (:`then_0`
                (bind _returnvalue (`WidgetLayoutLibrary.GetMousePositionOnViewport`))
                (set `self.start_point_widget` _returnvalue)
                (set `self.start_point_true` (* (`self.start_point_widget`) (`WidgetLayoutLibrary.GetViewportScale`))))
              (:`then_1`
                (`KismetArrayLibrary.Array_Clear` (`self.current_rectangle`))
                (set `self.is_pressed` true)
                (`self.rectangle_clear_selection` (`|MakeArray`))))
            (else
              (`|ExecutionSequence`
                (:`then_0`
                  (set `self.is_pressed` false)
                  (set `self.is_dragging` false)
                  (`self.rectangle_clear_selection` (`|MakeArray`) true))
                (:`then_1`
                  (set `self.start_point_widget` (0.0 0.0))
                  (set `self.start_point_true` (0.0 0.0)))
                (:`then_2`
                  (`KismetArrayLibrary.Array_Clear` (`self.current_rectangle`))
                  (`/Game/ai_component/example_data/rectangle_system/w_rectangle_layout.rectangle_enabled` (`self.rectangle_widget_reference`) false)
                  (`self.ed_enabled` (`self.is_dragging`)))))))
        (:`then_1`
          (`/Game/ai_component/example_data/rectangle_system/w_rectangle_layout.rectangle_pressed` (`self.rectangle_widget_reference`) (`local.local_pressed`) (`self.start_point_widget`))
          (`self.ed_pressed` (`local.local_pressed`)))))))

(fn `rectangle_tick`
  (locals (local_mouse :type "Vector2D Structure"))
  (bind (_x _y) (`KismetMathLibrary.BreakVector2D` (`self.start_point_widget`)))
  (bind (_x_2 _y_2) (`KismetMathLibrary.BreakVector2D` (`local.local_mouse`)))
  (bind (_x_3 _y_3) (`KismetMathLibrary.BreakVector2D` (`local.local_mouse`)))
  (bind (_x_4 _y_4) (`KismetMathLibrary.BreakVector2D` (/ (`WidgetLayoutLibrary.GetViewportSize`) (`WidgetLayoutLibrary.GetViewportScale`))))
  ;[1 1 1] Tick rectangle movement.
  (if (`self.is_pressed`)
    (bind _returnvalue (`WidgetLayoutLibrary.GetMousePositionOnViewport`))
    (set `local.local_mouse` _returnvalue)
    (set `self.end_point_widget` (`KismetMathLibrary.MakeVector2D` (- _x_2 _x) (- _y_2 _y)))
    (set `self.end_point_true` (* (`local.local_mouse`) (`WidgetLayoutLibrary.GetViewportScale`)))
    (set `self.mouse_on_screen` (and (`KismetMathLibrary.InRange_FloatFloat` _x_3 -2.0 (+ _x_4 2.0)) (`KismetMathLibrary.InRange_FloatFloat` _y_3 -2.0 (+ _y_4 2.0))))
    (if (`self.is_dragging`)
      _
      (elif (!= (`self.start_point_true`) (`self.end_point_true`) :`ErrorTolerance` (`self.drag_enable_tolerance`))
        (set `self.is_dragging` true)
        (`/Game/ai_component/example_data/rectangle_system/w_rectangle_layout.rectangle_enabled` (`self.rectangle_widget_reference`) (`self.is_dragging`))
        (`self.ed_enabled` (`self.is_dragging`))))))