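; HUD Blueprint that handles drag rectangle selection and shows an on-screen framerate counter.
; While its BpRectangleComponent is dragging, DrawHUD gathers all actors inside the screen rectangle, since that query only works during this event.
; The end point is scaled slightly down for precision, and the result feeds the component's HudDrawRectangle.
; A rounded FPS value from clamped delta time is drawn top-left every frame.
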(event `self.ReceiveBeginPlay`
  ;[1 1 1] Hud beginplay logic.
)

(event `self.ReceiveDrawHUD`
  (params (SizeX :type Integer) (SizeY :type Integer))
  ;[1 1 1] Hud beginplay logic.
  (`|ExecutionSequence`
    (:`then_0`
      (if (`/Game/ai_component/example_data/rectangle_system/bp_rectangle_component.is_dragging` (`self.bp_rectangle_component`))
        (`/Game/ai_component/example_data/rectangle_system/bp_rectangle_component.hud_draw_rectangle` (`self.bp_rectangle_component`) (`self.GetActorsInSelectionRectangle` "/Script/Engine.Actor" (`/Game/ai_component/example_data/rectangle_system/bp_rectangle_component.start_point_true` (`self.bp_rectangle_component`)) (* (`/Game/ai_component/example_data/rectangle_system/bp_rectangle_component.end_point_true` (`self.bp_rectangle_component`)) 0.975) false))))
    (:`then_1`
      (`self.DrawText` (`KismetStringLibrary.Conv_IntToString` (`KismetMathLibrary.Round` (/ 1.0 (`KismetMathLibrary.FClamp` (`GameplayStatics.GetWorldDeltaSeconds`) 0.001 100.0)))) (struct :`R` 1.0 :`G` 0.666667 :`A` 1.0) 8.0 8.0 null) ; here we can draw framerate.
    )))

(fn `UserConstructionScript`)