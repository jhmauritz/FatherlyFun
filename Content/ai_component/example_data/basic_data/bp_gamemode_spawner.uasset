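; Game mode helper Blueprint from the AI component's example data that ensures the manager actors the AI relies on exist when the game mode starts.
; A gamemode_started event finds or spawns the faction spawner, then the easy AI recast manager.
; Each uses the first existing instance or spawns one at the origin, then gets its setup call: InitFactions for factions, AssignRecastTags for recast tags.
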(event `gamemode_started`
  ;[1 1 1] Should spawn all the necessary actors for safe work.
  (`|ExecutionSequence`
    (:`then_0`
      (bind _outactors (`GameplayStatics.GetAllActorsOfClass` "/Game/ai_component/example_data/faction_system/bp_faction_spawner.bp_faction_spawner_C"))
      (if (`KismetArrayLibrary.Array_IsValidIndex` _outactors)
        (`/Game/ai_component/example_data/faction_system/bp_faction_spawner.init_factions` (`|GetArrayItem` _outactors))
        (else
          (bind _returnvalue (`|SpawnActorFromClass` "/Game/ai_component/example_data/faction_system/bp_faction_spawner.bp_faction_spawner_C" (`KismetMathLibrary.MakeTransform` (0.0 0.0 0.0)) "AlwaysSpawn" "OverrideRootScale" null null))
          (`/Game/ai_component/example_data/faction_system/bp_faction_spawner.init_factions` _returnvalue))))
    (:`then_1`
      (bind _outactors_2 (`GameplayStatics.GetAllActorsOfClass` "/Game/ai_component/base_system/blueprints/bp_easy_ai_recast_manager.bp_easy_ai_recast_manager_C"))
      (if (`KismetArrayLibrary.Array_IsValidIndex` _outactors_2)
        (`/Game/ai_component/base_system/blueprints/bp_easy_ai_recast_manager.assign_recast_tags` (`|GetArrayItem` _outactors_2))
        (else
          (bind _returnvalue_2 (`|SpawnActorFromClass` "/Game/ai_component/base_system/blueprints/bp_easy_ai_recast_manager.bp_easy_ai_recast_manager_C" (`KismetMathLibrary.MakeTransform` (0.0 0.0 0.0)) "AlwaysSpawn" "OverrideRootScale" null null))
          (`/Game/ai_component/base_system/blueprints/bp_easy_ai_recast_manager.assign_recast_tags` _returnvalue_2))))))