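; Player pawn for a strategy camera that selects and commands units of its owning faction through the EasyAi system.
; Input stays disabled until the AI loads, then left mouse drives HUD rectangle or single-unit selection and right click sends selected groups.
; Swept movement scales with spring-arm zoom, while middle mouse rotates the view with 90-degree snapping and screen-edge turning.
; Extra keys start or stop time-manager waiting and emit test noise for AI.
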(event `Key|LeftMouseButton` :consume false :paused true :overrideparent false
  (params (Key :type "Key Structure"))
  ;[1 1 1] Mouse input, left click and right click,
  ; to select and control units.
  (:`Pressed`
    (`|ExecutionSequence`
      (:`then_0`
        (`/Game/ai_component/example_data/rectangle_system/bp_rectangle_component.rectangle_enabled` (`self.GetComponentByClass` (`PlayerController.GetHUD` (`GameplayStatics.GetPlayerController` 0)) "/Game/ai_component/example_data/rectangle_system/bp_rectangle_component.bp_rectangle_component_C") true))
      (:`then_1`
        (bind (_return_node _unit_reference) (`/Game/ai_component/base_system/blueprints/bp_easy_ai_library.easy_ai_get_unit` (`.HitActor` (`GameplayStatics.BreakHitResult` (`PlayerController.GetHitResultUnderCursorForObjects` (`GameplayStatics.GetPlayerController` 0) (`|MakeArray` "ObjectTypeQuery3" :!type "EObjectTypeQuery Enum") false)))))
        (if _return_node
          (`/Game/ai_component/example_data/faction_system/bp_faction_manager.select_actor` (`self.owning_faction`) false (`.group_actor` (`/Game/ai_component/example_data/group_system/bp_unit_component.get_group_info` _unit_reference)))))))
  (:`Released`
    (`/Game/ai_component/example_data/rectangle_system/bp_rectangle_component.rectangle_enabled` (`self.GetComponentByClass` (`PlayerController.GetHUD` (`GameplayStatics.GetPlayerController` 0)) "/Game/ai_component/example_data/rectangle_system/bp_rectangle_component.bp_rectangle_component_C") false)))

(event `self.ReceiveBeginPlay`
  ;[1 1 1] Strategic pawn,
  ; beginplay is here.
  (`|ExecutionSequence`
    (:`then_0`
      (`self.DisableInput` (`GameplayStatics.GetPlayerController` 0)))
    (:`then_1`
      (`/Game/ai_component/base_system/blueprints/bp_easy_ai_macro_library.easy_ai_is_loaded` ; after AI system\nis managed to load.
        (:`success`
          (bind (_return_node _faction_reference) (`/Game/ai_component/example_data/faction_system/bp_faction_link.get_owner_faction` (`self.bp_faction_link`)))
          (bind _output_get (set `self.owning_faction` _faction_reference)) ; set owning faction for pawn by index.
          (`/Game/ai_component/example_data/rectangle_system/bp_rectangle_component.init_rectangle` (`self.GetComponentByClass` (`PlayerController.GetHUD` (`GameplayStatics.GetPlayerController` 0)) "/Game/ai_component/example_data/rectangle_system/bp_rectangle_component.bp_rectangle_component_C") _output_get)
          (`self.EnableInput` (`GameplayStatics.GetPlayerController` 0)))))
    (:`then_2`
      (bind (_return_node_2 _time_manager) (`/Game/ai_component/base_system/blueprints/bp_easy_ai_library.easy_ai_get_time_manager`))
      (set `self.time_manager` _time_manager)
      (`ActorComponent.SetTickableWhenPaused` (`self.SpringArm`) true))))

(event `Key|RightMouseButton` :consume false :paused true :overrideparent false
  (params (Key :type "Key Structure"))
  (bind _owning_faction (`self.owning_faction`))
  (bind (_hitresult _returnvalue) (`PlayerController.GetHitResultUnderCursorForObjects` (`GameplayStatics.GetPlayerController` 0) (`|MakeArray` "ObjectTypeQuery1" :!type "EObjectTypeQuery Enum") false))
  (bind (_bblockinghit _binitialoverlap _time _distance _location) (`GameplayStatics.BreakHitResult` _hitresult))
  ;[1 1 1] Mouse input, left click and right click,
  ; to select and control units.
  (:`Pressed`
    (if _returnvalue
      (`/Game/ai_component/example_data/faction_system/bp_faction_manager.send_group` :`self` _owning_faction :`target_location` _location :`use_proxy` true)
      (if (`KismetArrayLibrary.Array_IsValidIndex` (`/Game/ai_component/example_data/faction_system/bp_faction_manager.selected_groups` _owning_faction))
        (`KismetSystemLibrary.DrawDebugPoint` _location 20.0 (struct :`R` 0.533333 :`G` 1.0 :`A` 1.0) 1.0) ; draw debug point if groups exist.
      ))))

(event `Key|Six`
  (params (Key :type "Key Structure"))
  ;[1 1 1] Mouse input, left click and right click,
  ; to select and control units.
  (:`Pressed`
    (`/Game/ai_component/day_system/blueprints/bp_easy_ai_time_manager.start_wait` (`self.time_manager`) 5)))

(event `Key|Seven`
  (params (Key :type "Key Structure"))
  ;[1 1 1] Mouse input, left click and right click,
  ; to select and control units.
  (:`Pressed`
    (`/Game/ai_component/day_system/blueprints/bp_easy_ai_time_manager.stop_wait` (`self.time_manager`))))

(event `Key|N`
  (params (Key :type "Key Structure"))
  (bind (_bblockinghit _binitialoverlap _time _distance _location) (`GameplayStatics.BreakHitResult` (`PlayerController.GetHitResultUnderCursorForObjects` (`GameplayStatics.GetPlayerController` 0) (`|MakeArray` "ObjectTypeQuery1" :!type "EObjectTypeQuery Enum") false)))
  ;[1 1 1] Mouse input, left click and right click,
  ; to select and control units.
  (:`Pressed`
    (`self.MakeNoise` 1.0 self _location 0.0 "testnoise2")
    (`KismetSystemLibrary.DrawDebugSphere` _location 100.0 12 (struct :`R` 1.0 :`B` 0.011936 :`A` 1.0) 2.0 1.0) ; draw debug for noise point
  ))

(event `InputAxis|move_y` :consume false :paused true :overrideparent false
  (params (AxisValue :type "Float (single-precision)"))
  ;[1 1 1] Player Pawn movement logic.
  (`self.K2_AddActorWorldOffset` (* (* (`self.GetActorForwardVector`) (`KismetMathLibrary.MapRangeClamped` (`SpringArmComponent.TargetArmLength` (`self.SpringArm`)) 1000.0 10000.0 50.0 200.0)) AxisValue) true) ; camera pawn movement,\nwith sweep, so it can hit invisible walls.
)

(event `InputAxisKey|MouseWheelAxis` :consume false :paused true :overrideparent false
  (params (AxisValue :type "Float (single-precision)"))
  ;[1 1 1] Mouse wheel for camera distance,
  ; also camera rotation by middle mouse.
  (set `SpringArmComponent.TargetArmLength` (`KismetMathLibrary.FClamp` (+ (* AxisValue -500.0) (`SpringArmComponent.TargetArmLength` (`self.SpringArm`))) 1000.0 10000.0) (`self.SpringArm`))
  (if (`self.is_middle_down`)
    (`self.camera_rotation` 5.0) ; if middle mouse is down,\nrotate camera with snap.
  ))

(event `Key|MiddleMouseButton` :consume false :paused true :overrideparent false
  (params (Key :type "Key Structure"))
  ;[1 1 1] Mouse wheel for camera distance,
  ; also camera rotation by middle mouse.
  (:`Pressed`
    (set `self.is_middle_down` true) ; middle mouse bool,\nfor camera rortation.
  )
  (:`Released`
    (set `self.is_middle_down` false)))

(event `InputAxis|move_x` :consume false :paused true :overrideparent false
  (params (AxisValue :type "Float (single-precision)"))
  ;[1 1 1] Player Pawn movement logic.
  (`self.K2_AddActorWorldOffset` (* (* (`self.GetActorRightVector`) (`KismetMathLibrary.MapRangeClamped` (`SpringArmComponent.TargetArmLength` (`self.SpringArm`)) 1000.0 10000.0 50.0 200.0)) AxisValue) true) ; camera pawn movement,\nwith sweep, so it can hit invisible walls.
)

(fn `camera_rotation`
  (params (rotation_scale :type "Float (double-precision)"))
  (locals (local_scale :type "Float (double-precision)"))
  (bind _yaw (.yaw (`self.K2_GetActorRotation`)))
  (bind _returnvalue (`KismetMathLibrary.GridSnap_Float` _yaw 90.0))
  ;[1 1 1] Camera rotation with snap logic.
  (set `local.local_scale` rotation_scale)
  (`|ExecutionSequence`
    (:`then_0`
      (bind _returnvalue_2 (`self.get_mouse_rotation_delta`))
      (`self.K2_AddActorLocalRotation` (`KismetMathLibrary.MakeRotator` 0.0 0.0 (* _returnvalue_2 (`local.local_scale`)))))
    (:`then_1`
      (if (`KismetMathLibrary.NearlyEqual_FloatFloat` _yaw _returnvalue 2.0)
        (`self.K2_SetActorRotation` (`KismetMathLibrary.MakeRotator` 0.0 0.0 _returnvalue))))))

(fn `get_mouse_rotation_delta`
  (returns (ReturnValue :type "Float (double-precision)"))
  ;[1 1 1] Get mouse delta for camera rotation.
  (bind _returnvalue (`WidgetLayoutLibrary.GetMousePositionOnViewport`))
  (bind _x (`KismetMathLibrary.BreakVector2D` (/ (* _returnvalue (`WidgetLayoutLibrary.GetViewportScale`)) (`WidgetLayoutLibrary.GetViewportSize`))))
  (return (`KismetMathLibrary.SelectFloat` (`self.GetInputAxisKeyValue`) (`KismetMathLibrary.SelectFloat` -0.5 0.5 (< _x 0.5)) (`KismetMathLibrary.InRange_FloatFloat` _x 0.01 0.99 false false))))

(fn `UserConstructionScript`)