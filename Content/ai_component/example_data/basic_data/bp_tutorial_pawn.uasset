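; Strategy camera pawn for an AI component tutorial, with RTS-style selection and test commands.
; Camera pans with swept, zoom-scaled movement, zooms by spring arm (tickable while paused), and rotates on middle mouse with edge-of-screen turning and 90-degree snapping.
; Left mouse drives the HUD rectangle component, initialized with the owner's faction; right mouse sends every AI Character to the cursor.
; Debug keys emit a noise or start a time-manager wait.
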(event `self.ReceiveBeginPlay`
  ;[1 1 1] Strategic pawn,
  ; beginplay is here.
  (`ActorComponent.SetTickableWhenPaused` (`self.SpringArm`) true)
  (bind (_return_node _faction_reference) (`/Game/ai_component/example_data/faction_system/bp_faction_link.get_owner_faction` (`self.bp_faction_link`)))
  (`/Game/ai_component/example_data/rectangle_system/bp_rectangle_component.init_rectangle` (`self.GetComponentByClass` (`PlayerController.GetHUD` (`GameplayStatics.GetPlayerController` 0)) "/Game/ai_component/example_data/rectangle_system/bp_rectangle_component.bp_rectangle_component_C") _faction_reference))

(event `Key|LeftMouseButton` :consume false :paused true :overrideparent false
  (params (Key :type "Key Structure"))
  ;[1 1 1] Mouse input, left click and right click,
  ; to select and control units.
  (:`Pressed`
    (`/Game/ai_component/example_data/rectangle_system/bp_rectangle_component.rectangle_enabled` (`self.GetComponentByClass` (`PlayerController.GetHUD` (`GameplayStatics.GetPlayerController` 0)) "/Game/ai_component/example_data/rectangle_system/bp_rectangle_component.bp_rectangle_component_C") true))
  (:`Released`
    (`/Game/ai_component/example_data/rectangle_system/bp_rectangle_component.rectangle_enabled` (`self.GetComponentByClass` (`PlayerController.GetHUD` (`GameplayStatics.GetPlayerController` 0)) "/Game/ai_component/example_data/rectangle_system/bp_rectangle_component.bp_rectangle_component_C") false)))

(event `Key|Three`
  (params (Key :type "Key Structure"))
  ;[1 1 1] Mouse input, left click and right click,
  ; to select and control units.
  (:`Pressed`
    (`self.MakeNoise` 1.0 self (`.Location` (`GameplayStatics.BreakHitResult` (`PlayerController.GetHitResultUnderCursorForObjects` (`GameplayStatics.GetPlayerController` 0) (`|MakeArray` "ObjectTypeQuery1" :!type "EObjectTypeQuery Enum") false))) 0.0 "unique_noise")))

(event `Key|Four`
  (params (Key :type "Key Structure"))
  ;[1 1 1] Mouse input, left click and right click,
  ; to select and control units.
  (:`Pressed`
    (bind (_return_node _time_manager) (`/Game/ai_component/base_system/blueprints/bp_easy_ai_library.easy_ai_get_time_manager`))
    (if _return_node
      (`/Game/ai_component/day_system/blueprints/bp_easy_ai_time_manager.start_wait` _time_manager 10))))

(event `Key|RightMouseButton` :consume false :paused true :overrideparent false
  (params (Key :type "Key Structure"))
  (bind (_bblockinghit _binitialoverlap _time _distance _location) (`GameplayStatics.BreakHitResult` (`PlayerController.GetHitResultUnderCursorForObjects` (`GameplayStatics.GetPlayerController` 0) (`|MakeArray` "ObjectTypeQuery1" :!type "EObjectTypeQuery Enum") false)))
  ;[1 1 1] Mouse input, left click and right click,
  ; to select and control units.
  (:`Pressed`
    (`KismetSystemLibrary.DrawDebugSphere` _location 100.0 0 (struct :`R` 1.0 :`G` 1.0 :`B` 1.0 :`A` 1.0) 1.0 3.0)
    (bind _outactors (`GameplayStatics.GetAllActorsOfClass` "/Script/Engine.Character"))
    (for _array_element _outactors
      (bind (_return_node _ai_component) (`/Game/ai_component/base_system/blueprints/bp_easy_ai_library.easy_ai_get_component` _array_element))
      (if _return_node
        (`/Game/ai_component/base_system/blueprints/bp_easy_ai_pathfinder_component.ai_set_travel` _ai_component (make `/Game/ai_component/base_system/structs/01_base/s_ai_05_travel` null _location (0.0 0.0 0.0) (struct) 0.0 150.0 0.0 true false true false "path_id" "attack=1?defend=2?special_info=3"))))))

(event `InputAxis|move_y` :consume false :paused true :overrideparent false
  (params (AxisValue :type "Float (single-precision)"))
  ;[1 1 1] Player Pawn movement logic.
  (`self.K2_AddActorWorldOffset` (* (* (`self.GetActorForwardVector`) (`KismetMathLibrary.MapRangeClamped` (`SpringArmComponent.TargetArmLength` (`self.SpringArm`)) 1000.0 10000.0 50.0 200.0)) AxisValue) true) ; camera pawn movement,\nwith sweep, so it can hit invisible walls.
)

(event `InputAxisKey|MouseWheelAxis` :consume false :paused true :overrideparent false
  (params (AxisValue :type "Float (single-precision)"))
  ;[1 1 1] Mouse wheel for camera distance,
  ; also camera rotation by middle mouse.
  (set `SpringArmComponent.TargetArmLength` (`KismetMathLibrary.FClamp` (+ (* AxisValue -500.0) (`SpringArmComponent.TargetArmLength` (`self.SpringArm`))) 1000.0 10000.0) (`self.SpringArm`))
  (if (`self.is_middle_down`)
    (`self.camera_rotation` 5.0) ; if middle mouse is down,\nrotate camera with snap.
  ))

(event `Key|MiddleMouseButton` :consume false :paused true :overrideparent false
  (params (Key :type "Key Structure"))
  ;[1 1 1] Mouse wheel for camera distance,
  ; also camera rotation by middle mouse.
  (:`Pressed`
    (set `self.is_middle_down` true) ; middle mouse bool,\nfor camera rortation.
  )
  (:`Released`
    (set `self.is_middle_down` false)))

(event `InputAxis|move_x` :consume false :paused true :overrideparent false
  (params (AxisValue :type "Float (single-precision)"))
  ;[1 1 1] Player Pawn movement logic.
  (`self.K2_AddActorWorldOffset` (* (* (`self.GetActorRightVector`) (`KismetMathLibrary.MapRangeClamped` (`SpringArmComponent.TargetArmLength` (`self.SpringArm`)) 1000.0 10000.0 50.0 200.0)) AxisValue) true) ; camera pawn movement,\nwith sweep, so it can hit invisible walls.
)

(fn `camera_rotation`
  (params (rotation_scale :type "Float (double-precision)"))
  (locals (local_scale :type "Float (double-precision)"))
  (bind _yaw (.yaw (`self.K2_GetActorRotation`)))
  (bind _returnvalue (`KismetMathLibrary.GridSnap_Float` _yaw 90.0))
  ;[1 1 1] Camera rotation with snap logic.
  (set `local.local_scale` rotation_scale)
  (`|ExecutionSequence`
    (:`then_0`
      (bind _returnvalue_2 (`self.get_mouse_rotation_delta`))
      (`self.K2_AddActorLocalRotation` (`KismetMathLibrary.MakeRotator` 0.0 0.0 (* _returnvalue_2 (`local.local_scale`)))))
    (:`then_1`
      (if (`KismetMathLibrary.NearlyEqual_FloatFloat` _yaw _returnvalue 2.0)
        (`self.K2_SetActorRotation` (`KismetMathLibrary.MakeRotator` 0.0 0.0 _returnvalue))))))

(fn `get_mouse_rotation_delta`
  (returns (ReturnValue :type "Float (double-precision)"))
  ;[1 1 1] Get mouse delta for camera rotation.
  (bind _returnvalue (`WidgetLayoutLibrary.GetMousePositionOnViewport`))
  (bind _x (`KismetMathLibrary.BreakVector2D` (/ (* _returnvalue (`WidgetLayoutLibrary.GetViewportScale`)) (`WidgetLayoutLibrary.GetViewportSize`))))
  (return (`KismetMathLibrary.SelectFloat` (`self.GetInputAxisKeyValue`) (`KismetMathLibrary.SelectFloat` -0.5 0.5 (< _x 0.5)) (`KismetMathLibrary.InRange_FloatFloat` _x 0.01 0.99 false false))))

(fn `UserConstructionScript`)