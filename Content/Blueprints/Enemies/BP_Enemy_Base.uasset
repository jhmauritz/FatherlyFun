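; BP_Enemy_Base is a base enemy Blueprint that tracks health and reacts to damage.
; Health starts at MaxHealth, and AnyDamage subtracts from it, calling OnDead at zero or below and OnHit otherwise.
; OnHit and OnDead are empty events here.
; Helpers print the enemy's name with death or debug health messages and swap the material on the Capsule component.
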(event `self.ReceiveBeginPlay`
  (set `self.CurrentHealth` (`self.MaxHealth`)))

(event `self.ReceiveAnyDamage`
  (params (Damage :type "Float (single-precision)") (DamageType :type "DamageType Object Reference") (InstigatedBy :type "Controller Object Reference") (DamageCauser :type "Actor Object Reference"))
  (set `self.CurrentHealth` (- (`self.CurrentHealth`) Damage))
  (if (<= (`self.CurrentHealth`) 0.0)
    (`self.PrintNameOfEnemy` " Dead")
    (`self.OnDead`)
    (if (`self.Debug?`)
      _)
    (else
      (if (`self.Debug?`)
        (`self.PrintNameOfEnemy` (`KismetStringLibrary.Conv_DoubleToString` (`self.CurrentHealth`))))
      (`self.OnHit`))))

(event `/Game/Blueprints/Interfaces/Enemy/BPI_Enemy.OnHit`)

(event `/Game/Blueprints/Interfaces/Enemy/BPI_Enemy.OnDead`)

(fn `ChangeMaterialColor`
  (params (NewMaterial :type "Material Object Reference"))
  (`PrimitiveComponent.SetMaterial` (`self.Capsule`) 0 NewMaterial))

(fn `PrintNameOfEnemy`
  (params (`End Test` :type String))
  (`KismetSystemLibrary.PrintString` (`KismetStringLibrary.Concat_StrStr` "Enemy: " (`KismetSystemLibrary.GetObjectName` self) " " `End Test`)))

(fn `UserConstructionScript`)