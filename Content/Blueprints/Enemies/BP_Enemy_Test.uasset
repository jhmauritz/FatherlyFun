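; BP_Enemy_Test is a test enemy that gives visual feedback on hits and death through its Sphere component's material.
; BeginPlay creates green and red grid dynamic material instances and applies the green one.
; OnHit briefly flashes the sphere red, while OnDead holds red for a few seconds.
; Both use a timer to restore green, so death changes only the look here.
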(event `self.ReceiveBeginPlay`
  (`parent.ReceiveBeginPlay`)
  (bind _returnvalue (`PrimitiveComponent.CreateDynamicMaterialInstance` (`self.Sphere`) 0 "/Game/PrototypeGridMaterial/Materials/MI_GridGreen.MI_GridGreen" "None"))
  (set `self.StartingMat` _returnvalue)
  (bind _returnvalue_2 (`PrimitiveComponent.CreateDynamicMaterialInstance` (`self.Sphere`) 0 "/Game/PrototypeGridMaterial/Materials/MI_GridRed.MI_GridRed" "None"))
  (set `self.DeadMat` _returnvalue_2)
  (`PrimitiveComponent.SetMaterial` (`self.Sphere`) 0 (`self.StartingMat`)))

(event `/Game/Blueprints/Interfaces/Enemy/BPI_Enemy.OnDead`
  (`PrimitiveComponent.SetMaterial` (`self.Sphere`) 0 (`self.DeadMat`))
  (`KismetSystemLibrary.K2_SetTimerDelegate` (delegate `ChangeMatBack`) 3.0))

(event `ChangeMatBack`
  (`PrimitiveComponent.SetMaterial` (`self.Sphere`) 0 (`self.StartingMat`)))

(event `/Game/Blueprints/Interfaces/Enemy/BPI_Enemy.OnHit`
  (`PrimitiveComponent.SetMaterial` (`self.Sphere`) 0 (`self.DeadMat`))
  (`KismetSystemLibrary.K2_SetTimerDelegate` (delegate `ChangeMatBack`) 0.1))

(fn `UserConstructionScript`
  (`parent.UserConstructionScript`))