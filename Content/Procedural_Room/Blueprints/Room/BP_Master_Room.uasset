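; BP_Master_Room is a procedural level room with three doors that spawns neighboring rooms on a grid.
; SpawnRoom, gated to one success per Open, derives the neighbor cell from door yaw and rejects occupied cells through coordinate tags.
; Spawned rooms are tagged Main or Annex and registered with GS_PlayerGeneration, which decrements its count.
; Endgeneration hides unused corridors and, if allowed, randomizes crate child actors from a seeded stream.
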(event `Spawn Room`
  (params (`Index Door` :type Integer) (Room :type "/Game/Procedural_Room/Blueprints/Room/BP_Master_Room Class Reference") (`main ?` :type Boolean))
  (bind _output (`|GetArrayItem` (`|MakeArray` (`self.Door 0`) (`self.Door 1`) (`self.Door 2`)) `Index Door`))
  (bind (_returnvalue_location _returnvalue_rotation) (`KismetMathLibrary.BreakTransform` (`SceneComponent.K2_GetComponentToWorld` _output)))
  (`/Engine/EditorBlueprintResources/StandardMacros.Gate` false :!label _label
    (:`Exit`
      (set `self.main ?` `main ?`)
      (bind (_new_x _new_y) (`self.Set X/Y` `Index Door`))
      ;[1 1 1] Check If Room Location and door Already taken
      (bind _outactors (`GameplayStatics.GetAllActorsWithTag` (`self.Tag Coord` _new_x _new_y)))
      (bind _door_chosen_ (`self.Door Choice` `Index Door`))
      (if (and _door_chosen_ (== (`KismetArrayLibrary.Array_Length` _outactors) 0) (not (`/Game/Procedural_Room/Blueprints/SC_Door.Generate ?` _output)))
        (`self.close`)
        (set `/Game/Procedural_Room/Blueprints/SC_Door.Generate ?` true _output)
        (bind _returnvalue (`|SpawnActorFromClass` Room (`KismetMathLibrary.MakeTransform` _returnvalue_location _returnvalue_rotation) "Undefined" "OverrideRootScale" null 0 null))
        (`/Engine/EditorBlueprintResources/StandardMacros.IsValid` _returnvalue
          (:`Is Valid`
            (bind _output_get (set `/Game/Procedural_Room/Blueprints/Room/BP_Master_Room.X` _new_x _returnvalue))
            (bind _output_get_2 (set `/Game/Procedural_Room/Blueprints/Room/BP_Master_Room.Y` _new_y _returnvalue))
            (bind _tags (`Actor.Tags` _returnvalue))
            (`KismetArrayLibrary.Array_Add` _tags (`self.Tag Coord` _output_get _output_get_2))
            (if (`self.main ?`)
              (`KismetArrayLibrary.Array_Add` _tags "Main")
              (else
                (`KismetArrayLibrary.Array_Add` _tags "Annex")))
            (set `/Game/Procedural_Room/Blueprints/Room/BP_Master_Room.RoomNumber` (+ (`self.RoomNumber`) 1) _returnvalue)
            (bind _asgs_player_generation (cast `/Game/Procedural_Room/Blueprints/GS_PlayerGeneration` (`GameplayStatics.GetGameState`)))
            (`/Game/Procedural_Room/Blueprints/GS_PlayerGeneration.Decrement` _asgs_player_generation (`self.main ?`))
            (`/Game/Procedural_Room/Blueprints/GS_PlayerGeneration.Add Room` _asgs_player_generation _returnvalue)))))))

(event `Open`
  (goto _label :!via `Open`))

(event `close`
  (goto _label :!via `Close`))

(event `End generation`
  (bind _child (`self.Child`))
  (bind _seed (`self.Seed`))
  (bind _crateclass (`self.CrateClass`))
  (bind _crate_child (`self.Crate child`))
  ;[1 1 1] hide corridor when no room was generated on it
  (for _array_element (`self.K2_GetComponentsByClass` "/Script/Engine.StaticMeshComponent")
    (bind _returnvalue (`KismetSystemLibrary.GetObjectName` _array_element))
    (if (and (`KismetStringLibrary.EqualEqual_StrStr` _returnvalue "corridor 1") (not (`/Game/Procedural_Room/Blueprints/SC_Door.Generate ?` (`self.Door 0`))))
      (`|ExecutionSequence`
        (:`then_0`
          (`SceneComponent.SetVisibility` _array_element false true :!label _label_2))
        (:`then_1`
          (if (and (`KismetStringLibrary.EqualEqual_StrStr` _returnvalue "corridor 2") (not (`/Game/Procedural_Room/Blueprints/SC_Door.Generate ?` (`self.Door 1`)))) :!label _label_3
            (`|ExecutionSequence`
              (:`then_0`
                (goto _label_2))
              (:`then_1`
                _)))
          (if (and (`KismetStringLibrary.EqualEqual_StrStr` _returnvalue "corridor 3") (not (`/Game/Procedural_Room/Blueprints/SC_Door.Generate ?` (`self.Door 2`))))
            (goto _label_2))))
      (else
        (goto _label_3))))
  (if (`self.Allow Crate ?`)
    ;[1 1 1] Random Number of crates
    (set `self.Crate child` (`|MakeArray` (`self.Crate 1`) (`self.Crate 2`) (`self.Crate 3`) (`self.Crate 4`) (`self.Crate 5`)))
    (for _ (range (+ (`KismetMathLibrary.RandomIntegerInRangeFromStream` 2 5 (`self.Seed`)) 1))
      (set `self.Child` (`|GetArrayItem` _crate_child (`KismetMathLibrary.RandomIntegerFromStream` (`KismetArrayLibrary.Array_Length` _crate_child) _seed)))
      (`/Engine/EditorBlueprintResources/StandardMacros.IsValid` _child
        (:`Is Valid`
          (`SceneComponent.K2_SetWorldRotation` _child (`KismetMathLibrary.MakeRotator` 0.0 0.0 (`KismetMathLibrary.RandomFloatInRangeFromStream` -45.0 45.0 _seed)) false false)
          (`ChildActorComponent.SetChildActorClass` _child (`|GetArrayItem` _crateclass (`KismetMathLibrary.RandomIntegerFromStream` (`KismetArrayLibrary.Array_Length` _crateclass) _seed)))
          (`KismetArrayLibrary.Array_RemoveItem` _crate_child _child))))))

(fn `Door Choice`
  (params (Selection :type Integer))
  (returns (`Door Chosen ` :type Boolean))
  (locals (`Door Chosen` :type Boolean :default false))
  (switch `int` Selection
    (:`0`
      (set `local.Door Chosen` (`self.A`)))
    (:`1`
      (set `local.Door Chosen` (`self.B`)))
    (:`2`
      (set `local.Door Chosen` (`self.C`))))
  (return (`local.Door Chosen`)))

(fn `Set X/Y`
  (params (Selection :type Integer))
  (returns (`new x` :type Integer) (`new y` :type Integer))
  (locals (xadd :type Integer) (yadd :type Integer) (`World Rotation` :type Integer :default 0))
  (bind (_returnvalue_roll _returnvalue_pitch _returnvalue_yaw) (`KismetMathLibrary.BreakRotator` (`SceneComponent.K2_GetComponentRotation` (`self.Door 2`))))
  (bind (_returnvalue_roll_2 _returnvalue_pitch_2 _returnvalue_yaw_2) (`KismetMathLibrary.BreakRotator` (`SceneComponent.K2_GetComponentRotation` (`self.Door 0`))))
  (bind (_returnvalue_roll_3 _returnvalue_pitch_3 _returnvalue_yaw_3) (`KismetMathLibrary.BreakRotator` (`SceneComponent.K2_GetComponentRotation` (`self.Door 1`))))
  (switch `int` Selection
    (:`0`
      (set `local.World Rotation` (`KismetMathLibrary.FTrunc` (+ (/ _returnvalue_yaw_2 90.0) 2.0))))
    (:`1`
      (set `local.World Rotation` (`KismetMathLibrary.FTrunc` (+ (/ _returnvalue_yaw_3 90.0) 2.0))))
    (:`2`
      (set `local.World Rotation` (`KismetMathLibrary.FTrunc` (+ (/ _returnvalue_yaw 90.0) 2.0)))))
  (`|ExecutionSequence`
    (:`then_0`
      (switch `int` (`local.World Rotation`)
        (:`0`
          (set `local.xadd` -1)
          (set `local.yadd` 0))
        (:`1`
          (set `local.xadd` 0)
          (set `local.yadd` -1))
        (:`2`
          (set `local.xadd` 1)
          (set `local.yadd` 0))
        (:`3`
          (set `local.xadd` 0)
          (set `local.yadd` 1))))
    (:`then_1`
      (return (+ (`local.xadd`) (`self.X`)) (+ (`local.yadd`) (`self.Y`))))))

(fn `UserConstructionScript`)