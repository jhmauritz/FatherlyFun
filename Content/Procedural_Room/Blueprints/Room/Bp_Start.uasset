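; Start room actor that tags itself "Start" and builds a live miniature map of the procedurally generated level at its Beacon.
; A gated loop waits RefreshTime, destroys the old map, finds all master rooms and updates their grid bounds.
; It spawns a Bp_RoomMap per room, scaled to the scan plane and colored by Start, End and Main tags and door generation flags.
; The loop re-triggers itself until StopScanning closes the gate.
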(event `self.ReceiveBeginPlay`
  (`parent.ReceiveBeginPlay`)
  (`KismetArrayLibrary.Array_Add` (`self.Tags`) "Start")
  (`self.Scanning`))

(event `Scanning`
  (bind (_returnvalue_x _returnvalue_y _returnvalue_z) (`KismetMathLibrary.BreakVector` (`SceneComponent.K2_GetComponentLocation` (`self.beacon`))))
  (bind _returnvalue (/ (`self.scanplane`) (`KismetMathLibrary.Conv_IntToDouble` (+ (+ (- (`self.xmax`) (`self.xmin`)) (- (`self.Ymax`) (`self.Ymin`))) 1))))
  (bind (_returnvalue_x_2 _returnvalue_y_2) (`KismetMathLibrary.BreakVector` (`KismetMathLibrary.Conv_DoubleToVector` (/ _returnvalue 100.0))))
  (`/Engine/EditorBlueprintResources/StandardMacros.Gate` false :!label _label
    (:`Exit`
      (`KismetSystemLibrary.Delay` (`self.refresh Time`))
      ;[1 1 1] Destroy map
      (for _array_element (`self.RoomMap Reference`)
        (`self.K2_DestroyActor` _array_element))
      (`KismetArrayLibrary.Array_Clear` (`self.RoomMap Reference`))
      (bind _outactors (`GameplayStatics.GetAllActorsOfClass` "/Game/Procedural_Room/Blueprints/Room/BP_Master_Room.BP_Master_Room_C"))
      (bind _output_get (set `self.Rooms Reference` _outactors))
      (for _array_element_2 _output_get
        ;[1 1 1] Get Min/Max of X and Y (level size)
        (`|ExecutionSequence`
          (:`then_0`
            (bind _x (`/Game/Procedural_Room/Blueprints/Room/BP_Master_Room.X` _array_element_2))
            (if (< _x (`self.xmin`))
              (set `self.xmin` _x)))
          (:`then_1`
            (if (> _x (`self.xmax`))
              (set `self.xmax` _x)))
          (:`then_2`
            (bind _y (`/Game/Procedural_Room/Blueprints/Room/BP_Master_Room.Y` _array_element_2))
            (if (< _y (`self.Ymin`))
              (set `self.Ymin` _y)))
          (:`then_3`
            (if (> _y (`self.Ymax`))
              (set `self.Ymax` _y)))))
      (for _array_element_3 (`self.Rooms Reference`)
        (bind (_returnvalue_roll _returnvalue_pitch _returnvalue_yaw) (`KismetMathLibrary.BreakRotator` (`self.K2_GetActorRotation` _array_element_3)))
        (bind _returnvalue_2 (`|SpawnActorFromClass` "/Game/Procedural_Room/Blueprints/Bp_RoomMap.Bp_RoomMap_C" (`KismetMathLibrary.MakeTransform` (`KismetMathLibrary.MakeVector` (+ _returnvalue_x (* _returnvalue (`KismetMathLibrary.Conv_IntToDouble` (`/Game/Procedural_Room/Blueprints/Room/BP_Master_Room.Y` _array_element_3)))) (+ _returnvalue_y (* (* _returnvalue (`KismetMathLibrary.Conv_IntToDouble` (`/Game/Procedural_Room/Blueprints/Room/BP_Master_Room.X` _array_element_3))) -1.0)) _returnvalue_z) (`KismetMathLibrary.MakeRotator` _returnvalue_roll _returnvalue_pitch (- _returnvalue_yaw 90.0)) (`KismetMathLibrary.MakeVector` _returnvalue_x_2 _returnvalue_y_2 0.2)) "Undefined" "OverrideRootScale" null null))
        ;[1 1 1] Change color and path of spawned room map
        (bind (_a__ _b__ _c__) (`self.Get Generate Door` _array_element_3))
        (`/Game/Procedural_Room/Blueprints/Bp_RoomMap.Set Color` _returnvalue_2 (`self.ActorHasTag` _array_element_3 "Start") (`self.ActorHasTag` _array_element_3 "End") _a__ _b__ _c__ (`self.ActorHasTag` _array_element_3 "Main"))
        (`KismetArrayLibrary.Array_AddUnique` (`self.RoomMap Reference`) _returnvalue_2))
      (`self.Scanning`))))

(event `Stop Scanning`
  (goto _label :!via `Close`))

(fn `Get Generate Door`
  (params (Room :type "Actor Object Reference"))
  (returns (`A  ` :type Boolean) (`B  ` :type Boolean) (`C  ` :type Boolean))
  (locals (`A ` :type Boolean) (`B ` :type Boolean) (`C ` :type Boolean))
  (for (_array_element _array_index) (`self.K2_GetComponentsByClass` Room "/Game/Procedural_Room/Blueprints/SC_Door.SC_Door_C")
    (switch `int` _array_index
      (:`0`
        (bind _generate__ (`/Game/Procedural_Room/Blueprints/SC_Door.Generate ?` _array_element))
        (set `local.A ` _generate__))
      (:`1`
        (set `local.B ` _generate__))
      (:`2`
        (set `local.C ` _generate__))))
  (return (`local.A `) (`local.B `) (`local.C `)))

(fn `UserConstructionScript`
  (`parent.UserConstructionScript`))