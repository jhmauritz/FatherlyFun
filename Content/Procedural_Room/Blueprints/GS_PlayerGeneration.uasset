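; Procedural room-layout generator that grows a level from BP_Start using a seeded random stream.
; A zero-delay self-calling loop chains main rooms from the newest, restarting if the shortfall exceeds 40%, then swaps the last for BP_End.
; An annex pass branches off rooms with free doors, with retry counters capping both phases.
; Finally, rooms with unconnected doors become matching corridor or dead-end variants, and the rest receive EndGeneration.
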(event `Generate room`
  (params (`Room list` :type "Array of /Game/Procedural_Room/Blueprints/Room/BP_Master_Room Class Reference") (`Main ?` :type Boolean))
  (bind _last_room_generate (`self.Last Room Generate`))
  (bind _game_seed (`self.Game Seed`))
  ;[1 1 1] Spawn random Room at random location using game seed
  (bind _door_list_ (`self.Get a Random Valide Door`))
  (`/Game/Procedural_Room/Blueprints/Room/BP_Master_Room.Open` _last_room_generate)
  (`/Game/Procedural_Room/Blueprints/Room/BP_Master_Room.Spawn Room` _last_room_generate (`KismetStringLibrary.Conv_StringToInt` (`KismetStringLibrary.Replace` (`KismetSystemLibrary.GetObjectName` (`|GetArrayItem` _door_list_ (`KismetMathLibrary.RandomIntegerFromStream` (`KismetArrayLibrary.Array_Length` _door_list_) _game_seed))) "Door")) (`|GetArrayItem` `Room list` (`KismetMathLibrary.RandomIntegerFromStream` (`KismetArrayLibrary.Array_Length` `Room list`) _game_seed)) `Main ?`))

(event `Start Generation`
  (params (`Game Seed` :type "RandomStream Structure"))
  (set `self.Game Seed` `Game Seed`)
  ;[1 1 1] Get start room reference
  (bind _outactors (`GameplayStatics.GetAllActorsOfClass` "/Game/Procedural_Room/Blueprints/Room/BP_Master_Room.BP_Master_Room_C"))
  (bind _output_get (set `self.Spawned Rooms List` _outactors))
  (bind _asbp_start (cast `/Game/Procedural_Room/Blueprints/Room/Bp_Start` (`|GetArrayItem` _output_get))
    (:`then`
      (set `self.Start Room reference` _asbp_start))
    (:`CastFailed`
      _))
  ;[1 1 1] reference of Needed Rooms For percent of errors after spawn end room
  (set `self.percent of Error` (`self.Main `))
  (`self.Generation`))

(event `Decrement`
  (params (`main ?` :type Boolean))
  ;[1 1 1] Decrement number of room needed to spawn
  (if `main ?`
    (`/Engine/EditorBlueprintResources/StandardMacros.DecrementInt` (`self.Main `))
    (else
      (`/Engine/EditorBlueprintResources/StandardMacros.DecrementInt` (`self.Annex`)))))

(event `Add Room`
  (params (`Room ref` :type "/Game/Procedural_Room/Blueprints/Room/BP_Master_Room Object Reference"))
  ;[1 1 1] List of rooms spawned
  (`KismetArrayLibrary.Array_Add` (`self.Spawned Rooms List`) `Room ref`))

(event `Generation`
  (bind _last_room_generate (`self.Last Room Generate`))
  (bind _percent_of_error (`self.percent of Error`))
  (bind _spawned_rooms_list (`self.Spawned Rooms List`))
  (bind _start_room_reference (`self.Start Room reference`))
  (bind (_returnvalue_location _returnvalue_rotation) (`KismetMathLibrary.BreakTransform` (`self.GetTransform` _last_room_generate)))
  ;[1 1 1 1 50] Main Generation
  (`KismetSystemLibrary.Delay` 0.0)
  (if (`self.Main Generation ?`)
    ;;[1 1 1] Generate rooms By selecting main rooms in the structure
    (`self.get Latest Room Spawned`)
    (`self.Generate room` (`self.Main Room`) true)
    ;;[1 1 1] If Generation is Stuck, force to pass main generation
    (bind _result (`/Engine/EditorBlueprintResources/StandardMacros.DecrementInt` (`self.Spawn try Remaining`))
      (:`  `
        (if (== _result 0)
          (set `self.Main ` 0))
        ;;[1 1 1] Finish To Generate all main rooms ?
        (if (> (`self.Main `) 0)
          ;;[1 1 1] Loop
          (`self.Generation`)
          (elif (> (- _percent_of_error (`KismetArrayLibrary.Array_Length` (`self.Spawned Rooms List`))) (`KismetMathLibrary.FTrunc` (* _percent_of_error 0.4)))
            ;;[1 1 1] Remove all Rooms but Keep Start
            (`KismetArrayLibrary.Array_RemoveItem` _spawned_rooms_list (`self.Start Room reference`))
            (for _array_element _spawned_rooms_list
              (`self.K2_DestroyActor` _array_element))
            ;;[1 1 1] Reset settings and start new generation
            (`KismetArrayLibrary.Array_Clear` _spawned_rooms_list)
            (`KismetArrayLibrary.Array_AddUnique` _spawned_rooms_list _start_room_reference)
            (bind _output_get (set `self.Main ` (`self.percent of Error`)))
            (set `self.Spawn try Remaining` (* _output_get 4))
            ;;[1 1 1] reset room door generate
            (set `/Game/Procedural_Room/Blueprints/SC_Door.Generate ?` false (`|GetArrayItem` (`self.K2_GetComponentsByClass` _start_room_reference "/Game/Procedural_Room/Blueprints/SC_Door.SC_Door_C") 1))
            (`/Game/Procedural_Room/Blueprints/Room/BP_Master_Room.Open` _start_room_reference)
            (`self.Generation`)
            (else
              ;;[1 1 1] Replace last room by end room
              (`/Engine/EditorBlueprintResources/StandardMacros.DoOnce` false
                (:`Completed`
                  (`self.get Latest Room Spawned`)
                  (bind _returnvalue (`|SpawnActorFromClass` "/Game/Procedural_Room/Blueprints/Room/BP_End.BP_End_C" (`KismetMathLibrary.MakeTransform` _returnvalue_location _returnvalue_rotation) "Undefined" "OverrideRootScale" null 0 null))
                  (`self.Set End Room Info` _returnvalue (`/Game/Procedural_Room/Blueprints/Room/BP_Master_Room.X` _last_room_generate) (`/Game/Procedural_Room/Blueprints/Room/BP_Master_Room.Y` _last_room_generate))
                  (`self.K2_DestroyActor` (`self.Last Room Generate`))
                  (set `self.Main Generation ?` false)
                  (set `self.Spawn try Remaining` (* (`self.percent of Error`) 5))
                  (`self.Generation`))))))))
    (else
      ;[1 1 1 1 50] Annex Generation
      ;;[1 1 1] get all room with valide door (faster generation)
      (bind _room_remaining_ (`self.Room accesibility`))
      (set `self.Last Room Generate` (`|GetArrayItem` _room_remaining_ (`KismetMathLibrary.RandomIntegerFromStream` (`KismetArrayLibrary.Array_Length` _room_remaining_) (`self.Game Seed`))))
      (`self.Generate room` (`self.Annex Room`))
      (bind _result_2 (`/Engine/EditorBlueprintResources/StandardMacros.DecrementInt` (`self.Spawn try Remaining`))
        (:`  `
          (if (== _result_2 0)
            (set `self.Annex` 0))
          (if (> (`self.Annex`) 0)
            (`self.Generation`)
            (else
              (for _array_element_2 (`self.Spawned Rooms List`)
                (`/Engine/EditorBlueprintResources/StandardMacros.IsValid` _array_element_2
                  (:`Is Valid`
                    (bind _ismissingroom_ (`self.hasEmptyHall` _array_element_2))
                    (if _ismissingroom_
                      (`self.replaceEmptyHall` _array_element_2)
                      (else
                        (set `/Game/Procedural_Room/Blueprints/Room/BP_Master_Room.Seed` (`self.Game Seed`) _array_element_2)
                        (`/Game/Procedural_Room/Blueprints/Room/BP_Master_Room.End generation` _array_element_2))))))
              (`/Game/Procedural_Room/Blueprints/Room/Bp_Start.Stop Scanning` (`self.Start Room reference`))
              (`KismetSystemLibrary.PrintString` "Finish"))))))))

(fn `Get a Random Valide Door`
  (returns (`Door list ` :type "Array of /Game/Procedural_Room/Blueprints/SC_Door Object Reference"))
  (locals (`Door list` :type "Array of /Game/Procedural_Room/Blueprints/SC_Door Object Reference"))
  (bind _last_room_generate (`self.Last Room Generate`))
  (for (_array_element _array_index) (`|MakeArray` (`/Game/Procedural_Room/Blueprints/Room/BP_Master_Room.Door 0` _last_room_generate) (`/Game/Procedural_Room/Blueprints/Room/BP_Master_Room.Door 1` _last_room_generate) (`/Game/Procedural_Room/Blueprints/Room/BP_Master_Room.Door 2` _last_room_generate))
    (if (and (not (`/Game/Procedural_Room/Blueprints/SC_Door.Generate ?` _array_element)) (`|GetArrayItem` (`|MakeArray` (`/Game/Procedural_Room/Blueprints/Room/BP_Master_Room.A` _last_room_generate) (`/Game/Procedural_Room/Blueprints/Room/BP_Master_Room.B` _last_room_generate) (`/Game/Procedural_Room/Blueprints/Room/BP_Master_Room.C` _last_room_generate)) _array_index))
      (`KismetArrayLibrary.Array_AddUnique` (`local.Door list`) _array_element)))
  (return (`local.Door list`)))

(fn `get Latest Room Spawned`
  (locals (RoomNumber :type Integer))
  ;[1 1 1] get the latest room spawned
  (set `local.RoomNumber` -1)
  (for _array_element (`self.Spawned Rooms List`)
    (bind _roomnumber (`/Game/Procedural_Room/Blueprints/Room/BP_Master_Room.RoomNumber` _array_element))
    (if (> _roomnumber (`local.RoomNumber`))
      (set `self.Last Room Generate` _array_element)
      (set `local.RoomNumber` _roomnumber)))
  (return))

(fn `hasEmptyHall`
  (params (Target :type "/Game/Procedural_Room/Blueprints/Room/BP_Master_Room Object Reference"))
  (returns (`IsMissingRoom ` :type Boolean))
  (locals (IsMissingRoom :type Boolean))
  (if (`/Game/Procedural_Room/Blueprints/Room/BP_Master_Room.A` Target)
    (if (`/Game/Procedural_Room/Blueprints/SC_Door.Generate ?` (`/Game/Procedural_Room/Blueprints/Room/BP_Master_Room.Door 0` Target))
      (if (`/Game/Procedural_Room/Blueprints/Room/BP_Master_Room.B` Target) :!label _label
        (if (`/Game/Procedural_Room/Blueprints/SC_Door.Generate ?` (`/Game/Procedural_Room/Blueprints/Room/BP_Master_Room.Door 1` Target))
          (if (`/Game/Procedural_Room/Blueprints/Room/BP_Master_Room.C` Target) :!label _label_2
            (if (not (`/Game/Procedural_Room/Blueprints/SC_Door.Generate ?` (`/Game/Procedural_Room/Blueprints/Room/BP_Master_Room.Door 2` Target)))
              (set `local.IsMissingRoom` true)))
          (else
            (set `local.IsMissingRoom` true)))
        (else
          (goto _label_2)))
      (else
        (set `local.IsMissingRoom` true)))
    (else
      (goto _label)))
  (return (`local.IsMissingRoom`)))

(fn `replaceEmptyHall`
  (params (Room :type "/Game/Procedural_Room/Blueprints/Room/BP_Master_Room Object Reference"))
  (locals (NewRoomClass :type "/Game/Procedural_Room/Blueprints/Room/BP_Master_Room Class Reference") (DoorA :type "/Game/Procedural_Room/Blueprints/SC_Door Object Reference") (DoorB :type "/Game/Procedural_Room/Blueprints/SC_Door Object Reference") (DoorC :type "/Game/Procedural_Room/Blueprints/SC_Door Object Reference"))
  (bind _room (`local.Room`))
  (bind _a (`/Game/Procedural_Room/Blueprints/Room/BP_Master_Room.A` Room))
  (bind _b (`/Game/Procedural_Room/Blueprints/Room/BP_Master_Room.B` Room))
  (bind _c (`/Game/Procedural_Room/Blueprints/Room/BP_Master_Room.C` Room))
  (bind _returnvalue (not _b))
  (bind _returnvalue_2 (not _c))
  (bind _returnvalue_3 (not _a))
  (bind (_returnvalue_location _returnvalue_rotation) (`KismetMathLibrary.BreakTransform` (`self.GetTransform` _room)))
  (bind _generate__ (`/Game/Procedural_Room/Blueprints/SC_Door.Generate ?` (`local.DoorC`)))
  (bind _generate___2 (`/Game/Procedural_Room/Blueprints/SC_Door.Generate ?` (`local.DoorA`)))
  (bind _generate___3 (`/Game/Procedural_Room/Blueprints/SC_Door.Generate ?` (`local.DoorB`)))
  (bind _generate___4 (`/Game/Procedural_Room/Blueprints/SC_Door.Generate ?` (`local.DoorC`)))
  (bind _generate___5 (`/Game/Procedural_Room/Blueprints/SC_Door.Generate ?` (`local.DoorB`)))
  (bind _generate___6 (`/Game/Procedural_Room/Blueprints/SC_Door.Generate ?` (`local.DoorA`)))
  (bind _generate___7 (`/Game/Procedural_Room/Blueprints/SC_Door.Generate ?` (`local.DoorB`)))
  (bind _generate___8 (`/Game/Procedural_Room/Blueprints/SC_Door.Generate ?` (`local.DoorA`)))
  (bind _generate___9 (`/Game/Procedural_Room/Blueprints/SC_Door.Generate ?` (`local.DoorC`)))
  (bind _returnvalue_4 (not _generate___4))
  (bind _returnvalue_5 (not _generate___2))
  (bind _returnvalue_6 (not _generate___5))
  (bind _returnvalue_7 (not _generate___6))
  (bind _returnvalue_8 (not _generate___7))
  (bind _returnvalue_9 (not _generate___8))
  (bind _returnvalue_10 (not _generate__))
  (bind _returnvalue_11 (not _generate___9))
  (bind _returnvalue_12 (not _generate___3))
  (set `local.DoorA` (`/Game/Procedural_Room/Blueprints/Room/BP_Master_Room.Door 0` Room))
  (set `local.DoorB` (`/Game/Procedural_Room/Blueprints/Room/BP_Master_Room.Door 1` Room))
  (set `local.DoorC` (`/Game/Procedural_Room/Blueprints/Room/BP_Master_Room.Door 2` Room))
  ;[1 1 1] 1-Door A no room, Dead end
  ; 2-Door B no room, Dead end
  ; 3-Door C no Room, Dead end
  (if (and _a _returnvalue _returnvalue_2)
    (if (`/Game/Procedural_Room/Blueprints/SC_Door.Generate ?` (`local.DoorA`))
      (return)
      (else
        (set `local.NewRoomClass` "/Game/Procedural_Room/Blueprints/Room/BP_Room6.BP_Room6_C")
        ;[1 1 1] Spawn the new room and destroy the old one
        (bind _returnvalue_13 (`|SpawnActorFromClass` (`local.NewRoomClass`) (`KismetMathLibrary.MakeTransform` _returnvalue_location _returnvalue_rotation) "Undefined" "OverrideRootScale" null 0 null :!label _label))
        (`self.Set End Room Info` _returnvalue_13 (`/Game/Procedural_Room/Blueprints/Room/BP_Master_Room.X` _room) (`/Game/Procedural_Room/Blueprints/Room/BP_Master_Room.Y` _room))
        (set `/Game/Procedural_Room/Blueprints/Room/BP_Master_Room.main ?` (`/Game/Procedural_Room/Blueprints/Room/BP_Master_Room.main ?` _room) _returnvalue_13)
        (set `/Game/Procedural_Room/Blueprints/Room/BP_Master_Room.RoomNumber` (`/Game/Procedural_Room/Blueprints/Room/BP_Master_Room.RoomNumber` _room) _returnvalue_13)
        (if (`/Game/Procedural_Room/Blueprints/Room/BP_Master_Room.A` _returnvalue_13)
          (set `/Game/Procedural_Room/Blueprints/SC_Door.Generate ?` true (`/Game/Procedural_Room/Blueprints/Room/BP_Master_Room.Door 0` _returnvalue_13)))
        (if (`/Game/Procedural_Room/Blueprints/Room/BP_Master_Room.B` _returnvalue_13)
          (set `/Game/Procedural_Room/Blueprints/SC_Door.Generate ?` true (`/Game/Procedural_Room/Blueprints/Room/BP_Master_Room.Door 1` _returnvalue_13)))
        (if (`/Game/Procedural_Room/Blueprints/Room/BP_Master_Room.C` _returnvalue_13)
          (set `/Game/Procedural_Room/Blueprints/SC_Door.Generate ?` true (`/Game/Procedural_Room/Blueprints/Room/BP_Master_Room.Door 2` _returnvalue_13)))
        (`self.K2_DestroyActor` (`local.Room`))))
    (elif (and _returnvalue_3 _b _returnvalue_2)
      (if (`/Game/Procedural_Room/Blueprints/SC_Door.Generate ?` (`local.DoorB`))
        (return)
        (else
          (set `local.NewRoomClass` "/Game/Procedural_Room/Blueprints/Room/BP_Room6.BP_Room6_C")
          (goto _label)))
      (elif (and _returnvalue_3 _returnvalue _c)
        (if (`/Game/Procedural_Room/Blueprints/SC_Door.Generate ?` (`local.DoorC`))
          (return)
          (else
            (set `local.NewRoomClass` "/Game/Procedural_Room/Blueprints/Room/BP_Room6.BP_Room6_C")
            (goto _label)))
        (elif (and _a _b _returnvalue_2)
          ;[1 1 1] No Room attached, dead end
          (if (and _returnvalue_7 _returnvalue_8)
            (set `local.NewRoomClass` "/Game/Procedural_Room/Blueprints/Room/BP_Room6.BP_Room6_C")
            (goto _label)
            (else
              ;[1 1 1] Door A not generated so straight room (B)
              (if (and _returnvalue_7 _generate___7)
                (set `local.NewRoomClass` "/Game/Procedural_Room/Blueprints/Room/BP_Room1.BP_Room1_C")
                (goto _label)
                (else
                  ;[1 1 1] Door B not generated so left room (A)
                  (if (and _generate___6 _returnvalue_8)
                    (set `local.NewRoomClass` "/Game/Procedural_Room/Blueprints/Room/BP_Room4.BP_Room4_C")
                    (goto _label)
                    (else
                      (return)))))))
          (elif (and _a _returnvalue _c)
            ;[1 1 1] No Room attached, dead end
            (if (and _returnvalue_9 _returnvalue_11)
              (set `local.NewRoomClass` "/Game/Procedural_Room/Blueprints/Room/BP_Room6.BP_Room6_C")
              (goto _label)
              (else
                ;[1 1 1] Door A not generated so right room (C)
                (if (and _returnvalue_9 _generate___9)
                  (set `local.NewRoomClass` "/Game/Procedural_Room/Blueprints/Room/BP_Room3.BP_Room3_C")
                  (goto _label)
                  (else
                    ;[1 1 1] Door C not generated so left room (A)
                    (if (and _generate___8 _returnvalue_11)
                      (set `local.NewRoomClass` "/Game/Procedural_Room/Blueprints/Room/BP_Room4.BP_Room4_C")
                      (goto _label)
                      (else
                        (return)))))))
            (elif (and _returnvalue_3 _b _c)
              ;[1 1 1] No Room attached, dead end
              (if (and _returnvalue_6 _returnvalue_4)
                (set `local.NewRoomClass` "/Game/Procedural_Room/Blueprints/Room/BP_Room6.BP_Room6_C")
                (goto _label)
                (else
                  ;[1 1 1] Door B not generated so right room (C)
                  (if (and _returnvalue_6 _generate___4)
                    (set `local.NewRoomClass` "/Game/Procedural_Room/Blueprints/Room/BP_Room3.BP_Room3_C")
                    (goto _label)
                    (else
                      ;[1 1 1] Door C not generated so straight room (B)
                      (if (and _generate___5 _returnvalue_4)
                        (set `local.NewRoomClass` "/Game/Procedural_Room/Blueprints/Room/BP_Room1.BP_Room1_C")
                        (goto _label)
                        (else
                          (return)))))))
              (elif (and _a _b _c)
                ;[1 1 1] No Room attached, dead end
                (if (and _returnvalue_5 _returnvalue_12 _returnvalue_10)
                  (set `local.NewRoomClass` "/Game/Procedural_Room/Blueprints/Room/BP_Room6.BP_Room6_C")
                  (goto _label)
                  (else
                    ;[1 1 1] Door A not generated, So BC
                    (if (and _returnvalue_5 _generate___3 _generate__)
                      (set `local.NewRoomClass` "/Game/Procedural_Room/Blueprints/Room/BP_Room7.BP_Room7_C")
                      (goto _label)
                      (else
                        ;[1 1 1] Door B not generated, So AC
                        (if (and _generate___2 _returnvalue_12 _generate__)
                          (set `local.NewRoomClass` "/Game/Procedural_Room/Blueprints/Room/BP_Room5.BP_Room5_C")
                          (goto _label)
                          (else
                            ;[1 1 1] Door C not generated, So AB
                            (if (and _generate___2 _generate___3 _returnvalue_10)
                              (set `local.NewRoomClass` "/Game/Procedural_Room/Blueprints/Room/BP_Room8.BP_Room8_C")
                              (goto _label)
                              (else
                                ;[1 1 1] Door A,B not generated, So right (C)
                                (if (and _returnvalue_5 _returnvalue_12 _generate__)
                                  (set `local.NewRoomClass` "/Game/Procedural_Room/Blueprints/Room/BP_Room3.BP_Room3_C")
                                  (goto _label)
                                  (else
                                    ;[1 1 1] Door A,C not generated, So Straight (B)
                                    (if (and _returnvalue_5 _generate___3 _returnvalue_10)
                                      (set `local.NewRoomClass` "/Game/Procedural_Room/Blueprints/Room/BP_Room1.BP_Room1_C")
                                      (goto _label)
                                      (else
                                        ;[1 1 1] Door B,C not generated, So Left (A)
                                        (if (and _generate___2 _returnvalue_12 _returnvalue_10)
                                          (set `local.NewRoomClass` "/Game/Procedural_Room/Blueprints/Room/BP_Room4.BP_Room4_C")
                                          (goto _label)
                                          (else
                                            (return)))))))))))))))))))))))

(fn `Room accesibility`
  (returns (`Room Remaining ` :type "Array of /Game/Procedural_Room/Blueprints/Room/BP_Master_Room Object Reference"))
  (locals (`Door remaining ?` :type Boolean :default false) (`Room Remaining` :type "Array of /Game/Procedural_Room/Blueprints/Room/BP_Master_Room Object Reference"))
  (for _array_element (`self.Spawned Rooms List`)
    (`/Engine/EditorBlueprintResources/StandardMacros.IsValid` _array_element
      (:`Is Valid`
        (set `local.Door remaining ?` false)
        (for _array_element_2 (`self.K2_GetComponentsByClass` _array_element "/Game/Procedural_Room/Blueprints/SC_Door.SC_Door_C")
          (if (not (`/Game/Procedural_Room/Blueprints/SC_Door.Generate ?` _array_element_2))
            (set `local.Door remaining ?` true)))
        (if (`local.Door remaining ?`)
          (`KismetArrayLibrary.Array_AddUnique` (`local.Room Remaining`) _array_element)))))
  (return (`local.Room Remaining`)))

(fn `UserConstructionScript`)